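; Food dispenser actor that repeatedly spawns BP_Food along a line within its box.
; BeginPlay starts a looping timer at the FoodDispatch interval, with a random variance on the first delay.
; Each spawn takes X and Z from the actor's location and a random Y from the Box bounds.
; Spawned food receives the PlayerDistrib value as PlayerCheck and the HUD reference from the game manager.
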(event Custom|StartFood
  (bind _returnvalue (Transformation|GetActorLocation))
  (bind _box (Variables|Default|GetBox))
  (bind (_origin _boxextent) (Collision|GetComponentBounds _box))
  ;[0.15 0.15 0.15 0.5] Creer un BP_food en random de la box
  (Game|SpawnActorfromClass "/Game/Blueprints/Gameplay/BP_Food.BP_Food_C" (Math|Transform|MakeTransform (Math|Vector|MakeVector (.x _returnvalue) (.y (Math|Random|RandomPointinBoundingBox _origin _boxextent)) (.z _returnvalue)) "0, 0, 0" "1.000000,1.000000,1.000000") "Undefined" "MultiplyWithRoot" 0 (Variables|Default|GetplayerDistrib) (Variables|/Game/Blueprints/Gameplay/BP_GameManager.BP_GameManager_C|GetHUD_Ref (Variables|Default|GetGameManagerRef)) 0))

(event EventBeginPlay
  (Utilities|Time|SetTimerbyEvent (delegate Custom|StartFood) (Variables|Default|GetFoodDispatch) true false 0.0 5.0))

(event Collision|EventActorBeginOverlap
  (params (OtherActor :type Actor%20Object%20Reference)))

(event EventTick
  (params (DeltaSeconds :type Float%20%28single-precision%29)))

(fn ConstructionScript)