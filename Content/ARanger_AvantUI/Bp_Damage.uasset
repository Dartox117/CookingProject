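; Floating score popup actor that shows Score as four animated digit widgets, then destroys itself.
; BeginPlay splits Score into thousands, hundreds, tens and units, blanks leading digits by flags, and picks a color tier by threshold.
; A timeline lerps each WBP_PointEarnPopup widget to its own offset and drives alpha, with a cycling HSV rainbow for the top tier.
; The tens check overwrites IsCentaine, leaving IsDixiaine unset.
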(event Custom|Event_CutPoint
  (bind _score (Variables|Default|GetScore))
  (bind (_remainder _returnvalue) (Math|Float|Division(WholeandRemainder) _score 1e+03))
  (bind (_remainder_2 _returnvalue_2) (Math|Float|Division(WholeandRemainder) _remainder 1e+02))
  (bind (_remainder_3 _returnvalue_3) (Math|Float|Division(WholeandRemainder) _remainder_2 1e+01))
  ;[0.15 0.15 0.15 0.5] Get the Score Unite
  (Variables|Default|SetIs_Millier (!= 0 _returnvalue))
  (Variables|Default|SetText_Millier (Utilities|Text|ToText(Integer) _returnvalue))
  (Variables|Default|SetIs_Centaine (!= 0 _returnvalue_2))
  (Variables|Default|SetText_Centaine (Utilities|Text|ToText(Integer) _returnvalue_2))
  (Variables|Default|SetIs_Centaine (!= 0 _returnvalue_3))
  (Variables|Default|SetText_Dixiaine (Utilities|Text|ToText(Integer) _returnvalue_3))
  (Variables|Default|SetText_Unite (Utilities|Text|ToText(Integer) (Math|Float|Truncate _remainder_3))))

(event Custom|Prepare_Color
  (if (<= (Variables|Default|GetScore) 1e+02)
    (Variables|Default|SetLevelOfScore 0)
    (elif (<= (Variables|Default|GetScore) 2.5e+02)
      (Variables|Default|SetLevelOfScore 1)
      (elif (<= (Variables|Default|GetScore) 5e+02)
        (Variables|Default|SetLevelOfScore 2)
        (elif (<= (Variables|Default|GetScore) 7.5e+02)
          (Variables|Default|SetLevelOfScore 3)
          (elif (<= (Variables|Default|GetScore) 1e+03)
            (Variables|Default|SetLevelOfScore 4)
            (else
              (Variables|Default|SetLevelOfScore 5))))))))

(event Custom|Prepare_ScoreText
  ;[0.15 0.15 0.15 0.5] Prepare Score
  (if (not (Variables|Default|GetIs_Millier))
    (Variables|Default|SetText_Millier "")
    (if (not (Variables|Default|GetIs_Centaine))
      (Variables|Default|SetText_Centaine "")
      (if (not (Variables|Default|GetIs_Dixiaine))
        (Variables|Default|SetText_Dixiaine "")))))

(event EventBeginPlay
  (CallFunction|EventCutPoint)
  (CallFunction|PrepareScoreText)
  (CallFunction|PrepareColor)
  (Utilities|FlowControl|Sequence
    (:then_0
      (bind _aswbp_point_earn_popup (Utilities|Casting|CastToWBP_PointEarnPopup (UserInterface|GetWidget (Variables|Default|GetWidget_Unite))))
      (Default|SetTexy _aswbp_point_earn_popup (Variables|Default|GetText_Unite)))
    (:then_1
      (bind _aswbp_point_earn_popup_2 (Utilities|Casting|CastToWBP_PointEarnPopup (UserInterface|GetWidget (Variables|Default|GetWidget_Dixaine))))
      (Default|SetTexy _aswbp_point_earn_popup_2 (Variables|Default|GetText_Dixiaine)))
    (:then_2
      (bind _aswbp_point_earn_popup_3 (Utilities|Casting|CastToWBP_PointEarnPopup (UserInterface|GetWidget (Variables|Default|GetWidget_Centaine))))
      (Default|SetTexy _aswbp_point_earn_popup_3 (Variables|Default|GetText_Centaine)))
    (:then_3
      (bind _aswbp_point_earn_popup_4 (Utilities|Casting|CastToWBP_PointEarnPopup (UserInterface|GetWidget (Variables|Default|GetWidget_Millier))))
      (Default|SetTexy _aswbp_point_earn_popup_4 (Variables|Default|GetText_Millier)))
    (:then_4
      (Components|Timeline|SetPlayRate (Variables|Default|GetTimeline) (Variables|Default|GetPlaySpeed))
      (bind (_direction _t_unite _t_dixaine _t_centaine _t_millier _alpha _colors) (Timeline|Timeline PlayFromStart)
        (:Update
          (Utilities|FlowControl|Sequence
            (:then_0
              (Utilities|MacroMouvement :Widget (Variables|Default|GetWidget_Unite) :Finish "0.000000,30.000000,60.000000" :Progression _t_unite))
            (:then_1
              (Utilities|MacroMouvement :Widget (Variables|Default|GetWidget_Dixaine) :Finish "0.000000,10.000000,60.000000" :Progression _t_dixaine))
            (:then_2
              (Utilities|MacroMouvement :Widget (Variables|Default|GetWidget_Centaine) :Finish "0.000000,-10.000000,60.000000" :Progression _t_centaine))
            (:then_3
              (Utilities|MacroMouvement :Widget (Variables|Default|GetWidget_Millier) :Finish "0.000000,-30.000000,60.000000" :Progression _t_millier))
            (:then_4
              (switch int (Variables|Default|GetLevelOfScore)
                (:0
                  (Variables|Default|SetScoreColors "(R=1.000000,G=1.000000,B=1.000000,A=1.000000)")
                  (Utilities|MacroColors (Variables|Default|GetWidget_Unite) (Variables|Default|GetScoreColors) _alpha :!label _label)
                  (Utilities|MacroColors (Variables|Default|GetWidget_Dixaine) (Variables|Default|GetScoreColors) _alpha)
                  (Utilities|MacroColors (Variables|Default|GetWidget_Centaine) (Variables|Default|GetScoreColors) _alpha)
                  (Utilities|MacroColors (Variables|Default|GetWidget_Millier) (Variables|Default|GetScoreColors) _alpha))
                (:1
                  (Variables|Default|SetScoreColors "(R=1.000000,G=0.971796,B=0.000000,A=1.000000)")
                  (goto _label))
                (:2
                  (Variables|Default|SetScoreColors "(R=1.000000,G=0.458535,B=0.000000,A=1.000000)")
                  (goto _label))
                (:3
                  (Variables|Default|SetScoreColors "(R=1.000000,G=0.025093,B=0.000000,A=1.000000)")
                  (goto _label))
                (:4
                  (Variables|Default|SetScoreColors "(R=0.453125,G=0.003571,B=0.257745,A=1.000000)")
                  (goto _label))
                (:5
                  (Utilities|MacroColors (Variables|Default|GetWidget_Unite) (Class|KismetMathLibrary|HSVtoRGB (Math|Float|Lerp 0.0 1.08e+03 _colors) 1.0 1.0 1.0) _alpha)
                  (Utilities|MacroColors (Variables|Default|GetWidget_Dixaine) (Class|KismetMathLibrary|HSVtoRGB (Math|Float|Lerp 0.0 1.08e+03 _colors) 1.0 1.0 1.0) _alpha)
                  (Utilities|MacroColors (Variables|Default|GetWidget_Centaine) (Class|KismetMathLibrary|HSVtoRGB (Math|Float|Lerp 0.0 1.08e+03 _colors) 1.0 1.0 1.0) _alpha)
                  (Utilities|MacroColors (Variables|Default|GetWidget_Millier) (Class|KismetMathLibrary|HSVtoRGB (Math|Float|Lerp 0.0 1.08e+03 _colors) 1.0 1.0 1.0) _alpha))))))
        (:Finished
          (Utilities|FlowControl|Delay 1.0)
          (Actor|DestroyActor))))))

(fn ConstructionScript
  (Variables|Default|SetWidgetMillier_InitialLocation (Variables|/Script/Engine.SceneComponent|GetRelativeLocation (Variables|Default|GetWidget_Millier)))
  (Variables|Default|SetWidgetCentaine_InitialLocation (Variables|/Script/Engine.SceneComponent|GetRelativeLocation (Variables|Default|GetWidget_Centaine)))
  (Variables|Default|SetWidgetDixaine_InitialLocation (Variables|/Script/Engine.SceneComponent|GetRelativeLocation (Variables|Default|GetWidget_Dixaine)))
  (Variables|Default|SetWidgetUnite_InitialLocation (Variables|/Script/Engine.SceneComponent|GetRelativeLocation (Variables|Default|GetWidget_Unite))))