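; Anim notify that ends the player's cooking animation.
; When the owner implements BPI_Player and is a BP_Player, it switches the mesh back to Animation Blueprint mode, unfreezes the player and clears the cooking flag.
; It then triggers a scene capture on the plate camera and hides the plate.
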(fn ReceivedNotify
  (params (MeshComp :type Skeletal%20Mesh%20Component%20Object%20Reference) (Animation :type Anim%20Sequence%20Base%20Object%20Reference) (EventReference :type Anim%20Notify%20Event%20Reference%20Structure%20%28by%20ref%29))
  (bind _returnvalue (Components|GetOwner MeshComp))
  (if (Utilities|DoesObjectImplementInterface _returnvalue "/Game/Blueprints/BPI/BPI_Player.BPI_Player_C")
    (bind _asbp_player (Utilities|Casting|CastToBP_Player _returnvalue))
    (Components|Animation|SetAnimationMode (Variables|/Script/Engine.Character|GetMesh _asbp_player) "AnimationBlueprint" true)
    (Default|UnFreezePlayer _asbp_player)
    (Variables|/Game/Blueprints/Player/BP_Player.BP_Player_C|SetIsCooking _asbp_player false)
    (Rendering|SceneCapture|CaptureScene (Variables|/Game/Blueprints/Player/BP_Player.BP_Player_C|GetPlate_Camera _asbp_player) :!class /Script/Engine.SceneCaptureComponent2D)
    (Rendering|SetVisibility (Variables|/Game/Blueprints/Player/BP_Player.BP_Player_C|GetPlate _asbp_player) false false)
    (return false)))