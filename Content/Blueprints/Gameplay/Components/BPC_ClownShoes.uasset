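; BPC_ClownShoes is an actor component that applies a slow debuff to its owning BP_Player on BeginPlay, unless the player is protected.
; It scales down Speed, walk speed and DashPower, applying the multiplier twice to walk speed, then adds a Niagara burst and purple outline overlay.
; DestroySelf, which nothing here calls, restores base speed and a hardcoded dash power, clears the effects and slowed flag, and destroys the component.
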(event Custom|DestroySelf
  (bind _as_bp_player (Variables|Default|GetAs%20BP%20Player))
  ;[0.15 0.01245 0.01352 0.5] Destroy Self
  (bind _output_get (Variables|/Game/Blueprints/Player/BP_Player.BP_Player_C|SetSpeed _as_bp_player (Variables|/Game/Blueprints/Player/BP_Player.BP_Player_C|GetBaseSpeed _as_bp_player)))
  (Variables|/Script/Engine.CharacterMovementComponent|SetMaxWalkSpeed (Variables|/Script/Engine.Character|GetCharacterMovement _as_bp_player) _output_get)
  (Variables|/Game/Blueprints/Player/BP_Player.BP_Player_C|SetDashPower (Variables|Default|GetAs%20BP%20Player) 3e+03)
  (Components|DestroyComponent (Variables|Default|GetNewVar))
  (Rendering|Material|SetOverlayMaterial (Variables|/Script/Engine.Character|GetMesh (Variables|Default|GetAs%20BP%20Player)) 0 :!class /Script/Engine.MeshComponent)
  (Variables|/Game/Blueprints/Player/BP_Player.BP_Player_C|SetIsSlowed (Variables|Default|GetAs%20BP%20Player) false)
  (Components|DestroyComponent))

(event Custom|SpeedSlow
  ;[0.008808 0.15 0.00336 0.5] Slow the active Player
  (bind _asbp_player (Utilities|Casting|CastToBP_Player (Components|GetOwner)))
  (bind _output_get (Variables|Default|SetAs%20BP%20Player _asbp_player))
  (if (not (Variables|/Game/Blueprints/Player/BP_Player.BP_Player_C|GetIsProtected _asbp_player))
    (Variables|/Game/Blueprints/Player/BP_Player.BP_Player_C|SetSpeed _output_get (* (Variables|/Game/Blueprints/Player/BP_Player.BP_Player_C|GetSpeed _asbp_player) 0.75))
    (Variables|/Script/Engine.CharacterMovementComponent|SetMaxWalkSpeed (Variables|/Script/Engine.Character|GetCharacterMovement _asbp_player) (* (Variables|/Game/Blueprints/Player/BP_Player.BP_Player_C|GetSpeed _asbp_player) 0.75))
    (Variables|/Game/Blueprints/Player/BP_Player.BP_Player_C|SetDashPower (Variables|Default|GetAs%20BP%20Player) (* (Variables|/Game/Blueprints/Player/BP_Player.BP_Player_C|GetDashPower (Variables|Default|GetAs%20BP%20Player)) 0.75))
    (bind _returnvalue (Game|AddComponentbyClass (Variables|Default|GetAs%20BP%20Player) "/Script/Niagara.NiagaraComponent" false))
    (bind _output_get_2 (Variables|Default|SetNewVar _returnvalue))
    (Class|NiagaraComponent|SetAsset _output_get_2 "/Game/Art/VFX/NG_Player_SlowBurst.NG_Player_SlowBurst" true)
    (Rendering|Material|SetOverlayMaterial (Variables|/Script/Engine.Character|GetMesh (Variables|Default|GetAs%20BP%20Player)) "/Game/Art/Materials/Shader/Outline/MI_Outline_Purple.MI_Outline_Purple" :!class /Script/Engine.MeshComponent)
    (Variables|/Game/Blueprints/Player/BP_Player.BP_Player_C|SetIsSlowed (Variables|Default|GetAs%20BP%20Player) true)))

(event EventBeginPlay
  (CallFunction|SpeedSlow))

(event EventTick
  (params (DeltaSeconds :type Float%20%28single-precision%29)))