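; Player component for the GymAds debuff, which temporarily lowers ingredient carry capacity by one.
; On BeginPlay, an unprotected player gets the matching HUD slot flagged via the controller's inventory widget; with four or more items held, the last is removed and inventory-down Niagara activates.
; EndEffect restores capacity, clears the HUD and effect, then destroys the component.
; Players protected at start are only recorded, so removal changes nothing.
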(event Custom|CarryLess
  (bind _asbp_player (Utilities|Casting|CastToBP_Player (Components|GetOwner)))
  (bind _output_get (Variables|Default|SetAs%20BP%20Player _asbp_player))
  (if (not (Variables|/Game/Blueprints/Player/BP_Player.BP_Player_C|GetIsProtected _output_get))
    (CallFunction|WrongInventory)
    (Variables|/Game/Blueprints/Player/BP_Player.BP_Player_C|SetMaxIngrediantCarry (Variables|Default|GetAs%20BP%20Player) (- (Variables|/Game/Blueprints/Player/BP_Player.BP_Player_C|GetMaxIngrediantCarry (Variables|Default|GetAs%20BP%20Player)) 1))
    (if (>= (Utilities|Array|Length (Variables|/Game/Blueprints/Player/BP_Player.BP_Player_C|GetStructureInfoArray (Variables|Default|GetAs%20BP%20Player))) 4)
      (Utilities|Array|RemoveItem (Variables|/Game/Blueprints/Player/BP_Player.BP_Player_C|GetStructureInfoArray (Variables|Default|GetAs%20BP%20Player)) (Utilities|Array|Get(acopy) (Variables|/Game/Blueprints/Player/BP_Player.BP_Player_C|GetStructureInfoArray (Variables|Default|GetAs%20BP%20Player)) (Utilities|Array|LastIndex (Variables|/Game/Blueprints/Player/BP_Player.BP_Player_C|GetStructureInfoArray (Variables|Default|GetAs%20BP%20Player)))))
      (Components|StaticMesh|SetStaticMesh (Utilities|Array|Get(acopy) (Variables|/Game/Blueprints/Player/BP_Player.BP_Player_C|GetStaticmesh_Array (Variables|Default|GetAs%20BP%20Player)) (Utilities|Array|LastIndex (Variables|/Game/Blueprints/Player/BP_Player.BP_Player_C|GetStaticmesh_Array (Variables|Default|GetAs%20BP%20Player)))) 0)
      (Default|SetInventory (Variables|Default|GetAs%20BP%20Player))
      (Components|Activation|Activate (Variables|/Game/Blueprints/Player/BP_Player.BP_Player_C|GetNG_InventoryDown (Variables|Default|GetAs%20BP%20Player)) false))
    (else
      (Variables|Default|SetIsPlayerProtected true))))

(event Custom|EndEffect
  (bind _as_bp_player (Variables|Default|GetAs%20BP%20Player))
  (if (not (Variables|Default|GetIsPlayerProtected))
    (Variables|/Game/Blueprints/Player/BP_Player.BP_Player_C|SetMaxIngrediantCarry _as_bp_player (+ (Variables|/Game/Blueprints/Player/BP_Player.BP_Player_C|GetMaxIngrediantCarry _as_bp_player) 1))
    (Variables|Default|SetOpacity 0.0)
    (CallFunction|WrongInventory)
    (Components|Activation|Deactivate (Variables|/Game/Blueprints/Player/BP_Player.BP_Player_C|GetNG_InventoryDown (Variables|Default|GetAs%20BP%20Player)))
    (Components|DestroyComponent)
    (else
      (Components|DestroyComponent))))

(event Custom|WrongInventory
  (bind _as_bp_player (Variables|Default|GetAs%20BP%20Player))
  (bind _as_bp_player_2 (Variables|Default|GetAs%20BP%20Player))
  (switch int (Variables|/Game/Blueprints/Player/BP_Player.BP_Player_C|Getid_controler (Variables|Default|GetAs%20BP%20Player))
    (:0
      (Default|GymAdsEvent (Variables|/Game/Blueprints/Widget/WG_HUD.WG_HUD_C|GetWG_Inventory (Variables|/Game/Blueprints/GameManager/BP_GameManager.BP_GameManager_C|GetHUD_Ref (Variables|/Game/Blueprints/Player/BP_Player.BP_Player_C|GetRef%20Game%20Manager (Variables|Default|GetAs%20BP%20Player)))) (Variables|/Game/Blueprints/Player/BP_Player.BP_Player_C|Getid_controler _as_bp_player_2) (Variables|Default|GetOpacity) (- (Variables|/Game/Blueprints/Player/BP_Player.BP_Player_C|GetMaxIngrediantCarry _as_bp_player_2) 1)))
    (:1
      (Default|GymAdsEvent (Variables|/Game/Blueprints/Widget/WG_HUD.WG_HUD_C|GetWG_Inventory_1 (Variables|/Game/Blueprints/GameManager/BP_GameManager.BP_GameManager_C|GetHUD_Ref (Variables|/Game/Blueprints/Player/BP_Player.BP_Player_C|GetRef%20Game%20Manager (Variables|Default|GetAs%20BP%20Player)))) (Variables|/Game/Blueprints/Player/BP_Player.BP_Player_C|Getid_controler _as_bp_player) (Variables|Default|GetOpacity) (- (Variables|/Game/Blueprints/Player/BP_Player.BP_Player_C|GetMaxIngrediantCarry _as_bp_player) 1)))))

(event EventBeginPlay
  (CallFunction|CarryLess))

(event EventTick
  (params (DeltaSeconds :type Float%20%28single-precision%29)))