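; Three-lane fairy tale road hazard that spawns BP_FaryTale_Danger actors on left, center and right splines.
; At BeginPlay it caches pattern and danger DataTables, then spawns three timed dangers from random pattern picks, repeating while CanContinue is set.
; Each danger starts at its spline's first point with mesh, material, size and direction; the speed input goes unused.
; When IsMesh is set, the construction script tiles collision-free spline meshes along all three lanes.
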(event Custom|Event_Spawn%20Patern
  (bind _storage_dangerpatern (Variables|Default|GetStorage_DangerPatern))
  (bind _outitem (Utilities|Array|Random _storage_dangerpatern))
  (CallFunction|FunctionSomthingGo (.danger_1 _outitem) (.d1_line _outitem) (.d1_speed _outitem) (.d1_direction _outitem))
  (Utilities|FlowControl|Delay (.d1_delay _outitem))
  (CallFunction|FunctionSomthingGo (.danger_2 _outitem) (.d2_line _outitem) (.d2_speed _outitem) (.d2_direction _outitem))
  (Utilities|FlowControl|Delay (.d2_delay _outitem))
  (CallFunction|FunctionSomthingGo (.danger_3 _outitem) (.d3_line _outitem) (.d3_speed _outitem) (.d3_direction _outitem))
  (Utilities|FlowControl|Delay (Math|Random|RandomFloatinRange 4.0 6.0))
  (if (Variables|Default|GetCan%20continue)
    (CallFunction|EventSpawnPatern)))

(event Custom|Event_GetDanger
  (bind _outrownames (DataTable|GetDataTableRowNames "/Game/Blueprints/Structures_Data/DT_FairyTale_Danger.DT_FairyTale_Danger"))
  (for _array_element _outrownames
    (bind _returnvalue (Utilities|GetDataTableRow "/Game/Blueprints/Structures_Data/DT_FairyTale_Danger.DT_FairyTale_Danger" _array_element)
      (:then
        (Utilities|Map|Add (Variables|Default|GetStorage_Danger) (.name _returnvalue) (Utilities|Struct|MakeSTR_FairyTale_Danger (.name _returnvalue) (.mesh _returnvalue) (.material _returnvalue) (.isbig _returnvalue)))))))

(event Custom|Event_GetPatern
  (bind _outrownames (DataTable|GetDataTableRowNames "/Game/Blueprints/Structures_Data/DT_FairyTale_DangerPatern.DT_FairyTale_DangerPatern"))
  (for _array_element _outrownames
    (bind _returnvalue (Utilities|GetDataTableRow "/Game/Blueprints/Structures_Data/DT_FairyTale_DangerPatern.DT_FairyTale_DangerPatern" _array_element)
      (:then
        (Utilities|Array|Add (Variables|Default|GetStorage_DangerPatern) _returnvalue)))))

(event EventBeginPlay
  (CallFunction|EventGetPatern)
  (CallFunction|EventGetDanger)
  (CallFunction|EventSpawnPatern))

(fn ConstructionScript
  (bind _meshonspline (Variables|Default|GetMeshOnSpline))
  (bind _returnvalue (StaticMesh|GetBoundingBox _meshonspline))
  ;[0.15 0.15 0.15 0.5] Do we draw the mesh ?
  (if (Variables|Default|GetIsMesh)
    (Utilities|MacroSetSpline)
    (Utilities|FlowControl|Sequence
      (:then_0
        (bind _output_get (Variables|Default|SetMeshBoundSize (- (.max _returnvalue) (.min _returnvalue))))
        (Variables|Default|SetSectionLenght (+ (.x _output_get) (Variables|Default|GetSectionsRarity))))
      (:then_1
        (for _array_element (Variables|Default|GetCurrentSpline_0)
          ;[0.15 0.15 0.15 0.5] Define the number of mesh that can fit on the spline
          (Variables|Default|SetCurrentSpline _array_element)
          (bind _output_get_2 (Variables|Default|SetNumOfParts (.ReturnValue (Math|Float|Division(WholeandRemainder) (Spline|GetSplineLength (Variables|Default|GetCurrentSpline)) (Variables|Default|GetSectionLenght)))))
          (for _index (range 0 _output_get_2)
            ;[0.15 0.15 0.15 0.5] Define the Starting and ending Position of the current mesh
            (Variables|Default|SetDIstanceStart (+ (* _index (Variables|Default|GetSectionLenght)) (Variables|Default|GetOffset)))
            (Variables|Default|SetDIstanceEnd (+ (+ (* _index (Variables|Default|GetSectionLenght)) (Variables|Default|GetOffset)) (Variables|Default|GetSectionLenght) (Variables|Default|GetOffset)))
            ;[0.15 0.15 0.15 0.5] on the spline
            (bind _returnvalue_2 (AddComponent|AddSplineMeshComponent false))
            (Variables|Default|SetCurrentMesh _returnvalue_2)
            (Components|StaticMesh|SetStaticMesh (Variables|Default|GetCurrentMesh) (Variables|Default|GetMeshOnSpline))
            ;[0.15 0.15 0.15 0.5] Set Start And End Position of the mesh on the spline
            (SplineMesh|SetStartandEnd (Variables|Default|GetCurrentMesh) (Utilities|MacroGroundZto-85 (Spline|GetLocationatDistanceAlongSpline (Variables|Default|GetCurrentSpline) (Variables|Default|GetDIstanceStart) "Local")) (Utilities|MacroGroundZto-85 (Math|Vector|ClampVectorSize (Spline|GetTangentatDistanceAlongSpline (Variables|Default|GetCurrentSpline) (Variables|Default|GetDIstanceStart) "Local") 0.0 (Variables|Default|GetSectionLenght))) (Utilities|MacroGroundZto-85 (Spline|GetLocationatDistanceAlongSpline (Variables|Default|GetCurrentSpline) (Variables|Default|GetDIstanceEnd) "Local")) (Utilities|MacroGroundZto-85 (Math|Vector|ClampVectorSize (Spline|GetTangentatDistanceAlongSpline (Variables|Default|GetCurrentSpline) (Variables|Default|GetDIstanceEnd) "Local") 0.0 (Variables|Default|GetSectionLenght))) false :!class /Script/Engine.SplineMeshComponent)
            ;[0.15 0.15 0.15 0.5] Set Rotation at the Start of the Mesh (in Radians)
            (Class|SplineMeshComponent|SetStartRoll (Variables|Default|GetCurrentMesh) (Math|Trig|DegreesToRadians (.Roll (Math|Rotator|BreakRotator (Spline|GetRotationatDistanceAlongSpline (Variables|Default|GetCurrentSpline) (Variables|Default|GetDIstanceStart) "Local")))) false)
            ;[0.15 0.15 0.15 0.5] Set Rotation at the End of the Mesh (in Radians)
            (Class|SplineMeshComponent|SetEndRoll (Variables|Default|GetCurrentMesh) (Math|Trig|DegreesToRadians (.Roll (Math|Rotator|BreakRotator (Spline|GetRotationatDistanceAlongSpline (Variables|Default|GetCurrentSpline) (Variables|Default|GetDIstanceEnd) "Local")))) false)
            ;[0.15 0.15 0.15 0.5] Set Scale at the Start of the Mesh
            (SplineMesh|SetStartScale (Variables|Default|GetCurrentMesh) (Math|Vector2D|MakeVector2D (.y (Class|SplineComponent|GetScaleatDistanceAlongSpline (Variables|Default|GetCurrentSpline) (Variables|Default|GetDIstanceStart))) (.z (Class|SplineComponent|GetScaleatDistanceAlongSpline (Variables|Default|GetCurrentSpline) (Variables|Default|GetDIstanceStart)))) false :!class /Script/Engine.SplineMeshComponent)
            ;[0.15 0.15 0.15 0.5] Set Scale at the end of the Mesh
            (SplineMesh|SetEndScale (Variables|Default|GetCurrentMesh) (Math|Vector2D|MakeVector2D (.y (Class|SplineComponent|GetScaleatDistanceAlongSpline (Variables|Default|GetCurrentSpline) (Variables|Default|GetDIstanceEnd))) (.z (Class|SplineComponent|GetScaleatDistanceAlongSpline (Variables|Default|GetCurrentSpline) (Variables|Default|GetDIstanceEnd)))) true :!class /Script/Engine.SplineMeshComponent)
            ;[0.15 0.15 0.15 0.5] Set Collision
            (Collision|SetCollisionEnabled (Variables|Default|GetCurrentMesh) "NoCollision")))))))

(fn FunctionSomthingGo
  (params (Danger_Type :type E_DangerCaracterisitc%20Enum :default "NewEnumerator0") (Line :type Integer) (Speeed :type E_DangerSpeed%20Enum :default "NewEnumerator0") (Direction :type Boolean))
  (switch int Line
    (:0
      (Utilities|MaSpawnDanger (Variables|Default|GetLeft_Spline) Danger_Type Direction))
    (:1
      (Utilities|MaSpawnDanger (Variables|Default|GetCenter_Spline) Danger_Type Direction))
    (:2
      (Utilities|MaSpawnDanger (Variables|Default|GetRight_Spline) Danger_Type Direction))))