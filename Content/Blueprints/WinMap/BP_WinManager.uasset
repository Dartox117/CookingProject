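; BP_WinManager is the actor that runs the end-of-match win screen.
; On BeginPlay it registers itself with BP_GameInstance, waits a tick, then makes itself player 0's view target.
; It then shows WG_Win, passing in the winner and both players' scores from the game instance.
; A WinMenu event, called from outside this graph, adds the WG_WinAfter widget and switches input to UI only.
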(event Custom|WinMenu
  (bind _returnvalue (UserInterface|CreateWidget "/Game/Blueprints/Widget/WG_WinAfter.WG_WinAfter_C"))
  (UserInterface|Viewport|AddtoViewport _returnvalue 0)
  (Input|SetInputModeUIOnly (Game|GetPlayerController 0) 0 "DoNotLock" false))

(event EventBeginPlay
  (bind _asbp_game_instance (Utilities|Casting|CastToBP_GameInstance (Game|GetGameInstance)))
  (bind _output_get (Variables|Default|SetAs%20BP%20Game%20Instance _asbp_game_instance))
  (Variables|/Game/Blueprints/GameInstance/BP_GameInstance.BP_GameInstance_C|SetWinManagerRef _output_get self)
  (Utilities|FlowControl|DelayUntilNextTick)
  (Game|Player|SetViewTargetwithBlend (Game|GetPlayerController 0) self 0.0 "VTBlend_Linear" 0.0 false)
  (bind _returnvalue (UserInterface|CreateWidget "/Game/Blueprints/Widget/WG_Win.WG_Win_C"))
  (UserInterface|Viewport|AddtoViewport _returnvalue 0)
  (Default|AffichageWin _returnvalue (Variables|/Game/Blueprints/GameInstance/BP_GameInstance.BP_GameInstance_C|GetPlayerWin (Variables|Default|GetAs%20BP%20Game%20Instance)) (Variables|/Game/Blueprints/GameInstance/BP_GameInstance.BP_GameInstance_C|GetP1Score (Variables|Default|GetAs%20BP%20Game%20Instance)) (Variables|/Game/Blueprints/GameInstance/BP_GameInstance.BP_GameInstance_C|GetP2Score (Variables|Default|GetAs%20BP%20Game%20Instance))))

(event Collision|EventActorBeginOverlap
  (params (OtherActor :type Actor%20Object%20Reference)))

(event EventTick
  (params (DeltaSeconds :type Float%20%28single-precision%29)))

(fn ConstructionScript)