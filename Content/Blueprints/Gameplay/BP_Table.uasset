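; Table actor that holds one food ingredient a player sets down and lets only that player take it back.
; FoodInterract calls GetFood when the table is free and the player has food, moving their last carried ingredient onto the table mesh and refreshing their inventory.
; When occupied, it returns the stored food only if the placer's identifier matches and they have carrying room, then clears the table.
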(event Custom|GetFood
  (bind _player_ref (Variables|Default|GetPlayer%20Ref))
  (bind _structureinfoarray (Variables|/Game/Blueprints/Player/BP_Player.BP_Player_C|GetStructureInfoArray _player_ref))
  (bind _returnvalue (Utilities|Array|LastIndex _structureinfoarray))
  (bind _output (Utilities|Array|Get(acopy) _structureinfoarray _returnvalue))
  ;[0.15 0.15 0.15 0.5] Recupere l'info de l'ingrediant et l'enleve au joueur
  (Components|StaticMesh|SetStaticMesh (Utilities|Array|Get(acopy) (Variables|/Game/Blueprints/Player/BP_Player.BP_Player_C|GetStaticmesh_Array (Variables|Default|GetPlayer%20Ref)) (Utilities|Array|LastIndex (Variables|/Game/Blueprints/Player/BP_Player.BP_Player_C|GetStructureInfoArray (Variables|Default|GetPlayer%20Ref)))) 0)
  (Variables|Default|SetUsed true)
  (Variables|Default|SetFoodOn _output)
  (Components|StaticMesh|SetStaticMesh (Variables|Default|GetFood) (.StaticMesh (Utilities|Struct|BreakST_Foods _output)))
  (Utilities|Array|RemoveItem _structureinfoarray _output)
  (Default|SetInventory (Variables|Default|GetPlayer%20Ref))
  (Variables|Default|SetPlayerUsed (Variables|Default|GetPlayer%20Check)))

(event EventBeginPlay)

(event Collision|EventActorBeginOverlap
  (params (OtherActor :type Actor%20Object%20Reference)))

(event EventTick
  (params (DeltaSeconds :type Float%20%28single-precision%29)))

(event EventFoodInterract
  (params (PlayerRef :type BP%20Player%20Object%20Reference) (PlayerCheck :type Integer) (HasFood :type Boolean))
  (Variables|Default|SetPlayer%20Check PlayerCheck)
  (Variables|Default|SetPlayer%20Ref PlayerRef)
  (if (and HasFood (not (Variables|Default|GetUsed)))
    (CallFunction|GetFood)
    (else
      ;[0.15 0.15 0.15 0.5] Redonne l'ingredient au joueur qui l'a posé
      (if (and (Variables|Default|GetUsed) (== (Variables|Default|GetPlayerUsed) (Variables|Default|GetPlayer%20Check)))
        (if (< (Utilities|Array|Length (Variables|/Game/Blueprints/Player/BP_Player.BP_Player_C|GetStructureInfoArray (Variables|Default|GetPlayer%20Ref))) (Variables|/Game/Blueprints/Player/BP_Player.BP_Player_C|GetMaxIngrediantCarry (Variables|Default|GetPlayer%20Ref)))
          (Default|AddFood (Variables|Default|GetPlayer%20Ref) (Variables|Default|GetFoodOn))
          (Components|StaticMesh|SetStaticMesh (Variables|Default|GetFood) 0)
          (Variables|Default|SetUsed false))))))

(fn ConstructionScript)