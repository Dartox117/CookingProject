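; SpawnMenu is a menu manager actor that opens the title screen when play begins.
; On BeginPlay it registers itself as MenuManagerRef on BP_GameInstance, adds the WG_TitleScreen widget to the viewport and sets Game and UI input mode.
; Its CharacterChoseCam event blends the player's view to this actor, apparently for character selection.
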(event Custom|CharacterChoseCam
  (Game|Player|SetViewTargetwithBlend (Game|GetPlayerController 0) self 0.5 "VTBlend_Linear" 0.0 false))

(event EventBeginPlay
  (bind _asbp_game_instance (Utilities|Casting|CastToBP_GameInstance (Game|GetGameInstance)))
  (Variables|/Game/Blueprints/GameInstance/BP_GameInstance.BP_GameInstance_C|SetMenuManager_Ref _asbp_game_instance self)
  (bind _returnvalue (UserInterface|CreateWidget "/Game/Blueprints/Widget/Menu/WG_TitleScreen.WG_TitleScreen_C"))
  (UserInterface|Viewport|AddtoViewport _returnvalue 0)
  (Input|SetInputModeGameandUI (Game|GetPlayerController 0) 0 "LockOnCapture" false false))

(event Collision|EventActorBeginOverlap
  (params (OtherActor :type Actor%20Object%20Reference)))

(event EventTick
  (params (DeltaSeconds :type Float%20%28single-precision%29)))

(fn ConstructionScript)