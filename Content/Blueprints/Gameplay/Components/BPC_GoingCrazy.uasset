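; BPC_GoingCrazy is a player component that grants a temporary speed and dash power boost.
; On BeginPlay it casts its owner to BP_Player, multiplies Speed and DashPower, and activates the Niagara speed effect.
; MaxWalkSpeed multiplies the already boosted Speed again, compounding the bonus.
; DestroySelf, not called within this file, restores base speed, divides dash power back, stops the effect and destroys the component.
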(event Custom|DestroySelf
  (bind _as_bp_player (Variables|Default|GetAs%20BP%20Player))
  (bind _as_bp_player_2 (Variables|Default|GetAs%20BP%20Player))
  ;[0.15 0.15 0.15 0.5] Redonne Les bonnes stats au joueurs
  (bind _output_get (Variables|/Game/Blueprints/Player/BP_Player.BP_Player_C|SetSpeed _as_bp_player_2 (Variables|/Game/Blueprints/Player/BP_Player.BP_Player_C|GetBaseSpeed _as_bp_player_2)))
  (Variables|/Script/Engine.CharacterMovementComponent|SetMaxWalkSpeed (Variables|/Script/Engine.Character|GetCharacterMovement _as_bp_player_2) _output_get)
  (Variables|/Game/Blueprints/Player/BP_Player.BP_Player_C|SetDashPower _as_bp_player (/ (Variables|/Game/Blueprints/Player/BP_Player.BP_Player_C|GetDashPower _as_bp_player) 1.5))
  (Components|Activation|Deactivate (Variables|/Game/Blueprints/Player/BP_Player.BP_Player_C|GetNG_SpeedEffect (Variables|Default|GetAs%20BP%20Player)))
  (Components|DestroyComponent))

(event Custom|SpeedBonus
  ;[0.15 0.15 0.15 0.5] Augmente la puissance du dash ainsi que de la speed
  (bind _asbp_player (Utilities|Casting|CastToBP_Player (Components|GetOwner)))
  (bind _output_get (Variables|Default|SetAs%20BP%20Player _asbp_player))
  (Variables|/Game/Blueprints/Player/BP_Player.BP_Player_C|SetSpeed _output_get (* (Variables|/Game/Blueprints/Player/BP_Player.BP_Player_C|GetSpeed _asbp_player) 1.5))
  (Variables|/Script/Engine.CharacterMovementComponent|SetMaxWalkSpeed (Variables|/Script/Engine.Character|GetCharacterMovement _asbp_player) (* (Variables|/Game/Blueprints/Player/BP_Player.BP_Player_C|GetSpeed _asbp_player) 1.5))
  (Variables|/Game/Blueprints/Player/BP_Player.BP_Player_C|SetDashPower (Variables|Default|GetAs%20BP%20Player) (* (Variables|/Game/Blueprints/Player/BP_Player.BP_Player_C|GetDashPower (Variables|Default|GetAs%20BP%20Player)) 1.5))
  (Components|Activation|Activate (Variables|/Game/Blueprints/Player/BP_Player.BP_Player_C|GetNG_SpeedEffect (Variables|Default|GetAs%20BP%20Player)) true))

(event EventBeginPlay
  (CallFunction|SpeedBonus))

(event EventTick
  (params (DeltaSeconds :type Float%20%28single-precision%29)))