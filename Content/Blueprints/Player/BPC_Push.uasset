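; BPC_Push is a player component that lets a BP_Player shove other players or press active buttons on push input.
; When the owner is not cooking, stunned or holding food, a forward sphere trace finds the target, with debug drawing left on.
; A hit player is launched away with an effect and starts the cooldown, while an active BP_Button receives EventPush without one.
; A timed flag drives the push animation.
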(event Custom|PushStopAnim
  (Utilities|FlowControl|Delay (Variables|Default|GetAnimationLenght))
  (Variables|Default|SetPushAnimationReady false))

(event Custom|PushColdown
  (Variables|Default|SetCanPush? false)
  (Utilities|FlowControl|Delay (Variables|Default|GetPush_Coldown))
  (Variables|Default|SetCanPush? true))

(event Input|EnhancedActionEvents|EnhancedInputActionIA_Push
  (params (ActionValue :type Boolean) (ElapsedSeconds :type Float%20%28double-precision%29) (TriggeredSeconds :type Float%20%28double-precision%29) (InputAction :type Input%20Action%20Object%20Reference :default "/Game/Input/Input_Actions/IA_Push.IA_Push"))
  (bind _ref_owner (Variables|Default|GetRef_Owner))
  (bind _ref_owner_2 (Variables|Default|GetRef_Owner))
  (bind _capsulecomponent (Variables|/Script/Engine.Character|GetCapsuleComponent _ref_owner_2))
  (bind _returnvalue (Transformation|GetWorldLocation _capsulecomponent))
  (:Started
    (if (Math|Boolean|ANDBoolean (Variables|Default|GetCanPush?) (not (Variables|/Game/Blueprints/Player/BP_Player.BP_Player_C|GetIsCooking _ref_owner)) (not (Variables|/Game/Blueprints/Player/BP_Player.BP_Player_C|GetIsStunned _ref_owner)) (not (Variables|/Game/Blueprints/Player/BP_Player.BP_Player_C|GetHasFood (Variables|Default|GetRef_Owner))))
      (Variables|Default|SetPushAnimationReady true)
      (Utilities|FlowControl|Sequence
        (:then_0
          (bind _outhit (Collision|SphereTraceByChannel (+ (* (Variables|Default|GetPush_Offset) (Math|Vector|GetForwardVector (Variables|/Script/Engine.Character|GetCapsuleComponent (Variables|Default|GetRef_Owner)))) _returnvalue) (+ _returnvalue (* (Math|Vector|GetForwardVector (Variables|/Script/Engine.Character|GetCapsuleComponent (Variables|Default|GetRef_Owner))) (Variables|Default|GetPush_Range))) 5e+01 "TraceTypeQuery1" false 0 "ForDuration" true "(R=1.000000,G=0.000000,B=0.000000,A=1.000000)" "(R=0.000000,G=1.000000,B=0.000000,A=1.000000)" 3.0))
          (bind _asbp_player (Utilities|Casting|CastToBP_Player (.hitactor _outhit))
            (:then
              (bind _output_get (Variables|Default|SetRef_Target _asbp_player))
              (Components|Activation|Activate (Variables|/Game/Blueprints/Player/BP_Player.BP_Player_C|GetNG_Push _output_get) true)
              (Character|LaunchCharacter (Variables|Default|GetRef_Target) (Math|Vector|MakeVector (.x (* (Math|Vector|GetUnitDirection(Vector) (Transformation|GetWorldLocation (Variables|/Script/Engine.Character|GetCapsuleComponent (Variables|Default|GetRef_Owner))) (Transformation|GetWorldLocation (Variables|/Script/Engine.Character|GetCapsuleComponent (Variables|Default|GetRef_Target)))) (Variables|Default|GetPush_Power))) (.y (* (Math|Vector|GetUnitDirection(Vector) (Transformation|GetWorldLocation (Variables|/Script/Engine.Character|GetCapsuleComponent (Variables|Default|GetRef_Owner))) (Transformation|GetWorldLocation (Variables|/Script/Engine.Character|GetCapsuleComponent (Variables|Default|GetRef_Target)))) (Variables|Default|GetPush_Power))) 0.0) false true)
              (CallFunction|PushColdown))
            (:CastFailed
              (bind _asbp_button (Utilities|Casting|CastToBP_Button (.hitactor _outhit)))
              (if (Variables|/Game/Blueprints/Gameplay/BP_Button.BP_Button_C|GetActive? _asbp_button)
                (Default|EventPush _asbp_button)))))
        (:then_1
          (CallFunction|PushStopAnim))))))

(event EventBeginPlay
  (Variables|Default|SetRef_Owner (.AsBP%20Player (Utilities|Casting|CastToBP_Player (Components|GetOwner)))))