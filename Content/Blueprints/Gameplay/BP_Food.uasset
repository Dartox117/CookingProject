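; BP_Food is a food pickup that rides a spline conveyor, driven by the game manager's conveyor event.
; On spawn it sets its mesh, or a gift for surprise food, and certain alterations triple or divide its points.
; Alterations also set overlay, Niagara VFX and a spinning type token, which surprise mode masks.
; Players with spare carry space see an outline and prompt; interacting adds the food and destroys the actor.
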(event Custom|Event_Destroy_Self
  ;[0.08333 0 0 0.5] Destruction
  (Actor|DestroyActor))

(event Custom|Event_InitialSetting
  ;[0.15 0.15 0.15 0.5] Setting
  (Components|StaticMesh|SetStaticMesh (Variables|Default|GetFood_Mesh) (.staticmesh (Variables|Setting|GetFood_Information))))

(event EventBeginPlay
  (bind _ref_gamemanager (Utilities|GetGameManager))
  ;[0.06545 1 0 0.5] Begin Play
  (CallFunction|EventInitialSetting)
  ;;[0 0 0] Bind Food Mouvement
  (EventDispatchers|BindEventtoEDCallConveyor _ref_gamemanager (EventDispatchers|CreateEvent :!event Custom|Event_Mouv_AlongSpline))
  (Utilities|SetStaticMeshOverlay)
  (if (Variables|/Game/Blueprints/GameManager/BP_GameManager.BP_GameManager_C|GetIsSurpriseFood _ref_gamemanager)
    (Components|StaticMesh|SetStaticMesh (Variables|Default|GetFood_Mesh) "/Game/Art/Meshes/Food/Ingredient/Gift.Gift"))
  (if (Utilities|Enum|Equal(Enum) (Variables|Setting|GetAlterationSelected) "NewEnumerator1")
    (bind _structout (Utilities|Struct|SetmembersinST_Foods (Variables|Setting|GetFood_Information) (* (.Points (Utilities|Struct|BreakST_Foods (Variables|Setting|GetFood_Information))) 3)))
    (Variables|Setting|SetFood_Information _structout)
    (elif (Utilities|Enum|Equal(Enum) (Variables|Setting|GetAlterationSelected) "NewEnumerator18")
      (bind _structout_2 (Utilities|Struct|SetmembersinST_Foods (Variables|Setting|GetFood_Information) (/ (.Points (Utilities|Struct|BreakST_Foods (Variables|Setting|GetFood_Information))) 3)))
      (Variables|Setting|SetFood_Information _structout_2))))

(event EventTick
  (params (DeltaSeconds :type Float%20%28single-precision%29))
  (Transformation|AddLocalRotation (Variables|Default|GetSM_Alt-Token) "0.000000,-1.500000,0.000000" false false))

(event EventOverlay
  (params (playerRef :type BP%20Player%20Object%20Reference))
  ;[0 0.1396 0.15 0.5] ChangeOverlay Material
  (if (and (not (Variables|Default|GetHasOverlay)) (< (Utilities|Array|Length (Variables|/Game/Blueprints/Player/BP_Player.BP_Player_C|GetStructureInfoArray playerRef)) (Variables|/Game/Blueprints/Player/BP_Player.BP_Player_C|GetMaxIngrediantCarry playerRef)))
    (Variables|Default|SetBaseOverlay (Rendering|Material|GetOverlayMaterial (Variables|Default|GetFood_Mesh) :!class /Script/Engine.MeshComponent))
    (Rendering|Material|SetOverlayMaterial (Variables|Default|GetFood_Mesh) "/Game/Art/Materials/Shader/Outline/MI_Outline_White.MI_Outline_White" :!class /Script/Engine.MeshComponent)
    (Variables|Default|SetHasOverlay true)
    (Rendering|SetVisibility (Variables|Default|GetInteract) true false)
    (else
      (Rendering|Material|SetOverlayMaterial (Variables|Default|GetFood_Mesh) (Variables|Default|GetBaseOverlay) :!class /Script/Engine.MeshComponent)
      (Variables|Default|SetHasOverlay false)
      (Rendering|SetVisibility (Variables|Default|GetInteract) false false))))

(event EventFoodInterract
  (params (PlayerRef :type BP%20Player%20Object%20Reference) (PlayerCheck :type Integer) (HasFood :type Boolean))
  ;[1 0.4123 0 0.5] Food Pick Up
  ;;[0.15 0.15 0.15 0.5] Verif de si le joueur peut prendre un aliment, si oui, alors l'aliment s'ajoute au player et se delete
  (Variables|Reference|SetRef_Player PlayerRef)
  (if (< (Utilities|Array|Length (Variables|/Game/Blueprints/Player/BP_Player.BP_Player_C|GetStructureInfoArray PlayerRef)) (Variables|/Game/Blueprints/Player/BP_Player.BP_Player_C|GetMaxIngrediantCarry PlayerRef))
    (Default|AddFood (Variables|Reference|GetRef_Player) (Variables|Setting|GetFood_Information))
    (Actor|DestroyActor)))

(event Custom|Event_Mouv_AlongSpline
  (params (Speed :type Float%20%28double-precision%29))
  (Variables|Default|SetSplineProgression (+ (Variables|Default|GetSplineProgression) Speed))
  (Transformation|SetActorTransform (Math|Transform|MakeTransform (Math|Vector|MakeVector (.x (Spline|GetLocationatDistanceAlongSpline (Variables|/Game/Blueprints/Gameplay/BP_TapisQuiRoule.BP_TapisQuiRoule_C|GetSpline_Path (Variables|Reference|GetRef_Path)) (Math|Float|Lerp 0.0 (Spline|GetSplineLength (Variables|/Game/Blueprints/Gameplay/BP_TapisQuiRoule.BP_TapisQuiRoule_C|GetSpline_Path (Variables|Reference|GetRef_Path))) (Variables|Default|GetSplineProgression)) "World")) (.y (Spline|GetLocationatDistanceAlongSpline (Variables|/Game/Blueprints/Gameplay/BP_TapisQuiRoule.BP_TapisQuiRoule_C|GetSpline_Path (Variables|Reference|GetRef_Path)) (Math|Float|Lerp 0.0 (Spline|GetSplineLength (Variables|/Game/Blueprints/Gameplay/BP_TapisQuiRoule.BP_TapisQuiRoule_C|GetSpline_Path (Variables|Reference|GetRef_Path))) (Variables|Default|GetSplineProgression)) "World")) (+ (.z (Spline|GetLocationatDistanceAlongSpline (Variables|/Game/Blueprints/Gameplay/BP_TapisQuiRoule.BP_TapisQuiRoule_C|GetSpline_Path (Variables|Reference|GetRef_Path)) (Math|Float|Lerp 0.0 (Spline|GetSplineLength (Variables|/Game/Blueprints/Gameplay/BP_TapisQuiRoule.BP_TapisQuiRoule_C|GetSpline_Path (Variables|Reference|GetRef_Path))) (Variables|Default|GetSplineProgression)) "World")) 25.0)) (Spline|GetRotationatDistanceAlongSpline (Variables|/Game/Blueprints/Gameplay/BP_TapisQuiRoule.BP_TapisQuiRoule_C|GetSpline_Path (Variables|Reference|GetRef_Path)) (Math|Float|Lerp 0.0 (Spline|GetSplineLength (Variables|/Game/Blueprints/Gameplay/BP_TapisQuiRoule.BP_TapisQuiRoule_C|GetSpline_Path (Variables|Reference|GetRef_Path))) (Variables|Default|GetSplineProgression)) "World") (.scale (Transformation|GetActorTransform))) true))

(fn ConstructionScript)