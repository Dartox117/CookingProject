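; BP_Screen is a screen actor that briefly shows a random dish image, then returns to black.
; On BeginPlay it creates a dynamic material instance from M_ImageScreen1 and applies it to element 2 of the Screen mesh.
; ChangeImage picks one of four textures from DishTextureArray, sets it on the ImageScreen parameter, and swaps back to the black texture after a short delay.
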(event Custom|ChangeImage
  ;[0.15 0.15 0.15 0.5] Change l'image sur un random puis reaffiche l'écran noir
  (Variables|Default|SetDish_texture (Utilities|Array|Get(acopy) (Variables|Default|GetDish_Texture_Array) (Math|Random|RandomIntegerinRange 0 3)))
  (Rendering|Material|SetTextureParameterValue (Variables|Default|GetMaterial_Instance) "ImageScreen" (Variables|Default|GetDish_texture))
  (Utilities|FlowControl|Delay 2.5)
  (Rendering|Material|SetTextureParameterValue (Variables|Default|GetMaterial_Instance) "ImageScreen" "/Game/Art/Textures/2D/T_BlakcScreen.T_BlakcScreen"))

(event EventBeginPlay
  (bind _screen (Variables|Default|GetScreen))
  ;[0.15 0.15 0.15 0.5] Creation du dynamic material instance et set sur le material du mesh
  (bind _returnvalue (Rendering|Material|CreateDynamicMaterialInstance _screen 2 "/Game/Art/Materials/2D/M_ImageScreen1.M_ImageScreen1" "None" :!class /Script/Engine.PrimitiveComponent))
  (bind _output_get (Variables|Default|SetMaterial_Instance _returnvalue))
  (Rendering|Material|SetMaterial _screen 2 _output_get))

(event Collision|EventActorBeginOverlap
  (params (OtherActor :type Actor%20Object%20Reference)))

(event EventTick
  (params (DeltaSeconds :type Float%20%28single-precision%29)))

(fn ConstructionScript)