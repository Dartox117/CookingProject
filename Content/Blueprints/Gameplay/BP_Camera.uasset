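; Shared two-player camera that registers with the game instance and becomes player one's view target at game start.
; After a startup delay, Tick eases the FOV toward FOVCalcul's result, whose helper nodes derive zoom from player distance.
; A flag from that function switches between moving toward the players' midpoint, with clamped X, and returning to the base position.
; CaptureEnd triggers a scene capture.
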(event Custom|CaptureEnd
  (Rendering|SceneCapture|CaptureScene (Variables|Default|GetSceneCaptureComponent2D) :!class /Script/Engine.SceneCaptureComponent2D))

(event EventBeginPlay
  (bind _returnvalue (Transformation|GetActorLocation))
  ;[0.15 0.15 0.15 0.5] Set la camera en debut de jeu
  (Utilities|FlowControl|Delay 0.01)
  (bind _asbp_game_instance (Utilities|Casting|CastToBP_GameInstance (Game|GetGameInstance)))
  (Variables|/Game/Blueprints/GameInstance/BP_GameInstance.BP_GameInstance_C|SetCamera _asbp_game_instance self)
  (Game|Player|SetViewTargetwithBlend (Game|GetPlayerController 0) self 0.0 "VTBlend_Linear" 0.0 false)
  (bind _asbp_player (Utilities|Casting|CastToBP_Player (Game|Player|GetPlayerPawn 0)))
  (Variables|Object_References|SetPlayer1_Ref _asbp_player)
  (bind _asbp_player_2 (Utilities|Casting|CastToBP_Player (Game|Player|GetPlayerPawn 1)))
  (Variables|ObjectReferences|SetPlayer2_Ref _asbp_player_2)
  (Variables|Default|SetBaseX (.x _returnvalue))
  (Variables|Default|SetBaseY (.y _returnvalue))
  (Utilities|FlowControl|Delay 5.0)
  (Variables|State|SetCanTick true))

(event Collision|EventActorBeginOverlap
  (params (OtherActor :type Actor%20Object%20Reference)))

(event EventTick
  (params (DeltaSeconds :type Float%20%28single-precision%29))
  (bind _returnvalue (Transformation|GetActorLocation))
  (bind (_newparam _newparam2 _newparam3) (Utilities|MiddlePointBetween))
  (bind (_returnvalue_2 _returnvalue2 _returnvalue_z) (Utilities|CameraBaseTransition))
  (bind (_returnvalue_3 _returnvalue2_2) (Utilities|FOVCalcul))
  ;[0.15 0.15 0.15 0.5] Déplacement de la Caméra
  (Variables|Default|SetDelta%20Seconds DeltaSeconds)
  (if (and (Variables|State|GetCanTick) (Variables|Default|GetCanMove))
    (Camera|SetFieldOfView (Variables|Default|GetCamera) (Math|Interpolation|FInterpTo (Variables|/Script/Engine.CameraComponent|GetFieldOfView (Variables|Default|GetCamera)) _returnvalue_3 (Variables|Default|GetDelta%20Seconds) 1.0))
    (if _returnvalue2_2
      ;;[0.15 0.15 0.15 0.5] Déplacement de la caméra quand les joueurs sont proches
      (Transformation|SetActorLocation (Math|Vector|MakeVector _newparam _newparam2 _newparam3) false false)
      (Transformation|SetActorLocation (Math|Vector|MakeVector (Math|Float|Clamp(Float) (.x _returnvalue) (Variables|Default|GetDown_Minimum%20) (Variables|Default|GetUp_Maximum)) (.y _returnvalue) (.z _returnvalue)) false false)
      (else
        ;;[0.15 0.15 0.15 0.5] La caméra qui revient au centre
        (Transformation|SetActorLocation (Math|Vector|MakeVector _returnvalue_2 _returnvalue2 _returnvalue_z) false false)))))

(fn ConstructionScript)

(fn CameraDistance
  (return 0.0 false))