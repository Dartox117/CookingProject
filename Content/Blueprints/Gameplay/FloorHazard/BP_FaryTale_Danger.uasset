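; Moving floor-hazard actor for the fairy tale danger, which stuns the player when its mesh overlaps their capsule.
; Setup applies the given mesh and material, then starts a timeline played forward or reversed by the Direction flag.
; The Speed mode picks the progression curve; only the Constant branch moves and rotates the actor along the referenced spline.
; The actor destroys itself when the timeline finishes.
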(event OnComponentBeginOverlap(Danger_Mesh)
  (params (OverlappedComponent :type Primitive%20Component%20Object%20Reference) (OtherActor :type Actor%20Object%20Reference) (OtherComp :type Primitive%20Component%20Object%20Reference) (OtherBodyIndex :type Integer) (bFromSweep :type Boolean) (SweepResult :type Hit%20Result%20Structure%20%28by%20ref%29))
  (bind _asbp_player (Utilities|Casting|CastToBP_Player OtherActor))
  (if (== (.AsCapsule%20Collision (Utilities|Casting|CastToCapsuleComponent OtherComp)) (Variables|/Script/Engine.Character|GetCapsuleComponent _asbp_player))
    (Default|FairyTaleStun _asbp_player)))

(event Custom|Event_Go_danger
  (bind _splineref (Variables|Default|GetSplineRef))
  (bind _splineref_2 (Variables|Default|GetSplineRef))
  ;[0.2122 0.1274 0.009134] Moving
  (Components|Timeline|SetPlayRate (Variables|Default|GetTimeline) 0.4)
  (if (Variables|Default|GetDirection)
    (bind (_direction _strait _speeding _sloing) (Timeline|Timeline PlayFromStart)
      (:Update
        (switch Utilities|FlowControl|Switch|SwitchonE_DangerSpeed (Variables|Default|GetSpeed)
          (:NewEnumerator0
            (Variables|Default|SetProgression _strait)
            (Transformation|SetActorLocation (Spline|GetLocationatDistanceAlongSpline _splineref_2 (Math|Float|Lerp 0.0 (Spline|GetSplineLength _splineref_2) (Variables|Default|GetProgression)) "World") true false)
            (Transformation|SetActorRotation (Spline|GetRotationatDistanceAlongSpline _splineref (Math|Float|Lerp 0.0 (Spline|GetSplineLength _splineref) (Variables|Default|GetProgression)) "World")))
          (:NewEnumerator1
            (Variables|Default|SetProgression _speeding))
          (:NewEnumerator2
            (Variables|Default|SetProgression _sloing))))
      (:Finished
        (Actor|DestroyActor)))
    (else
      (Timeline|Timeline ReverseFromEnd))))

(event Custom|Event_Setup
  ;[0 0 0 0.5] Setup
  (Components|StaticMesh|SetStaticMesh (Variables|Default|GetDanger_Mesh) (Variables|Default|GetMesh))
  (Rendering|Material|SetMaterial (Variables|Default|GetDanger_Mesh) 0 (Variables|Default|GetMaterial))
  (CallFunction|EventGoDanger))

(fn ConstructionScript)