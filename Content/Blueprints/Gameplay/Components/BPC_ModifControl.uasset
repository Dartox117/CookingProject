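; Actor component that applies a dizzy control-scrambling effect to the player it is attached to.
; On BeginPlay it checks the owner for BPI_Player, casts it to BP_Player and, unless IsProtected, swaps the WorldDirectionX and WorldDirectionY axes and activates NGDizzy.
; EndEffect, which is not called within this graph, restores both directions, deactivates NGDizzy and destroys the component.
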(event Custom|ModifControl
  (bind _returnvalue (Components|GetOwner))
  (if (Utilities|DoesObjectImplementInterface _returnvalue "/Game/Blueprints/BPI/BPI_Player.BPI_Player_C")
    (bind _asbp_player (Utilities|Casting|CastToBP_Player _returnvalue))
    (bind _output_get (Variables|Default|SetAs%20BP%20Player _asbp_player))
    (if (not (Variables|/Game/Blueprints/Player/BP_Player.BP_Player_C|GetIsProtected _output_get))
      (Variables|/Game/Blueprints/Player/BP_Player.BP_Player_C|SetWorld%20DirectionX (Variables|Default|GetAs%20BP%20Player) "0.000000,1.000000,0.000000")
      (Variables|/Game/Blueprints/Player/BP_Player.BP_Player_C|SetWorld%20DirectionY (Variables|Default|GetAs%20BP%20Player) "1.000000,0.000000,0.000000")
      (Components|Activation|Activate (Variables|/Game/Blueprints/Player/BP_Player.BP_Player_C|GetNG_Dizzy (Variables|Default|GetAs%20BP%20Player)) false))))

(event Custom|EndEffect
  (bind _as_bp_player (Variables|Default|GetAs%20BP%20Player))
  (Variables|/Game/Blueprints/Player/BP_Player.BP_Player_C|SetWorld%20DirectionX _as_bp_player "1.000000,0.000000,0.000000")
  (Variables|/Game/Blueprints/Player/BP_Player.BP_Player_C|SetWorld%20DirectionY _as_bp_player "0.000000,1.000000,0.000000")
  (Components|Activation|Deactivate (Variables|/Game/Blueprints/Player/BP_Player.BP_Player_C|GetNG_Dizzy (Variables|Default|GetAs%20BP%20Player)))
  (Components|DestroyComponent))

(event EventBeginPlay
  (CallFunction|ModifControl))

(event EventTick
  (params (DeltaSeconds :type Float%20%28single-precision%29)))