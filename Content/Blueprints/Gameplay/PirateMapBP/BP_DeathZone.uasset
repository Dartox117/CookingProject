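; Pirate map death zone that oscillates between its starting location and a raised offset, apparently as rising water.
; A timeline lerps the root's position and triggers a wave sound, with 30-second delays and a FlipFlop alternating replay and reverse.
; Players overlapping its box trigger a splash sound, then after a brief delay are killed and have their movement velocity zeroed.
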(event OnComponentBeginOverlap(Box)
  (params (OverlappedComponent :type Primitive%20Component%20Object%20Reference) (OtherActor :type Actor%20Object%20Reference) (OtherComp :type Primitive%20Component%20Object%20Reference) (OtherBodyIndex :type Integer) (bFromSweep :type Boolean) (SweepResult :type Hit%20Result%20Structure%20%28by%20ref%29))
  (if (Utilities|DoesObjectImplementInterface OtherActor "/Game/Blueprints/BPI/BPI_Player.BPI_Player_C")
    (bind _asbp_player (Utilities|Casting|CastToBP_Player OtherActor))
    (Audio|Components|Audio|Play (Variables|Default|GetSC_Splash) 0.0)
    (Utilities|FlowControl|Delay 0.25)
    (Default|Death _asbp_player)
    (Variables|/Script/Engine.MovementComponent|SetVelocity (Variables|/Script/Engine.Character|GetCharacterMovement _asbp_player) "0, 0, 0")))

(event Custom|Reverse%20play
  (bind _newtrack_0 (Timeline|Timeline ReverseFromEnd)
    (:Update
      (Transformation|SetWorldLocation (Variables|Default|GetDefaultSceneRoot) (Math|Vector|Lerp(Vector) (Variables|Default|GetInitail%20position) (Variables|Default|GetUp_Position) _newtrack_0) false false)
      (Audio|Components|Audio|Play (Variables|Default|GetSC_Wave) 0.0)
      (Utilities|FlowControl|Delay 3e+01)
      (Utilities|FlowControl|FlipFlop
        (:A
          (CallFunction|ReversePlay))
        (:B
          (CallFunction|Replay))))))

(event Custom|Replay
  (bind _newtrack_0 (Timeline|Timeline PlayFromStart)
    (:Update
      (Transformation|SetWorldLocation (Variables|Default|GetDefaultSceneRoot) (Math|Vector|Lerp(Vector) (Variables|Default|GetInitail%20position) (Variables|Default|GetUp_Position) _newtrack_0) false false)
      (Audio|Components|Audio|Play (Variables|Default|GetSC_Wave) 0.0)
      (Utilities|FlowControl|Delay 3e+01)
      (Utilities|FlowControl|FlipFlop
        (:A
          (CallFunction|ReversePlay))
        (:B
          (CallFunction|Replay))))))

(event EventBeginPlay
  (Variables|Default|SetInitail%20position (Transformation|GetWorldLocation (Variables|Default|GetDefaultSceneRoot)))
  (Variables|Default|SetUp_Position (+ (Variables|Default|GetInitail%20position) (Variables|Default|GetHight)))
  (Utilities|FlowControl|Delay 3e+01)
  (Components|Timeline|SetPlayRate (Variables|Default|GetTimeline) 1.0)
  (bind _newtrack_0 (Timeline|Timeline PlayFromStart)
    (:Update
      (Transformation|SetWorldLocation (Variables|Default|GetDefaultSceneRoot) (Math|Vector|Lerp(Vector) (Variables|Default|GetInitail%20position) (Variables|Default|GetUp_Position) _newtrack_0) false false)
      (Audio|Components|Audio|Play (Variables|Default|GetSC_Wave) 0.0)
      (Utilities|FlowControl|Delay 3e+01)
      (Utilities|FlowControl|FlipFlop
        (:A
          (CallFunction|ReversePlay))
        (:B
          (CallFunction|Replay))))))

(fn ConstructionScript)