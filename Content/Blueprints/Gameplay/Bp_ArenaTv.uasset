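; Arena TV actor that animates a set piece, moving a list of mesh actors vertically while rotating a linked RotatingSet.
; One timeline drives the height lerp and a 90-degree root rotation, calling MouveTAble on the set each update.
; A looping 20-second timer alternates forward and reverse through the NextStart flag, with the first reversal starting from the end.
; A separate HightJack button event plays or reverses the same timeline based on that flag without changing it.
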(event Custom|Event_Start
  (Variables|Default|SetNextStart? false)
  (bind _transformation (Timeline|Timeline Play)
    (:Update
      (Variables|Default|SetTransformation _transformation)
      (Utilities|FlowControl|Sequence
        (:then_0
          (for _array_element (Variables|Default|GetMeshToTranslate)
            (Transformation|SetActorLocation _array_element (Math|Vector|MakeVector (.x (.location (Transformation|GetActorTransform _array_element))) (.y (.location (Transformation|GetActorTransform _array_element))) (.z (Math|Vector|Lerp(Vector) "-502.000000,0.000000,-3.000000" "0.000000,0.000000,-173.000000" (Variables|Default|GetTransformation)))) false false)))
        (:then_1
          (Transformation|SetWorldRotation (Variables|/Game/Levels/PLAYTEST/RotatingPlateTv.RotatingPlateTv_C|GetSharedRoot (Variables|Default|GetRotatingSet)) (Math|Rotator|Lerp(Rotator) "0, 0, 0" "0.000000,90.000000,0.000000" (Variables|Default|GetTransformation)) false false)
          (Default|MouveTAble (Variables|Default|GetRotatingSet)))))))

(event Custom|Event_Reverse
  (Utilities|FlowControl|Sequence
    (:then_0
      (Utilities|FlowControl|DoOnce false
        (:Completed
          (bind _transformation (Timeline|Timeline ReverseFromEnd)
            (:Update
              (Variables|Default|SetTransformation _transformation)
              (Utilities|FlowControl|Sequence
                (:then_0
                  (for _array_element (Variables|Default|GetMeshToTranslate)
                    (Transformation|SetActorLocation _array_element (Math|Vector|MakeVector (.x (.location (Transformation|GetActorTransform _array_element))) (.y (.location (Transformation|GetActorTransform _array_element))) (.z (Math|Vector|Lerp(Vector) "-502.000000,0.000000,-3.000000" "0.000000,0.000000,-173.000000" (Variables|Default|GetTransformation)))) false false)))
                (:then_1
                  (Transformation|SetWorldRotation (Variables|/Game/Levels/PLAYTEST/RotatingPlateTv.RotatingPlateTv_C|GetSharedRoot (Variables|Default|GetRotatingSet)) (Math|Rotator|Lerp(Rotator) "0, 0, 0" "0.000000,90.000000,0.000000" (Variables|Default|GetTransformation)) false false)
                  (Default|MouveTAble (Variables|Default|GetRotatingSet)))))))))
    (:then_1
      (Variables|Default|SetNextStart? true)
      (Timeline|Timeline Reverse))))

(event Custom|HightJackStart
  (bind _transformation (Timeline|Timeline Play)
    (:Update
      (Variables|Default|SetTransformation _transformation)
      (Utilities|FlowControl|Sequence
        (:then_0
          (for _array_element (Variables|Default|GetMeshToTranslate)
            (Transformation|SetActorLocation _array_element (Math|Vector|MakeVector (.x (.location (Transformation|GetActorTransform _array_element))) (.y (.location (Transformation|GetActorTransform _array_element))) (.z (Math|Vector|Lerp(Vector) "-502.000000,0.000000,-3.000000" "0.000000,0.000000,-173.000000" (Variables|Default|GetTransformation)))) false false)))
        (:then_1
          (Transformation|SetWorldRotation (Variables|/Game/Levels/PLAYTEST/RotatingPlateTv.RotatingPlateTv_C|GetSharedRoot (Variables|Default|GetRotatingSet)) (Math|Rotator|Lerp(Rotator) "0, 0, 0" "0.000000,90.000000,0.000000" (Variables|Default|GetTransformation)) false false)
          (Default|MouveTAble (Variables|Default|GetRotatingSet)))))))

(event Custom|HightJackReverse
  (bind _transformation (Timeline|Timeline Reverse)
    (:Update
      (Variables|Default|SetTransformation _transformation)
      (Utilities|FlowControl|Sequence
        (:then_0
          (for _array_element (Variables|Default|GetMeshToTranslate)
            (Transformation|SetActorLocation _array_element (Math|Vector|MakeVector (.x (.location (Transformation|GetActorTransform _array_element))) (.y (.location (Transformation|GetActorTransform _array_element))) (.z (Math|Vector|Lerp(Vector) "-502.000000,0.000000,-3.000000" "0.000000,0.000000,-173.000000" (Variables|Default|GetTransformation)))) false false)))
        (:then_1
          (Transformation|SetWorldRotation (Variables|/Game/Levels/PLAYTEST/RotatingPlateTv.RotatingPlateTv_C|GetSharedRoot (Variables|Default|GetRotatingSet)) (Math|Rotator|Lerp(Rotator) "0, 0, 0" "0.000000,90.000000,0.000000" (Variables|Default|GetTransformation)) false false)
          (Default|MouveTAble (Variables|Default|GetRotatingSet)))))))

(event Custom|Event_HightJackButton
  (if (Variables|Default|GetNextStart?)
    (CallFunction|HightJackStart)
    (else
      (CallFunction|HightJackReverse))))

(event Custom|PlatformMouve
  (if (Variables|Default|GetNextStart?)
    (CallFunction|EventStart)
    (else
      (CallFunction|EventReverse))))

(event EventBeginPlay
  (Components|Timeline|SetPlayRate (Variables|Default|GetTimeline) 1.0)
  (Utilities|Time|SetTimerbyEvent (delegate Custom|PlatformMouve) 2e+01 true))

(fn ConstructionScript)