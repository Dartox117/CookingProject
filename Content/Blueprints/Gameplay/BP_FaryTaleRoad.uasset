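; BP_FaryTaleRoad is a fairy-tale road that keeps sending hazards along its left, center and right splines.
; On BeginPlay it caches pattern and danger DataTables, then loops delayed waves of three spawns while CanContinue holds.
; Random pattern picks are re-evaluated at each step rather than stored, so waves can mix rows.
; A macro spawns BP_FaryTale_Danger at the spline start with mesh, material, size and direction; pattern speed goes unused.
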(event Custom|Event_Spawn%20Patern
  (bind _storage_dangerpatern (Variables|Default|GetStorage_DangerPatern))
  (bind _outitem (Utilities|Array|Random _storage_dangerpatern))
  (CallFunction|FunctionSomthingGo (.danger_1 _outitem) (.d1_line _outitem) (.d1_speed _outitem) (.d1_direction _outitem))
  (Utilities|FlowControl|Delay (.d1_delay _outitem))
  (CallFunction|FunctionSomthingGo (.danger_2 _outitem) (.d2_line _outitem) (.d2_speed _outitem) (.d2_direction _outitem))
  (Utilities|FlowControl|Delay (.d2_delay _outitem))
  (CallFunction|FunctionSomthingGo (.danger_3 _outitem) (.d3_line _outitem) (.d3_speed _outitem) (.d3_direction _outitem))
  (Utilities|FlowControl|Delay (Math|Random|RandomFloatinRange 4.0 6.0))
  (if (Variables|Default|GetCan%20continue)
    (CallFunction|EventSpawnPatern)))

(event Custom|Event_GetDanger
  (bind _outrownames (DataTable|GetDataTableRowNames "/Game/Blueprints/Gameplay/DT_FairyTale_Danger.DT_FairyTale_Danger"))
  (for _array_element _outrownames
    (bind _returnvalue (Utilities|GetDataTableRow "/Game/Blueprints/Gameplay/DT_FairyTale_Danger.DT_FairyTale_Danger" _array_element)
      (:then
        (Utilities|Map|Add (Variables|Default|GetStorage_Danger) (.name _returnvalue) (Utilities|Struct|MakeSTR_FairyTale_Danger (.name _returnvalue) (.mesh _returnvalue) (.material _returnvalue) (.isbig _returnvalue)))))))

(event Custom|Event_GetPatern
  (bind _outrownames (DataTable|GetDataTableRowNames "/Game/Blueprints/Gameplay/DT_FairyTale_DangerPatern.DT_FairyTale_DangerPatern"))
  (for _array_element _outrownames
    (bind _returnvalue (Utilities|GetDataTableRow "/Game/Blueprints/Gameplay/DT_FairyTale_DangerPatern.DT_FairyTale_DangerPatern" _array_element)
      (:then
        (Utilities|Array|Add (Variables|Default|GetStorage_DangerPatern) _returnvalue)))))

(event EventBeginPlay
  (CallFunction|EventGetPatern)
  (CallFunction|EventGetDanger)
  (CallFunction|EventSpawnPatern))

(fn ConstructionScript)

(fn FunctionSomthingGo
  (params (Danger_Type :type E_DangerCaracterisitc%20Enum :default "NewEnumerator0") (Line :type Integer) (Speeed :type E_DangerSpeed%20Enum :default "NewEnumerator0") (Direction :type Boolean))
  (switch int Line
    (:0
      (Utilities|MaSpawnDanger (Variables|Default|GetLeft_Spline) Danger_Type Direction))
    (:1
      (Utilities|MaSpawnDanger (Variables|Default|GetCenter_Spline) Danger_Type Direction))
    (:2
      (Utilities|MaSpawnDanger (Variables|Default|GetRight_Spline) Danger_Type Direction))))