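; BPC_StrongMan is a player effect component that temporarily raises how many ingredients a BP_Player can carry.
; On BeginPlay it casts its owner to BP_Player, adds two to the clamped carry limit and calls AddInventory on the game manager with full opacity.
; EndEffect lowers the clamped limit by two, sends zero opacity, calls the player's CheckInventory and destroys the component.
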(event Custom|AugmentInventory
  (bind _asbp_player (Utilities|Casting|CastToBP_Player (Components|GetOwner)))
  (Variables|Default|SetAs%20BP%20Player _asbp_player)
  (Variables|/Game/Blueprints/Player/BP_Player.BP_Player_C|SetMaxIngrediantCarry (Variables|Default|GetAs%20BP%20Player) (Math|Integer|Clamp(Integer) (+ (Variables|/Game/Blueprints/Player/BP_Player.BP_Player_C|GetMaxIngrediantCarry (Variables|Default|GetAs%20BP%20Player)) 2) 0 6))
  (Default|AddInventory (Variables|/Game/Blueprints/Player/BP_Player.BP_Player_C|GetRef%20Game%20Manager (Variables|Default|GetAs%20BP%20Player)) (Variables|/Game/Blueprints/Player/BP_Player.BP_Player_C|Getid_controler (Variables|Default|GetAs%20BP%20Player)) 1.0))

(event Custom|EndEffect
  (bind _as_bp_player (Variables|Default|GetAs%20BP%20Player))
  (Variables|/Game/Blueprints/Player/BP_Player.BP_Player_C|SetMaxIngrediantCarry (Variables|Default|GetAs%20BP%20Player) (Math|Integer|Clamp(Integer) (- (Variables|/Game/Blueprints/Player/BP_Player.BP_Player_C|GetMaxIngrediantCarry (Variables|Default|GetAs%20BP%20Player)) 2) 3 6))
  (Default|AddInventory (Variables|/Game/Blueprints/Player/BP_Player.BP_Player_C|GetRef%20Game%20Manager _as_bp_player) (Variables|/Game/Blueprints/Player/BP_Player.BP_Player_C|Getid_controler _as_bp_player) 0.0)
  (Default|CheckInventory (Variables|Default|GetAs%20BP%20Player))
  (Components|DestroyComponent))

(event EventBeginPlay
  (CallFunction|AugmentInventory))

(event EventTick
  (params (DeltaSeconds :type Float%20%28single-precision%29)))