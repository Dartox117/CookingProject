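; Kitchen worktop where a player carrying food cooks it through a gamepad input combo.
; Interacting copies the player's food meshes and data, starts the combo on the GameManager and locks the station.
; SwitchCombo enables the player input flags matching the current food's input code, or ends the combo, resetting the station and briefly freezing the player.
; Separate events relay inputs to the GameManager, toggle the highlight, and play success effects.
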(event Custom|SwitchCombo
  (bind _player_ref (Variables|ObjectRef|GetPlayer%20Ref))
  ;[0.15 0.15 0.15 0.5] Switch le combo à faire pour le joueur
  (Variables|/Game/Blueprints/Player/BP_Player.BP_Player_C|SetBonusInputActive _player_ref true)
  (Default|ResetComboBool _player_ref)
  (if (>= (Variables|Combo|GetComboIndex) (Utilities|Array|Length (Variables|Array|GetStructureArray)))
    (CallFunction|EndCombo)
    (Variables|/Game/Blueprints/Player/BP_Player.BP_Player_C|SetStartCombo (Variables|ObjectRef|GetPlayer%20Ref) false)
    (else
      (Utilities|Time|SetTimerbyEvent (delegate Custom|DeActivateBonusInput) 0.5)
      (CallFunction|InputSelection))))

(event Custom|EndCombo
  ;[0.15 0.15 0.15 0.5] Code pour la réussite d'un combo (reset des variables, envoie des infos à l'hud)
  (Variables|Combo|SetComboIndex 0)
  (for _array_element (Variables|Array|GetPlatArrayMesh)
    (Components|StaticMesh|SetStaticMesh _array_element 0))
  (Default|FinishedCombo (Variables|ObjectRef|GetGameManagerRef) (Variables|/Game/Blueprints/Player/BP_Player.BP_Player_C|Getid_controler (Variables|ObjectRef|GetPlayer%20Ref)))
  (Utilities|Array|Clear (Variables|Array|GetStructureArray))
  (Variables|/Game/Blueprints/Player/BP_Player.BP_Player_C|SetIsCooking (Variables|ObjectRef|GetPlayer%20Ref) false)
  (Variables|State|SetIsUsed false)
  (Default|FreezePlayer (Variables|ObjectRef|GetPlayer%20Ref))
  (Components|Activation|Deactivate (Variables|Default|GetCooking_VFX))
  (Rendering|SetVisibility (Variables|Default|GetFlamme1) false true)
  (Utilities|FlowControl|Delay 1.5)
  (Default|UnFreezePlayer (Variables|ObjectRef|GetPlayer%20Ref)))

(event Custom|DeActivateBonusInput
  ;[0.15 0.15 0.15 0.5] Switch le combo à faire pour le joueur
  (Variables|/Game/Blueprints/Player/BP_Player.BP_Player_C|SetBonusInputActive (Variables|ObjectRef|GetPlayer%20Ref) false))

(event Custom|Event_%20FolowTheArrow
  (params (NewParam :type Transform))
  (Transformation|SetActorTransform NewParam true))

(event Custom|GetInput
  (params (InputValue :type Float%20%28double-precision%29))
  ;[0.15 0.15 0.15 0.5] Recupere l'input et l'envoie
  (Default|GetInput (Variables|ObjectRef|GetGameManagerRef) (Variables|/Game/Blueprints/Player/BP_Player.BP_Player_C|Getid_controler (Variables|ObjectRef|GetPlayer%20Ref)) InputValue))

(event Custom|WrongInput
  ;[0.15 0.15 0.15 0.5] Mauvaise input
  (Default|WrongInput (Variables|ObjectRef|GetGameManagerRef) (Variables|/Game/Blueprints/Player/BP_Player.BP_Player_C|Getid_controler (Variables|ObjectRef|GetPlayer%20Ref))))

(event Custom|SuccesCook
  ;[0.15 0.15 0.15 0.5] SuccesCook
  ;;[0.08203 0.9844 0.9521] POUR CROUSTI
  (Audio|PlaySound2D "/Game/Blueprints/AlterationFeedBack/deltarune-explosion.deltarune-explosion" 1.0 1.0 0.0 0 0)
  (Default|SendSFX (Variables|ObjectRef|GetGameManagerRef) (Variables|ObjectRef|GetPlayer%20Ref) (Variables|Default|GetNS_HommingAttack))
  (Default|MealCompleted (Variables|ObjectRef|GetPlayer%20Ref))
  (Rendering|SetVisibility (Variables|/Game/Blueprints/Player/BP_Player.BP_Player_C|GetPlate (Variables|ObjectRef|GetPlayer%20Ref)) true false)
  (Default|ChangeImage (Variables|ObjectRef|GetBp_ScreenRef) (Variables|/Game/Blueprints/Player/BP_Player.BP_Player_C|GetRenderTextureMaterial (Variables|ObjectRef|GetPlayer%20Ref)))
  (Default|CookEndVFX (Variables|ObjectRef|GetPlayer%20Ref)))

(event EventBeginPlay
  ;[0.15 0.15 0.15 0.5] Créer un tableau des static mesh component
  (Variables|Array|SetPlatArrayMesh (Utilities|Array|MakeArray (Variables|Default|GetFood_1) (Variables|Default|GetFood_2) (Variables|Default|GetFood_3) (Variables|Default|GetFood_4) (Variables|Default|GetFood_5) (Variables|Default|GetFood_6)))
  (Utilities|FlowControl|Delay 0.02)
  (bind _asbp_game_instance (Utilities|Casting|CastToBP_GameInstance (Game|GetGameInstance)))
  (Variables|ObjectRef|SetGameManagerRef (Variables|/Game/Blueprints/GameInstance/BP_GameInstance.BP_GameInstance_C|GetRef_GameManager _asbp_game_instance)))

(event EventOverlay
  (params (playerRef :type BP%20Player%20Object%20Reference))
  ;[0.15 0.15 0.15 0.5] Detection Event
  (if (and (not (Variables|Default|GetHasOverlay)) (> (Utilities|Array|Length (Variables|/Game/Blueprints/Player/BP_Player.BP_Player_C|GetStructureInfoArray playerRef)) 0))
    (Rendering|Material|SetOverlayMaterial (Variables|Default|GetSM_TableMesh) "/Game/Art/Materials/Shader/Outline/MI_Outline_White.MI_Outline_White" :!class /Script/Engine.MeshComponent)
    (Variables|Default|SetHasOverlay true)
    (Rendering|SetVisibility (Variables|Default|GetInteraction) true false)
    (else
      (Rendering|Material|SetOverlayMaterial (Variables|Default|GetSM_TableMesh) "/Game/Art/Materials/Shader/Outline/MI_Outline_Screen.MI_Outline_Screen" :!class /Script/Engine.MeshComponent)
      (Variables|Default|SetHasOverlay false)
      (Rendering|SetVisibility (Variables|Default|GetInteraction) false false))))

(event EventFoodInterract
  (params (PlayerRef :type BP%20Player%20Object%20Reference) (PlayerCheck :type Integer) (HasFood :type Boolean))
  ;[0.15 0.15 0.15 0.5] Récupere les infos des aliments et lance le combo
  (if (and HasFood (not (Variables|State|GetIsUsed)))
    (Variables|ObjectRef|SetPlayer%20Ref PlayerRef)
    (Components|Activation|Activate (Variables|Default|GetCooking_VFX) false)
    (Rendering|SetVisibility (Variables|Default|GetFlamme1) true true)
    (Variables|State|SetIsUsed true)
    (Variables|/Game/Blueprints/Player/BP_Player.BP_Player_C|SetIsCooking (Variables|ObjectRef|GetPlayer%20Ref) true)
    (Variables|Array|SetStructureArray (Variables|/Game/Blueprints/Player/BP_Player.BP_Player_C|GetStructureInfoArray (Variables|ObjectRef|GetPlayer%20Ref)))
    (for (_array_element _array_index) (Variables|/Game/Blueprints/Player/BP_Player.BP_Player_C|GetStaticmesh_Array (Variables|ObjectRef|GetPlayer%20Ref))
      (Components|StaticMesh|SetStaticMesh (Utilities|Array|Get(acopy) (Variables|Array|GetPlatArrayMesh) _array_index) (Variables|/Script/Engine.StaticMeshComponent|GetStaticMesh _array_element)))
    (Variables|/Game/Blueprints/Player/BP_Player.BP_Player_C|SetPlanDeTravailRef (Variables|ObjectRef|GetPlayer%20Ref) self)
    (CallFunction|SwitchCombo)
    (Default|StartCombo (Variables|ObjectRef|GetGameManagerRef) (Variables|/Game/Blueprints/Player/BP_Player.BP_Player_C|Getid_controler (Variables|ObjectRef|GetPlayer%20Ref)) (Variables|Array|GetStructureArray) self)
    (Default|ResetFood (Variables|ObjectRef|GetPlayer%20Ref))
    (Variables|/Game/Blueprints/Player/BP_Player.BP_Player_C|SetStartCombo (Variables|ObjectRef|GetPlayer%20Ref) true)
    (Default|ExhaustVFXEnd (Variables|ObjectRef|GetPlayer%20Ref))))

(event Custom|InputSelection
  (bind _player_ref (Variables|ObjectRef|GetPlayer%20Ref))
  (bind _player_ref_2 (Variables|ObjectRef|GetPlayer%20Ref))
  (bind _player_ref_3 (Variables|ObjectRef|GetPlayer%20Ref))
  (bind _player_ref_4 (Variables|ObjectRef|GetPlayer%20Ref))
  (bind _player_ref_5 (Variables|ObjectRef|GetPlayer%20Ref))
  (bind _player_ref_6 (Variables|ObjectRef|GetPlayer%20Ref))
  (switch int (Utilities|Struct|BreakST_Foods (Utilities|Array|Get(acopy) (Variables|Array|GetStructureArray) (Variables|Combo|GetComboIndex)))
    (:0
      (Variables|/Game/Blueprints/Player/BP_Player.BP_Player_C|SetCanStickUpDownCombo (Variables|ObjectRef|GetPlayer%20Ref) true))
    (:1
      (Variables|/Game/Blueprints/Player/BP_Player.BP_Player_C|SetCanStickLeftRight (Variables|ObjectRef|GetPlayer%20Ref) true))
    (:2
      (Variables|/Game/Blueprints/Player/BP_Player.BP_Player_C|SetCanStickRound (Variables|ObjectRef|GetPlayer%20Ref) true))
    (:3
      (Variables|/Game/Blueprints/Player/BP_Player.BP_Player_C|SetCanStickReverse (Variables|ObjectRef|GetPlayer%20Ref) true))
    (:4
      (Variables|/Game/Blueprints/Player/BP_Player.BP_Player_C|SetCan_ACombo (Variables|ObjectRef|GetPlayer%20Ref) true))
    (:5
      (Variables|/Game/Blueprints/Player/BP_Player.BP_Player_C|SetCanYCombo (Variables|ObjectRef|GetPlayer%20Ref) true))
    (:6
      (Variables|/Game/Blueprints/Player/BP_Player.BP_Player_C|SetCan_XA_Combo _player_ref_5 true)
      (Variables|/Game/Blueprints/Player/BP_Player.BP_Player_C|SetCan_ACombo _player_ref_5 true)
      (Variables|/Game/Blueprints/Player/BP_Player.BP_Player_C|SetCanXCombo _player_ref_5 true))
    (:7
      (Variables|/Game/Blueprints/Player/BP_Player.BP_Player_C|SetCan_ACombo _player_ref_3 true)
      (Variables|/Game/Blueprints/Player/BP_Player.BP_Player_C|SetCanFullButtonCombo _player_ref_3 true))
    (:8
      (Variables|/Game/Blueprints/Player/BP_Player.BP_Player_C|SetCan_L_trigger _player_ref_6 true)
      (Variables|/Game/Blueprints/Player/BP_Player.BP_Player_C|SetCan_R_trigger _player_ref_6 true)
      (Variables|/Game/Blueprints/Player/BP_Player.BP_Player_C|SetCan_Chicken_Combo _player_ref_6 true))
    (:9
      (Variables|/Game/Blueprints/Player/BP_Player.BP_Player_C|SetCan_LB _player_ref_2 true)
      (Variables|/Game/Blueprints/Player/BP_Player.BP_Player_C|SetCan_RB _player_ref_2 true)
      (Variables|/Game/Blueprints/Player/BP_Player.BP_Player_C|SetCan_Beef_Combo _player_ref_2 true))
    (:10
      (Variables|/Game/Blueprints/Player/BP_Player.BP_Player_C|SetCan_LBLT_combo _player_ref_4 true)
      (Variables|/Game/Blueprints/Player/BP_Player.BP_Player_C|SetCan_LB _player_ref_4 true)
      (Variables|/Game/Blueprints/Player/BP_Player.BP_Player_C|SetCan_L_trigger _player_ref_4 true))
    (:11
      (Variables|/Game/Blueprints/Player/BP_Player.BP_Player_C|SetCan_RBRT_combo _player_ref true)
      (Variables|/Game/Blueprints/Player/BP_Player.BP_Player_C|SetCan_RB _player_ref true)
      (Variables|/Game/Blueprints/Player/BP_Player.BP_Player_C|SetCan_R_trigger _player_ref true))
    (:12
      (Variables|/Game/Blueprints/Player/BP_Player.BP_Player_C|SetCan_Dpad_Up (Variables|ObjectRef|GetPlayer%20Ref) true))
    (:13
      (Variables|/Game/Blueprints/Player/BP_Player.BP_Player_C|SetCan_Dpad_Left (Variables|ObjectRef|GetPlayer%20Ref) true))
    (:14
      (Variables|/Game/Blueprints/Player/BP_Player.BP_Player_C|SetCan_Dpad_Round (Variables|ObjectRef|GetPlayer%20Ref) true))
    (:15
      (Variables|/Game/Blueprints/Player/BP_Player.BP_Player_C|SetCan_Dpad_Reverse (Variables|ObjectRef|GetPlayer%20Ref) true))))

(fn ConstructionScript
  (bind _sm_tablemesh (Variables|Default|GetSM_TableMesh))
  (Components|StaticMesh|SetStaticMesh _sm_tablemesh (Variables|Setting|GetTableMesh))
  (Transformation|SetRelativeLocation _sm_tablemesh "0, 0, 0" false true))