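; BP_Button is an interactable arena button that activates 30 seconds after play starts and calls the arena's HightJack event when pushed.
; While active, it shows an outline and interact widget for a player whose StructureInfoArray is empty, and FoodInterract can also push it.
; A looping timer ramps up the spotlight to signal readiness.
; A push disables the button, later switches the light off, then reactivates both after a cooldown.
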(event Custom|Event_Push
  (CallFunction|PushOverlay)
  (Variables|Default|SetActive? false)
  (Default|EventHightJackButton (Variables|Default|Getref%20Arena))
  (Rendering|Components|Light|SetLightColor (Variables|Default|GetSpotLight) "(R=1.000000,G=0.000000,B=0.000000,A=0.000000)" true)
  (Utilities|FlowControl|Delay 3.0)
  (Rendering|Components|Light|SetIntensity (Variables|Default|GetSpotLight) 0.0)
  (Utilities|FlowControl|Delay (Variables|Default|GetColdown))
  (Rendering|Components|Light|SetLightColor (Variables|Default|GetSpotLight) "(R=1.000000,G=0.000000,B=0.000000,A=1.000000)" true)
  (CallFunction|CALLlIGHT)
  (Variables|Default|SetActive? true))

(event Custom|CustomEvent
  (Variables|Default|SetAlpha (+ (Variables|Default|GetAlpha) 0.1))
  (Rendering|Components|Light|SetIntensity (Variables|Default|GetSpotLight) (Math|Float|Lerp 0.0 7e+03 (Variables|Default|GetAlpha)))
  (if (>= (Variables|/Script/Engine.LightComponentBase|GetIntensity (Variables|Default|GetSpotLight)) 7e+03)
    (Utilities|Time|ClearandInvalidateTimerbyHandle (Variables|Default|GetLightOnTimer))))

(event Custom|cALLlIGHT
  (bind _returnvalue (Utilities|Time|SetTimerbyEvent (delegate Custom|CustomEvent) 0.1 true))
  (Variables|Default|SetLightOnTimer _returnvalue))

(event Custom|PushOverlay
  (Rendering|Material|SetOverlayMaterial (Variables|Default|GetButtonBot) (Variables|Default|GetBaseOverlay) :!class /Script/Engine.MeshComponent)
  (Rendering|SetVisibility (Variables|Default|GetInteract) false false))

(event EventOverlay
  (params (playerRef :type BP%20Player%20Object%20Reference))
  (if (Math|Boolean|ANDBoolean (not (Variables|Default|GetHasOverlay)) (== (Utilities|Array|Length (Variables|/Game/Blueprints/Player/BP_Player.BP_Player_C|GetStructureInfoArray playerRef)) 0) (Variables|Default|GetActive?))
    (Variables|Default|SetHasOverlay true)
    (Rendering|Material|SetOverlayMaterial (Variables|Default|GetButtonBot) "/Game/Art/Materials/Shader/Outline/MI_Outline_White.MI_Outline_White" :!class /Script/Engine.MeshComponent)
    (Rendering|SetVisibility (Variables|Default|GetInteract) true false)
    (else
      (Variables|Default|SetHasOverlay false)
      (Rendering|Material|SetOverlayMaterial (Variables|Default|GetButtonBot) (Variables|Default|GetBaseOverlay) :!class /Script/Engine.MeshComponent)
      (Rendering|SetVisibility (Variables|Default|GetInteract) false false))))

(event EventFoodInterract
  (params (PlayerRef :type BP%20Player%20Object%20Reference) (PlayerCheck :type Integer) (HasFood :type Boolean))
  (if (Variables|Default|GetActive?)
    (CallFunction|EventPush)))

(event EventBeginPlay
  (Variables|Default|SetBaseOverlay (Rendering|Material|GetOverlayMaterial (Variables|Default|GetButtonBot) :!class /Script/Engine.MeshComponent))
  (Variables|Default|SetActive? false)
  (Utilities|FlowControl|Delay 3e+01)
  (Variables|Default|SetActive? true)
  (bind _returnvalue (Utilities|Time|SetTimerbyEvent (delegate Custom|CustomEvent) 0.1 true))
  (Variables|Default|SetLightOnTimer _returnvalue))

(fn ConstructionScript)