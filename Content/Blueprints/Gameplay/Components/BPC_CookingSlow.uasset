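; BPC_CookingSlow is a component that applies a slowdown debuff to the player it is attached to.
; On BeginPlay, its CookingFast event checks that the owner is a BP_Player and, unless protected, halves its InputMultiplier and activates the NGStatDown effect.
; EndEffect deactivates that effect, resets the multiplier to normal and destroys the component; nothing in this graph calls it.
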(event Custom|CookingFast
  (bind _returnvalue (Components|GetOwner))
  (if (Utilities|DoesObjectImplementInterface _returnvalue "/Game/Blueprints/BPI/BPI_Player.BPI_Player_C")
    (bind _asbp_player (Utilities|Casting|CastToBP_Player _returnvalue))
    (bind _output_get (Variables|Default|SetAs%20BP%20Player _asbp_player))
    (if (not (Variables|/Game/Blueprints/Player/BP_Player.BP_Player_C|GetIsProtected _asbp_player))
      (Variables|/Game/Blueprints/Player/BP_Player.BP_Player_C|SetInputMultiplier _output_get 0.5)
      (Components|Activation|Activate (Variables|/Game/Blueprints/Player/BP_Player.BP_Player_C|GetNG_StatDown (Variables|Default|GetAs%20BP%20Player)) false))))

(event Custom|EndEffect
  (Components|Activation|Deactivate (Variables|/Game/Blueprints/Player/BP_Player.BP_Player_C|GetNG_StatDown (Variables|Default|GetAs%20BP%20Player)))
  (Variables|/Game/Blueprints/Player/BP_Player.BP_Player_C|SetInputMultiplier (Variables|Default|GetAs%20BP%20Player) 1.0)
  (Components|DestroyComponent))

(event EventBeginPlay
  (CallFunction|CookingFast))

(event EventTick
  (params (DeltaSeconds :type Float%20%28single-precision%29)))