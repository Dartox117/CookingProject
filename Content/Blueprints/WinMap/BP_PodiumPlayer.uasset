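; Podium character for the win map that shows either the winning or losing player with their chosen animal rig and material.
; On BeginPlay, IdControler picks the winner or loser slot, and the game instance's PlayerWin maps it to that player's mesh and material.
; The stored rig index then selects the one-shot win or loss animation.
; Looping idle variants exist as events, but nothing in this graph calls them.
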(event Custom|RigChoice2
  (switch int (Variables|/Game/Blueprints/GameInstance/BP_GameInstance.BP_GameInstance_C|GetPlayerWin (Variables|Default|GetAs%20BP%20Game%20Instance))
    (:0
      (Components|SkeletalMesh|SetSkeletalMeshAsset (Variables|Default|GetSkeletalMesh) (Utilities|Array|Get(acopy) (Variables|Default|GetRIG) (Variables|/Game/Blueprints/GameInstance/BP_GameInstance.BP_GameInstance_C|GetRig_Index_Player_2 (Variables|Default|GetAs%20BP%20Game%20Instance))))
      (Rendering|Material|SetMaterial (Variables|Default|GetSkeletalMesh) 0 (Variables|/Game/Blueprints/GameInstance/BP_GameInstance.BP_GameInstance_C|GetMaterialPlayer_2 (Variables|Default|GetAs%20BP%20Game%20Instance)))
      (Variables|Default|SetUsedRig (Variables|/Game/Blueprints/GameInstance/BP_GameInstance.BP_GameInstance_C|GetRig_Index_Player_2 (Variables|Default|GetAs%20BP%20Game%20Instance))))
    (:1
      (Components|SkeletalMesh|SetSkeletalMeshAsset (Variables|Default|GetSkeletalMesh) (Utilities|Array|Get(acopy) (Variables|Default|GetRIG) (Variables|/Game/Blueprints/GameInstance/BP_GameInstance.BP_GameInstance_C|GetRig_Index_Player_1 (Variables|Default|GetAs%20BP%20Game%20Instance))))
      (Rendering|Material|SetMaterial (Variables|Default|GetSkeletalMesh) 0 (Variables|/Game/Blueprints/GameInstance/BP_GameInstance.BP_GameInstance_C|GetMaterialPlayer_1 (Variables|Default|GetAs%20BP%20Game%20Instance)))
      (Variables|Default|SetUsedRig (Variables|/Game/Blueprints/GameInstance/BP_GameInstance.BP_GameInstance_C|GetRig_Index_Player_1 (Variables|Default|GetAs%20BP%20Game%20Instance))))))

(event Custom|PlayLooseAnim
  (bind _skeletalmesh (Variables|Default|GetSkeletalMesh))
  (switch int (Variables|Default|GetUsedRig)
    (:0
      (Components|Animation|PlayAnimation _skeletalmesh "/Game/Art/Animation/Character/Cameleon/Loss/Anim_Cameleon_Loss.Anim_Cameleon_Loss" false))
    (:1
      (Components|Animation|PlayAnimation _skeletalmesh "/Game/Art/Animation/Character/Lemurien/Loss/Anim_Lemurien_Loss.Anim_Lemurien_Loss" false))
    (:2
      (Components|Animation|PlayAnimation _skeletalmesh "/Game/Art/Animation/Character/Poulpe/Loss/Anim_Poulpe_Loss.Anim_Poulpe_Loss" false))
    (:3
      (Components|Animation|PlayAnimation _skeletalmesh "/Game/Art/Animation/Character/Renard/Loss/Anim_Renard_Loss.Anim_Renard_Loss" false))))

(event Custom|LooseAnimIdle
  (bind _skeletalmesh (Variables|Default|GetSkeletalMesh))
  (switch int (Variables|Default|GetUsedRig)
    (:0
      (Components|Animation|PlayAnimation _skeletalmesh "/Game/Art/Animation/Character/Cameleon/Loss/Anim_Cameleon_Loss_Idle.Anim_Cameleon_Loss_Idle" true))
    (:1
      (Components|Animation|PlayAnimation _skeletalmesh "/Game/Art/Animation/Character/Lemurien/Loss/Anim_Lemurien_Loss_Idle.Anim_Lemurien_Loss_Idle" true))
    (:2
      (Components|Animation|PlayAnimation _skeletalmesh "/Game/Art/Animation/Character/Poulpe/Loss/Anim_Poulpe_Loss_Idle.Anim_Poulpe_Loss_Idle" true))
    (:3
      (Components|Animation|PlayAnimation _skeletalmesh "/Game/Art/Animation/Character/Renard/Loss/Anim_Renard_Loss_Idle.Anim_Renard_Loss_Idle" true))))

(event Custom|WinIdle
  (bind _skeletalmesh (Variables|Default|GetSkeletalMesh))
  (switch int (Variables|Default|GetUsedRig)
    (:0
      (Components|Animation|PlayAnimation _skeletalmesh "/Game/Art/Animation/Character/Cameleon/Win/Anim_Cameleon_Win_Idle.Anim_Cameleon_Win_Idle" true))
    (:1
      (Components|Animation|PlayAnimation _skeletalmesh "/Game/Art/Animation/Character/Lemurien/Win/Anim_Lemurien_Win_Idle.Anim_Lemurien_Win_Idle" true))
    (:2
      (Components|Animation|PlayAnimation _skeletalmesh "/Game/Art/Animation/Character/Poulpe/Win/Anim_Poulpe_Win_Idle.Anim_Poulpe_Win_Idle" true))
    (:3
      (Components|Animation|PlayAnimation _skeletalmesh "/Game/Art/Animation/Character/Renard/Win/Anim_Renard_Win_Idle.Anim_Renard_Win_Idle" true))))

(event Custom|RigChoice1
  (switch int (Variables|/Game/Blueprints/GameInstance/BP_GameInstance.BP_GameInstance_C|GetPlayerWin (Variables|Default|GetAs%20BP%20Game%20Instance))
    (:0
      (Components|SkeletalMesh|SetSkeletalMeshAsset (Variables|Default|GetSkeletalMesh) (Utilities|Array|Get(acopy) (Variables|Default|GetRIG) (Variables|/Game/Blueprints/GameInstance/BP_GameInstance.BP_GameInstance_C|GetRig_Index_Player_1 (Variables|Default|GetAs%20BP%20Game%20Instance))))
      (Rendering|Material|SetMaterial (Variables|Default|GetSkeletalMesh) 0 (Variables|/Game/Blueprints/GameInstance/BP_GameInstance.BP_GameInstance_C|GetMaterialPlayer_1 (Variables|Default|GetAs%20BP%20Game%20Instance)))
      (Variables|Default|SetUsedRig (Variables|/Game/Blueprints/GameInstance/BP_GameInstance.BP_GameInstance_C|GetRig_Index_Player_1 (Variables|Default|GetAs%20BP%20Game%20Instance))))
    (:1
      (Components|SkeletalMesh|SetSkeletalMeshAsset (Variables|Default|GetSkeletalMesh) (Utilities|Array|Get(acopy) (Variables|Default|GetRIG) (Variables|/Game/Blueprints/GameInstance/BP_GameInstance.BP_GameInstance_C|GetRig_Index_Player_2 (Variables|Default|GetAs%20BP%20Game%20Instance))))
      (Rendering|Material|SetMaterial (Variables|Default|GetSkeletalMesh) 0 (Variables|/Game/Blueprints/GameInstance/BP_GameInstance.BP_GameInstance_C|GetMaterialPlayer_2 (Variables|Default|GetAs%20BP%20Game%20Instance)))
      (Variables|Default|SetUsedRig (Variables|/Game/Blueprints/GameInstance/BP_GameInstance.BP_GameInstance_C|GetRig_Index_Player_2 (Variables|Default|GetAs%20BP%20Game%20Instance))))))

(event Custom|PlayWinAnim
  (bind _skeletalmesh (Variables|Default|GetSkeletalMesh))
  (switch int (Variables|Default|GetUsedRig)
    (:0
      (Components|Animation|PlayAnimation _skeletalmesh "/Game/Art/Animation/Character/Cameleon/Win/Anim_Cameleon_Win.Anim_Cameleon_Win" false))
    (:1
      (Components|Animation|PlayAnimation _skeletalmesh "/Game/Art/Animation/Character/Lemurien/Win/Anim_Lemurien_Win.Anim_Lemurien_Win" false))
    (:2
      (Components|Animation|PlayAnimation _skeletalmesh "/Game/Art/Animation/Character/Poulpe/Win/Anim_Poulpe_Win.Anim_Poulpe_Win" false))
    (:3
      (Components|Animation|PlayAnimation _skeletalmesh "/Game/Art/Animation/Character/Renard/Win/Anim_Renard_Win.Anim_Renard_Win" false))))

(event EventBeginPlay
  (bind _asbp_game_instance (Utilities|Casting|CastToBP_GameInstance (Game|GetGameInstance)))
  (Variables|Default|SetAs%20BP%20Game%20Instance _asbp_game_instance)
  (switch int (Variables|Default|Getid_controler)
    (:0
      (CallFunction|RigChoice1)
      (CallFunction|PlayWinAnim))
    (:1
      (CallFunction|RigChoice2)
      (CallFunction|PlayLooseAnim))))

(event Collision|EventActorBeginOverlap
  (params (OtherActor :type Actor%20Object%20Reference)))

(event EventTick
  (params (DeltaSeconds :type Float%20%28single-precision%29)))

(fn ConstructionScript)