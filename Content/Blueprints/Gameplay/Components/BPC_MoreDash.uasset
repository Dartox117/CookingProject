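; BPC_MoreDash is a temporary dash buff component that shortens the owning player's dash cooldown.
; On BeginPlay it confirms the owner implements BPI_Player, casts it to BP_Player, lowers DashCD and activates the player's NGMoreDash effect.
; EndEffect sets the cooldown back to a hardcoded value, deactivates NGMoreDash and destroys the component.
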(event Custom|ReduceDashCd
  (bind _returnvalue (Components|GetOwner))
  (if (Utilities|DoesObjectImplementInterface _returnvalue "/Game/Blueprints/BPI/BPI_Player.BPI_Player_C")
    (bind _asbp_player (Utilities|Casting|CastToBP_Player _returnvalue))
    (bind _output_get (Variables|Default|SetAs%20BP%20Player _asbp_player))
    (Variables|/Game/Blueprints/Player/BP_Player.BP_Player_C|SetDash_CD _output_get 0.3)
    (Components|Activation|Activate (Variables|/Game/Blueprints/Player/BP_Player.BP_Player_C|GetNG_MoreDash (Variables|Default|GetAs%20BP%20Player)) false)))

(event Custom|EndEffect
  (Variables|/Game/Blueprints/Player/BP_Player.BP_Player_C|SetDash_CD (Variables|Default|GetAs%20BP%20Player) 1.0)
  (Components|Activation|Deactivate (Variables|/Game/Blueprints/Player/BP_Player.BP_Player_C|GetNG_MoreDash (Variables|Default|GetAs%20BP%20Player)))
  (Components|DestroyComponent))

(event EventBeginPlay
  (CallFunction|ReduceDashCd))

(event EventTick
  (params (DeltaSeconds :type Float%20%28single-precision%29)))