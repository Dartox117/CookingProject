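; Conveyor belt actor that spawns BP_Food at the start of a spline, passing itself as the path, and destroys food overlapping a box at the end.
; It caches DT_Foods by name and registers with the game manager.
; A looping timer spawns random food with a chance of a rolled alteration, while a manual event spawns specified food.
; The construction script optionally tiles spline meshes along the path, sized from mesh bounds.
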(event OnComponentBeginOverlap(DestroyFood)
  (params (OverlappedComponent :type Primitive%20Component%20Object%20Reference) (OtherActor :type Actor%20Object%20Reference) (OtherComp :type Primitive%20Component%20Object%20Reference) (OtherBodyIndex :type Integer) (bFromSweep :type Boolean) (SweepResult :type Hit%20Result%20Structure%20%28by%20ref%29))
  ;[0 0 0] Destroy Food
  (bind _asbp_food (Utilities|Casting|CastToBP_Food OtherActor))
  (Actor|DestroyActor _asbp_food))

(event Custom|Event_StartConveyor
  ;[0.15 0.1029 0 0.5] Spawn Call
  ;;[0.15 0.15 0.15 0.5] Automatic
  (bind _returnvalue (Utilities|Time|SetTimerbyEvent (delegate Custom|Event_Constant_Call_Spawn) (Variables|Setting|GetItem_SpawnRate) true))
  (Variables|Reference|SetRef_SpawnTimer _returnvalue))

(event Custom|Event_Constant_Call_Spawn
  ;[0.15 0.1029 0 0.5] Spawn Call
  ;;[0.15 0.15 0.15 0.5] Automatic
  (bind _selected_alteration (Default|FunctionRollAlteration (Variables|Reference|GetRef%20Game%20Manager)))
  (if (Math|Random|RandomBoolwithWeight (Variables|Setting|GetAutoSpawnChance))
    (CallFunction|EventSpawnonSpline _selected_alteration (Utilities|McGetRandomFood))
    (else
      (CallFunction|EventSpawnonSpline "NewEnumerator7" (Utilities|McGetRandomFood)))))

(event Custom|Event_EndDensity
  ;[0.15 0.1029 0 0.5] Spawn Call
  ;;[0.15 0.15 0.15 0.5] Clear autospawn
  (Utilities|Time|ClearandInvalidateTimerbyHandle (Variables|Reference|GetRef_SpawnTimer)))

(event Custom|Event_Spawn_On_Spline
  (params (Draw_Alteration :type E_Alteration%20Enum :default "NewEnumerator0") (Food_Info :type ST%20Foods%20Structure))
  ;[0.5938 0.002354 0 0.5] Spawn Item on spline
  (Game|SpawnActorfromClass "/Game/Blueprints/Gameplay/BP_Food.BP_Food_C" (Math|Transform|MakeTransform (Variables|Temp|GetStartingSplinePoint) "0, 0, 0" "1.000000,1.000000,1.000000") "AlwaysSpawn" "MultiplyWithRoot" 0 (Utilities|Struct|MakeST_Foods (.index Food_Info) (.foodname Food_Info) (.input Food_Info) (.points Food_Info) (.staticmesh Food_Info) (.cooked Food_Info) (.surprise Food_Info) Draw_Alteration (.image Food_Info)) self Draw_Alteration 0))

(event Custom|Event_Manual_Call_Spawn
  (params (Food :type E_Food%20Enum :default "NewEnumerator6") (Alteration :type E_Alteration%20Enum :default "NewEnumerator7"))
  ;[0.15 0.1029 0 0.5] Spawn Call
  ;;[0.15 0.15 0.15 0.5] Manual
  (CallFunction|EventSpawnonSpline Alteration (.Value (Utilities|Map|Find (Variables|Data|GetStorage_Food) Food))))

(event Custom|Event_Setting_GameManager
  ;[0 0.1228 0.15 0.5] Game manager Link
  (bind _asbp_game_instance (Utilities|Casting|CastToBP_GameInstance (Game|GetGameInstance)))
  (Variables|Reference|SetRef%20Game%20Manager (Variables|/Game/Blueprints/GameInstance/BP_GameInstance.BP_GameInstance_C|GetRef_GameManager _asbp_game_instance))
  (Default|CallEDListenConveyor (Variables|Reference|GetRef%20Game%20Manager) self))

(event EventBeginPlay
  ;[0.003705 0.485 0] Begin play
  (if (Variables|Setting|GetIsReal)
    (Variables|Temp|SetStartingSplinePoint (.location (Spline|GetTransformatSplinePoint (Variables|Default|GetSpline_Path) 0 "World" false)))
    (Utilities|FlowControl|DelayUntilNextTick)
    (CallFunction|EventSettingGameManager)
    (CallFunction|FuctionGetFood)))

(fn ConstructionScript
  ;[0.15 0.15 0.15 0.5] Set The Destruction Box at the End of the Spline
  (Transformation|SetWorldLocation (Variables|Default|GetDestroyFood) (.location (Spline|GetTransformatSplinePoint (Variables|Default|GetSpline_Path) (Spline|GetNumberOfSplinePoints (Variables|Default|GetSpline_Path)) "World" false)) false true)
  ;[0.15 0.15 0.15 0.5] Do we draw the mesh ?
  (if (Variables|Setting|GetIsMesh)
    ;[0.15 0.15 0.15 0.5] Spline And mesh Setting
    (LocalVariables|SetOffset (Variables|Setting|GetMeshOffset))
    (LocalVariables|SetCurrentSpline (Variables|Default|GetSpline_Path))
    (LocalVariables|SetMeshOnSpline (Variables|Setting|GetMesh))
    (Utilities|FlowControl|Sequence
      (:then_0
        (Utilities|McGettheSizeOfASplineSection))
      (:then_1
        ;[0.15 0.15 0.15 0.5] Define the number of mesh that can fit on the spline
        (bind _output_get (LocalVariables|SetNumOfParts (.ReturnValue (Math|Float|Division(WholeandRemainder) (Spline|GetSplineLength (LocalVariables|GetCurrentSpline)) (LocalVariables|GetSectionLenght)))))
        (for _index (range 0 _output_get)
          ;[0.15 0.15 0.15 0.5] Define the Starting and ending Position of the current mesh
          (LocalVariables|SetDIstanceStart (+ (* _index (LocalVariables|GetSectionLenght)) (LocalVariables|GetOffset)))
          (LocalVariables|SetDIstanceEnd (+ (+ (* _index (LocalVariables|GetSectionLenght)) (LocalVariables|GetOffset)) (LocalVariables|GetSectionLenght) (LocalVariables|GetOffset)))
          ;[0.15 0.15 0.15 0.5] on the spline
          (bind _returnvalue (AddComponent|AddSplineMeshComponent false))
          (LocalVariables|SetCurrentMesh _returnvalue)
          (Components|StaticMesh|SetStaticMesh (LocalVariables|GetCurrentMesh) (LocalVariables|GetMeshOnSpline))
          ;[0.15 0.15 0.15 0.5] Set Start And End Position of the mesh on the spline
          (SplineMesh|SetStartandEnd (LocalVariables|GetCurrentMesh) (Spline|GetLocationatDistanceAlongSpline (LocalVariables|GetCurrentSpline) (LocalVariables|GetDIstanceStart) "Local") (Math|Vector|ClampVectorSize (Spline|GetTangentatDistanceAlongSpline (LocalVariables|GetCurrentSpline) (LocalVariables|GetDIstanceStart) "Local") 0.0 (LocalVariables|GetSectionLenght)) (Spline|GetLocationatDistanceAlongSpline (LocalVariables|GetCurrentSpline) (LocalVariables|GetDIstanceEnd) "Local") (Math|Vector|ClampVectorSize (Spline|GetTangentatDistanceAlongSpline (LocalVariables|GetCurrentSpline) (LocalVariables|GetDIstanceEnd) "Local") 0.0 (LocalVariables|GetSectionLenght)) false :!class /Script/Engine.SplineMeshComponent)
          ;[0.15 0.15 0.15 0.5] Set Rotation at the Start of the Mesh (in Radians)
          (Class|SplineMeshComponent|SetStartRoll (LocalVariables|GetCurrentMesh) (Math|Trig|DegreesToRadians (.Roll (Math|Rotator|BreakRotator (Spline|GetRotationatDistanceAlongSpline (LocalVariables|GetCurrentSpline) (LocalVariables|GetDIstanceStart) "Local")))) false)
          ;[0.15 0.15 0.15 0.5] Set Rotation at the End of the Mesh (in Radians)
          (Class|SplineMeshComponent|SetEndRoll (LocalVariables|GetCurrentMesh) (Math|Trig|DegreesToRadians (.Roll (Math|Rotator|BreakRotator (Spline|GetRotationatDistanceAlongSpline (LocalVariables|GetCurrentSpline) (LocalVariables|GetDIstanceEnd) "Local")))) false)
          ;[0.15 0.15 0.15 0.5] Set Scale at the Start of the Mesh
          (SplineMesh|SetStartScale (LocalVariables|GetCurrentMesh) (Math|Vector2D|MakeVector2D (.y (Class|SplineComponent|GetScaleatDistanceAlongSpline (LocalVariables|GetCurrentSpline) (LocalVariables|GetDIstanceStart))) (.z (Class|SplineComponent|GetScaleatDistanceAlongSpline (LocalVariables|GetCurrentSpline) (LocalVariables|GetDIstanceStart)))) false :!class /Script/Engine.SplineMeshComponent)
          ;[0.15 0.15 0.15 0.5] Set Scale at the end of the Mesh
          (SplineMesh|SetEndScale (LocalVariables|GetCurrentMesh) (Math|Vector2D|MakeVector2D (.y (Class|SplineComponent|GetScaleatDistanceAlongSpline (LocalVariables|GetCurrentSpline) (LocalVariables|GetDIstanceEnd))) (.z (Class|SplineComponent|GetScaleatDistanceAlongSpline (LocalVariables|GetCurrentSpline) (LocalVariables|GetDIstanceEnd)))) true :!class /Script/Engine.SplineMeshComponent)
          ;[0.15 0.15 0.15 0.5] Set Collision
          (Collision|SetCollisionEnabled (LocalVariables|GetCurrentMesh) "NoCollision"))))))

(fn FunctionGetStartPosition/Tangent
  (params (Index :type Integer))
  (bind _returnvalue (* Index 0.0))
  (bind _spline_path (Variables|Default|GetSpline_Path))
  (return (Spline|GetLocationatDistanceAlongSpline _spline_path _returnvalue "Local") (Math|Vector|ClampVectorSize (Spline|GetTangentatDistanceAlongSpline _spline_path _returnvalue "Local") 0.0 0.0)))

(fn FunctionGetEndPosition/Tangent
  (params (Index :type Integer))
  (bind _returnvalue (+ Index 1))
  (bind _spline_path (Variables|Default|GetSpline_Path))
  (bind _returnvalue_2 (* _returnvalue 0.0))
  (return (Spline|GetLocationatDistanceAlongSpline _spline_path _returnvalue_2 "Local") (Math|Vector|ClampVectorSize (Spline|GetTangentatDistanceAlongSpline _spline_path _returnvalue_2 "Local") 0.0 0.0)))

(fn FuctionGetFood
  (bind _outrownames (DataTable|GetDataTableRowNames "/Game/Blueprints/Structures_Data/DT_Foods.DT_Foods"))
  (for _array_element _outrownames
    (bind _returnvalue (Utilities|GetDataTableRow "/Game/Blueprints/Structures_Data/DT_Foods.DT_Foods" _array_element)
      (:then
        (LocalVariables|SetTemp_Row _returnvalue)
        (Utilities|Map|Add (Variables|Data|GetStorage_Food) (.foodname (LocalVariables|GetTemp_Row)) (LocalVariables|GetTemp_Row))))))