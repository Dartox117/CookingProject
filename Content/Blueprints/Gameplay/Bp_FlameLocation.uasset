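; Flame spawn location actor that turns a Niagara wall flame on for a given duration, tracking its state with IsActive.
; BeginPlay caches the game manager from the game instance and fires a debug test flame.
; Construction stores the Start and End component world positions, which are not used further here.
; The Box overlap filters for BP_Player but has no effect yet.
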(event OnComponentBeginOverlap(Box)
  (params (OverlappedComponent :type Primitive%20Component%20Object%20Reference) (OtherActor :type Actor%20Object%20Reference) (OtherComp :type Primitive%20Component%20Object%20Reference) (OtherBodyIndex :type Integer) (bFromSweep :type Boolean) (SweepResult :type Hit%20Result%20Structure%20%28by%20ref%29))
  (Utilities|Casting|CastToBP_Player OtherActor))

(event Custom|Event_Spawn_Flame
  (params (ActivationTime :type Float%20%28double-precision%29))
  (Variables|Default|SetIsActive true)
  (Components|Activation|Activate (Variables|Default|GetNG_WallFlame) false)
  (Utilities|FlowControl|Delay ActivationTime)
  (Components|Activation|SetActive (Variables|Default|GetNG_WallFlame) false false)
  (Variables|Default|SetIsActive false))

(event EventBeginPlay
  (Utilities|McGetGameManager)
  ;[1 0 0] DEBUG
  (CallFunction|EventSpawnFlame 5.0))

(fn ConstructionScript
  (Variables|Default|SetStart_Location (Transformation|GetWorldLocation (Variables|Default|GetStart)))
  (Variables|Default|SetEnd_Location (Transformation|GetWorldLocation (Variables|Default|GetEnd))))