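; BPC_Protection is a component that gives the player a protection effect while it is attached.
; On BeginPlay it checks that its owner implements BPI_Player, casts it to BP_Player, then sets IsProtected and activates the NGShield effect.
; EndEffect clears both on the cached player and destroys the component; nothing in this graph calls it or times the duration.
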(event Custom|ProtectPlayer
  (bind _returnvalue (Components|GetOwner))
  (if (Utilities|DoesObjectImplementInterface _returnvalue "/Game/Blueprints/BPI/BPI_Player.BPI_Player_C")
    (bind _asbp_player (Utilities|Casting|CastToBP_Player _returnvalue))
    (bind _output_get (Variables|Default|SetAs%20BP%20Player _asbp_player))
    (Variables|/Game/Blueprints/Player/BP_Player.BP_Player_C|SetIsProtected _output_get true)
    (Components|Activation|SetActive (Variables|/Game/Blueprints/Player/BP_Player.BP_Player_C|GetNG_Shield (Variables|Default|GetAs%20BP%20Player)) true false)))

(event Custom|EndEffect
  (Variables|/Game/Blueprints/Player/BP_Player.BP_Player_C|SetIsProtected (Variables|Default|GetAs%20BP%20Player) false)
  (Components|Activation|SetActive (Variables|/Game/Blueprints/Player/BP_Player.BP_Player_C|GetNG_Shield (Variables|Default|GetAs%20BP%20Player)) false false)
  (Components|DestroyComponent))

(event EventBeginPlay
  (CallFunction|ProtectPlayer))

(event EventTick
  (params (DeltaSeconds :type Float%20%28single-precision%29)))