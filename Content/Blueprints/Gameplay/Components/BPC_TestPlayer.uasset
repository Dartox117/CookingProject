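; BPC_TestPlayer is an actor component that gives its owning BP_Player a movement speed bonus.
; On BeginPlay it casts the owner, doubles Speed, then sets MaxWalkSpeed to twice that updated Speed, four times the starting value.
; DestroySelf restores Speed and MaxWalkSpeed from BaseSpeed and destroys the component; nothing in this Blueprint calls it.
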(event Custom|DestroySelf
  (bind _as_bp_player (Variables|Default|GetAs%20BP%20Player))
  (bind _output_get (Variables|/Game/Blueprints/Player/BP_Player.BP_Player_C|SetSpeed _as_bp_player (Variables|/Game/Blueprints/Player/BP_Player.BP_Player_C|GetBaseSpeed _as_bp_player)))
  (Variables|/Script/Engine.CharacterMovementComponent|SetMaxWalkSpeed (Variables|/Script/Engine.Character|GetCharacterMovement _as_bp_player) _output_get)
  (Components|DestroyComponent))

(event Custom|SpeedBonus
  (bind _asbp_player (Utilities|Casting|CastToBP_Player (Components|GetOwner)))
  (bind _output_get (Variables|Default|SetAs%20BP%20Player _asbp_player))
  (Variables|/Game/Blueprints/Player/BP_Player.BP_Player_C|SetSpeed _output_get (* (Variables|/Game/Blueprints/Player/BP_Player.BP_Player_C|GetSpeed _asbp_player) 2.0))
  (Variables|/Script/Engine.CharacterMovementComponent|SetMaxWalkSpeed (Variables|/Script/Engine.Character|GetCharacterMovement _asbp_player) (* (Variables|/Game/Blueprints/Player/BP_Player.BP_Player_C|GetSpeed _asbp_player) 2.0)))

(event EventBeginPlay
  (CallFunction|SpeedBonus))

(event EventTick
  (params (DeltaSeconds :type Float%20%28single-precision%29)))