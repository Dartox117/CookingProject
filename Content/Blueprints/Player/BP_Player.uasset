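; Player character for a cooking game: moves, dashes, interacts through a forward sphere trace and carries a limited stack of ingredients shown on meshes.
; While cooking, button mash, stick and alternating trigger combos send progress to the workstation (PlanDeTravailRef), with penalties for wrong inputs.
; A looping downward trace switches friction, braking and dash power between wood and ice surfaces.
; Also toggles a debug menu and drives movement, dash and cook-end VFX.
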(event Custom|ResetFood
  ;[0.15 0.15 0.15 0.5] Reset des aliments portés
  (Variables|Speed|SetSpeed (Variables|Speed|GetBaseSpeed))
  (CallFunction|SetSpeed)
  (Utilities|Array|Clear (Variables|Array|GetStructureInfoArray))
  (Variables|StateBoolean|SetHasFood false)
  (for _array_element (Variables|Array|GetStaticmesh_Array)
    (Components|StaticMesh|SetStaticMesh _array_element 0)))

(event Custom|AddFood
  (params (BP_Food_Ref :type BP%20Food%20Object%20Reference))
  ;[0.15 0.15 0.15 0.5] Code de récupération d'un aliment
  (if (< (Utilities|Array|Length (Variables|Array|GetStructureInfoArray)) (Variables|Default|GetMaxIngrediantCarry))
    (CallFunction|SetSpeed)
    (Variables|StateBoolean|SetHasFood true)
    (Components|StaticMesh|SetStaticMesh (Utilities|Array|Get(acopy) (Variables|Array|GetStaticmesh_Array) (Utilities|Array|Length (Variables|Array|GetStructureInfoArray))) (Variables|/Script/Engine.StaticMeshComponent|GetStaticMesh (Variables|/Game/Blueprints/Gameplay/BP_Food.BP_Food_C|GetStaticMesh BP_Food_Ref)))
    (Utilities|Array|Add (Variables|Array|GetStructureInfoArray) (Variables|/Game/Blueprints/Gameplay/BP_Food.BP_Food_C|GetStructureInfo BP_Food_Ref))))

(event Custom|SetSpeed
  ;[0.15 0.15 0.15 0.5] SetSpeed
  (Variables|/Script/Engine.CharacterMovementComponent|SetMaxWalkSpeed (Variables|Character|GetCharacterMovement) (* (Variables|Speed|GetSpeed) (Utilities|SpeedMultiplicateur))))

(event Custom|ComboReset
  ;[0.15 0.15 0.15 0.5] Reset du Combo
  (Default|GetInput (Variables|ObjectReference|GetPlanDeTravailRef) (Variables|Default|GetInput_Value)))

(event Custom|ResetComboBool
  ;[0.15 0.15 0.15 0.5] Reset du combo
  (Variables|CanDoBoolean|SetCanXCombo false)
  (Variables|CanDoBoolean|SetCanYCombo false)
  (Variables|CanDoBoolean|SetCanStickUpDownCombo false)
  (Variables|CanDoBoolean|SetCanStickRound false)
  (Variables|CanDoBoolean|SetCan_R_trigger false)
  (Variables|CanDoBoolean|SetCan_L_trigger false))

(event Custom|WrongInput
  ;[0.15 0.15 0.15 0.5] Reset du Combo
  (Default|WrongInput (Variables|ObjectReference|GetPlanDeTravailRef))
  (Default|GetInput (Variables|ObjectReference|GetPlanDeTravailRef) -1e+01)
  (Variables|StateBoolean|SetStartCombo false)
  (Utilities|FlowControl|Delay 1.0)
  (Variables|StateBoolean|SetStartCombo true))

(event Custom|EndDashVfx
  ;[0.15 0.15 0.15 0.5] Dash
  (Components|Activation|Deactivate (Variables|Default|GetDash_VFX))
  (Variables|StateBoolean|SetIs%20Dashing false))

(event Input|EnhancedActionEvents|EnhancedInputActionIA_Interract
  (params (ActionValue :type Boolean) (ElapsedSeconds :type Float%20%28double-precision%29) (TriggeredSeconds :type Float%20%28double-precision%29) (InputAction :type Input%20Action%20Object%20Reference :default "/Game/Input/Input_Actions/IA_Interract.IA_Interract"))
  (bind _capsulecomponent (Variables|Collision|GetCapsuleComponent))
  (bind _returnvalue (Transformation|GetWorldLocation _capsulecomponent))
  ;[0.15 0.15 0.15 0.5] Interract
  ;;[0.15 0.15 0.15 0.5] box trace pour l'interaction
  (:Started
    (if (and (not (Variables|StateBoolean|GetIsCooking)) (not (Variables|Default|GetIsStunned)))
      (bind _outhit (Collision|SphereTraceByChannel _returnvalue (+ _returnvalue (* (Transformation|GetActorForwardVector) 1e+02)) 8e+01 "TraceTypeQuery1" false 0 "None"))
      (Class|BPIInterract|FoodInterract(Message) (.HitActor (Collision|BreakHitResult _outhit)) self (Variables|Default|Getid_controler) (Variables|StateBoolean|GetHasFood)))))

(event Input|EnhancedActionEvents|EnhancedInputActionIA_Move
  (params (ActionValue :type Vector%202D%20Structure) (ElapsedSeconds :type Float%20%28double-precision%29) (TriggeredSeconds :type Float%20%28double-precision%29) (InputAction :type Input%20Action%20Object%20Reference :default "/Game/Input/Input_Actions/IA_Move.IA_Move"))
  ;[0.15 0.15 0.15 0.5] Move
  (:Triggered
    (if (and (not (Variables|StateBoolean|GetIsCooking)) (Variables|CanDoBoolean|GetCanMoove))
      (Variables|Default|SetAction%20Value%20X (.x ActionValue))
      (Variables|Default|SetAction%20Value%20Y (.y ActionValue))
      (Pawn|Input|AddMovementInput "1.000000,0.000000,0.000000" (Variables|Default|GetAction%20Value%20X) false)
      (Pawn|Input|AddMovementInput "0.000000,1.000000,0.000000" (Variables|Default|GetAction%20Value%20Y) false)))
  (:Started
    (Components|Activation|Activate (Variables|Default|GetSprint_VFX) true))
  (:Completed
    (Components|Activation|Deactivate (Variables|Default|GetSprint_VFX))))

(event Input|EnhancedActionEvents|EnhancedInputActionIA_Sprint
  (params (ActionValue :type Boolean) (ElapsedSeconds :type Float%20%28double-precision%29) (TriggeredSeconds :type Float%20%28double-precision%29) (InputAction :type Input%20Action%20Object%20Reference :default "/Game/Input/Input_Actions/IA_Sprint.IA_Sprint"))
  ;[0.15 0.15 0.15 0.5] Dash
  (:Started
    (if (Math|Boolean|ANDBoolean (Variables|CanDoBoolean|GetCanDash) (Variables|CanDoBoolean|GetCanMoove) (not (Variables|StateBoolean|GetIsCooking)))
      (Components|Activation|Activate (Variables|Default|GetDash_VFX) false)
      (Variables|CanDoBoolean|SetCanDash false)
      (Utilities|FlowControl|Delay 0.1)
      (Character|LaunchCharacter (* (Math|Vector|MakeVector (Variables|Default|GetAction%20Value%20X) (Variables|Default|GetAction%20Value%20Y) 0.0) (Variables|Dash|GetDashPower)) false false)
      (Variables|StateBoolean|SetIs%20Dashing true)
      (Utilities|Time|SetTimerbyEvent (delegate Custom|EndDashVfx) 0.48)
      (Utilities|FlowControl|Delay (Variables|Dash|GetDash_CD))
      (Variables|CanDoBoolean|SetCanDash true))))

(event Input|EnhancedActionEvents|EnhancedInputActionIA_Debug
  (params (ActionValue :type Boolean) (ElapsedSeconds :type Float%20%28double-precision%29) (TriggeredSeconds :type Float%20%28double-precision%29) (InputAction :type Input%20Action%20Object%20Reference :default "/Game/Input/Input_Actions/IA_Debug.IA_Debug"))
  (bind _returnvalue (Game|GetPlayerController 0))
  (bind _returnvalue_2 (Game|GetPlayerController 0))
  ;[0.15 0.15 0.15 0.5] DEBUG ONLY
  (:Started
    (if (Variables|StateBoolean|GetDoDebugExist)
      (Widget|RemovefromParent (Variables|ObjectReference|GetDebugMenuRef))
      (Input|SetInputModeGameOnly _returnvalue false)
      (Variables|StateBoolean|SetDoDebugExist false)
      (Variables|/Script/Engine.PlayerController|SetbShowMouseCursor _returnvalue false)
      (else
        (bind _returnvalue_3 (UserInterface|CreateWidget "/Game/Blueprints/Debug/WG_Debug.WG_Debug_C" (Game|GetPlayerController 0)))
        (bind _output_get (Variables|ObjectReference|SetDebugMenuRef _returnvalue_3))
        (UserInterface|Viewport|AddtoViewport _output_get 0)
        (Input|SetInputModeGameandUI _returnvalue_2 0 "DoNotLock" true false)
        (Variables|StateBoolean|SetDoDebugExist true)
        (Variables|/Script/Engine.PlayerController|SetbShowMouseCursor _returnvalue_2 true)))))

(event EventBeginPlay
  ;[0.15 0.15 0.15 0.5] beginPlay
  (Utilities|FlowControl|Delay 0.01)
  (bind _asplayer_controller (Utilities|Casting|CastToPlayerController (Pawn|GetController)))
  (Utilities|IsValid (PlayerController|LocalPlayerSubsystems|GetEnhancedInputLocalPlayerSubsystem _asplayer_controller)
    (:Is%20Valid
      (Input|AddMappingContext (PlayerController|LocalPlayerSubsystems|GetEnhancedInputLocalPlayerSubsystem _asplayer_controller) "/Game/Input/IMC_Default.IMC_Default" 0 "(bIgnoreAllPressedKeysUntilRelease=True,bForceImmediately=False,bNotifyUserSettings=False)")
      (Variables|Array|SetStaticmesh_Array (Utilities|Array|MakeArray (Variables|Default|GetFood_1) (Variables|Default|GetFood_2) (Variables|Default|GetFood_3) (Variables|Default|GetFood_4)))
      (Components|Activation|SetActive (Variables|Default|GetSprint_VFX) false false)
      (CallFunction|StartGroundDetection))))

(event Input|EnhancedActionEvents|EnhancedInputActionIA_XCombo
  (params (ActionValue :type Boolean) (ElapsedSeconds :type Float%20%28double-precision%29) (TriggeredSeconds :type Float%20%28double-precision%29) (InputAction :type Input%20Action%20Object%20Reference :default "/Game/Input/Input_Actions/IA_XCombo.IA_XCombo"))
  ;[0 0.15 0.122 0.5] Mash X/Y Button
  (:Started
    (if (Math|Boolean|ANDBoolean (Variables|StateBoolean|GetStartCombo) (Variables|StateBoolean|GetIsCooking) (not (Variables|Default|GetIsStunned)))
      (if (Variables|CanDoBoolean|GetCanXCombo)
        (Variables|Default|SetInput_Value 2e+01)
        (CallFunction|ComboReset)
        (elif (not (Variables|StateBoolean|GetBonusInputActive))
          (CallFunction|WrongInput))))))

(event Input|EnhancedActionEvents|EnhancedInputActionIA_YCombo
  (params (ActionValue :type Boolean) (ElapsedSeconds :type Float%20%28double-precision%29) (TriggeredSeconds :type Float%20%28double-precision%29) (InputAction :type Input%20Action%20Object%20Reference :default "/Game/Input/Input_Actions/IA_YCombo.IA_YCombo"))
  ;[0 0.15 0.122 0.5] Mash X/Y Button
  (:Started
    (if (Math|Boolean|ANDBoolean (Variables|StateBoolean|GetStartCombo) (Variables|StateBoolean|GetIsCooking) (not (Variables|Default|GetIsStunned)))
      (if (Variables|CanDoBoolean|GetCanYCombo)
        (Variables|Default|SetInput_Value 2e+01)
        (CallFunction|ComboReset)
        (elif (not (Variables|StateBoolean|GetBonusInputActive))
          (CallFunction|WrongInput))))))

(event Input|EnhancedActionEvents|EnhancedInputActionIA_R_Trigger
  (params (ActionValue :type Boolean) (ElapsedSeconds :type Float%20%28double-precision%29) (TriggeredSeconds :type Float%20%28double-precision%29) (InputAction :type Input%20Action%20Object%20Reference :default "/Game/Input/Input_Actions/IA_R_Trigger.IA_R_Trigger"))
  ;[0.15 0.00139 0.1013 0.7913] Trigger Swap
  (:Started
    (if (Math|Boolean|ANDBoolean (Variables|StateBoolean|GetStartCombo) (Variables|StateBoolean|GetIsCooking) (not (Variables|Default|GetIsStunned)))
      (if (Variables|CanDoBoolean|GetCan_R_trigger)
        (Variables|Default|SetInput_Value 8.0)
        (Variables|CanDoBoolean|SetCan_L_trigger true)
        (CallFunction|ComboReset)
        (Variables|CanDoBoolean|SetCan_R_trigger false)
        (elif (not (Variables|StateBoolean|GetBonusInputActive))
          (CallFunction|WrongInput)
          (Variables|CanDoBoolean|SetCan_R_trigger true)
          (Variables|CanDoBoolean|SetCan_L_trigger true))))))

(event Input|EnhancedActionEvents|EnhancedInputActionIA_StickRound
  (params (ActionValue :type Vector%202D%20Structure) (ElapsedSeconds :type Float%20%28double-precision%29) (TriggeredSeconds :type Float%20%28double-precision%29) (InputAction :type Input%20Action%20Object%20Reference :default "/Game/Input/Input_Actions/IA_StickRound.IA_StickRound"))
  ;[0.05485 0.15 0 0.7739] Move Stick
  (:Triggered
    (if (and (or (Variables|CanDoBoolean|GetCanStickRound) (Variables|CanDoBoolean|GetCanStickUpDownCombo)) (not (Variables|Default|GetIsStunned))) :!label _label
      (Variables|StickCheckVar|SetRightStickX (.x ActionValue))
      (Variables|StickCheckVar|SetRightStickY (.y ActionValue))
      (if (and (Variables|StateBoolean|GetStartCombo) (Variables|StateBoolean|GetIsCooking))
        (if (Variables|CanDoBoolean|GetCanStickRound)
          (if (and (Math|Float|NearlyEqual(Float) (Variables|StickCheckVar|GetRightStickX) (Variables|StickCheckVar|GetStickToGoRoundX) 0.2) (Math|Float|NearlyEqual(Float) (Variables|StickCheckVar|GetRightStickY) (Variables|StickCheckVar|GetStickToGoRoundY) 0.2))
            (Variables|Default|SetInput_Value 1e+01)
            ;;[0.15 0 0.003166 0.5] changement de l'angle de stick à avoir
            (CallFunction|ComboReset)
            (Math|Integer|IncrementInt (Variables|StickCheckVar|GetStickRoundSwitch)
              (:%20%20
                (if (>= (Variables|StickCheckVar|GetStickRoundSwitch) 4)
                  (Variables|StickCheckVar|SetStickRoundSwitch 0))
                (switch int (Variables|StickCheckVar|GetStickRoundSwitch)
                  (:0
                    (Variables|StickCheckVar|SetStickToGoRoundX 0.0)
                    (Variables|StickCheckVar|SetStickToGoRoundY -1.0))
                  (:1
                    (Variables|StickCheckVar|SetStickToGoRoundX 1.0)
                    (Variables|StickCheckVar|SetStickToGoRoundY 0.0))
                  (:2
                    (Variables|StickCheckVar|SetStickToGoRoundX 0.0)
                    (Variables|StickCheckVar|SetStickToGoRoundY 1.0))
                  (:3
                    (Variables|StickCheckVar|SetStickToGoRoundX -1.0)
                    (Variables|StickCheckVar|SetStickToGoRoundY 1.0))))))
          (elif (Variables|CanDoBoolean|GetCanStickUpDownCombo)
            (if (== (Variables|StickCheckVar|GetRightStickY) (Variables|StickCheckVar|GetStickToGoUp))
              (Variables|Default|SetInput_Value 1e+01)
              (CallFunction|ComboReset)
              (Variables|StickCheckVar|SetStickToGoUp (* (Variables|StickCheckVar|GetStickToGoUp) -1.0)))
            (else
              (CallFunction|WrongInput)))))))
  (:Ongoing
    (goto _label)))

(event Input|EnhancedActionEvents|EnhancedInputActionIA_L_Trigger
  (params (ActionValue :type Boolean) (ElapsedSeconds :type Float%20%28double-precision%29) (TriggeredSeconds :type Float%20%28double-precision%29) (InputAction :type Input%20Action%20Object%20Reference :default "/Game/Input/Input_Actions/IA_L_Trigger.IA_L_Trigger"))
  ;[0.15 0.00139 0.1013 0.7913] Trigger Swap
  (:Started
    (if (Math|Boolean|ANDBoolean (Variables|StateBoolean|GetStartCombo) (Variables|StateBoolean|GetIsCooking) (not (Variables|Default|GetIsStunned)))
      (if (Variables|CanDoBoolean|GetCan_L_trigger)
        (Variables|Default|SetInput_Value 8.0)
        (Variables|CanDoBoolean|SetCan_R_trigger true)
        (CallFunction|ComboReset)
        (Variables|CanDoBoolean|SetCan_L_trigger false)
        (elif (not (Variables|StateBoolean|GetBonusInputActive))
          (CallFunction|WrongInput)
          (Variables|CanDoBoolean|SetCan_R_trigger true)
          (Variables|CanDoBoolean|SetCan_L_trigger true))))))

(event Custom|Event_DetectSurface
  (bind _arrow1 (Variables|Default|GetArrow1))
  (bind _returnvalue (Transformation|GetWorldLocation _arrow1))
  (bind _outhit (Collision|LineTraceByChannel (Math|Vector|MakeVector (.x _returnvalue) (.y _returnvalue) (.z _returnvalue)) (Math|Vector|MakeVector (.x _returnvalue) (.y _returnvalue) (- (.z _returnvalue) 1e+02)) "TraceTypeQuery1" false 0 "ForDuration"))
  (switch Utilities|FlowControl|Switch|SwitchonEPhysicalSurface (Collision|GetSurfaceType _outhit)
    (:SurfaceType1
      (CallFunction|EventResetMouvement)
      (Development|PrintString "wood" true true "(R=0.000000,G=0.660000,B=1.000000,A=1.000000)" 2.0 "w"))
    (:SurfaceType2
      (CallFunction|EventSwitchMouvementIce)
      (Development|PrintString "ICe" true true "(R=0.000000,G=0.660000,B=1.000000,A=1.000000)" 2.0 "w"))))

(event Custom|Event_Switch_Mouvement_Ice
  (CallFunction|SetMouvmentSetting 0.05 0.5 2e+01 375.0 2048.0)
  (Variables|Dash|SetDashPower 1e+03))

(event Custom|Event_Reset_Mouvement
  (CallFunction|SetMouvmentSetting 2.0 8.0 2048.0 375.0 2048.0)
  (Variables|Dash|SetDashPower 3e+03))

(event Custom|Start_GroundDetection
  (Utilities|Time|SetTimerbyEvent (delegate Custom|Event_DetectSurface) 1.0 true))

(event Custom|Cook_End_VFX
  ;[0.15 0.15 0.15 0.5] CookEnd
  (Components|Activation|Activate (Variables|Default|GetCookEnd_VFX) false)
  (Utilities|FlowControl|Delay 2.0)
  (Components|Activation|Deactivate (Variables|Default|GetCookEnd_VFX)))

(fn ConstructionScript)

(fn SetMouvmentSetting
  (params (GroundFriction :type Float%20%28double-precision%29) (BreakingDecelerationWalking :type Float%20%28double-precision%29) (BreakingFactor :type Float%20%28double-precision%29) (MaxWalkSpeed :type Float%20%28double-precision%29) (MaxAcceleration :type Float%20%28double-precision%29))
  (Utilities|FlowControl|Sequence
    (:then_0
      (Variables|/Script/Engine.CharacterMovementComponent|SetGroundFriction (Variables|Character|GetCharacterMovement) GroundFriction))
    (:then_1
      (Variables|/Script/Engine.CharacterMovementComponent|SetBrakingFrictionFactor (Variables|Character|GetCharacterMovement) BreakingFactor))
    (:then_2
      (Variables|/Script/Engine.CharacterMovementComponent|SetBrakingDecelerationWalking (Variables|Character|GetCharacterMovement) BreakingDecelerationWalking))
    (:then_3
      (Variables|/Script/Engine.CharacterMovementComponent|SetMaxWalkSpeed (Variables|Character|GetCharacterMovement) MaxWalkSpeed))
    (:then_4
      (Variables|/Script/Engine.CharacterMovementComponent|SetMaxAcceleration (Variables|Character|GetCharacterMovement) MaxAcceleration))))