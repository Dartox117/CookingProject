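; Per-player menu pawn for choosing a character, then a skin, with buttons or stick.
; Input cycles wrapping indices, updating CharacterSelectionMesh and reporting to MenuCharacter by controller ID; the chosen character index is saved to BP_GameInstance for player 1 or 2.
; CanInput and CanTurn guard navigation, skin changes add a short cooldown, and a Gate filters stick input.
; Back undoes each stage; a debug key loads a test level.
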(event Custom|Change
  (Default|Change (Variables|Default|GetMenuCharacter) (Variables|Default|GetIDcontroller) (Variables|Default|GetActualSelection)))

(event Custom|SelectedCharacter
  (switch int (Variables|Default|GetIDcontroller)
    (:0
      (Variables|/Game/Blueprints/GameInstance/BP_GameInstance.BP_GameInstance_C|SetRig_Index_Player_1 (Variables|Default|GetAs%20BP%20Game%20Instance) (Variables|Default|GetActualSelection)))
    (:1
      (Variables|/Game/Blueprints/GameInstance/BP_GameInstance.BP_GameInstance_C|SetRig_Index_Player_2 (Variables|Default|GetAs%20BP%20Game%20Instance) (Variables|Default|GetActualSelection)))))

(event Custom|MenuRight
  (if (and (Variables|Default|GetCanTurn) (Variables|Default|GetCanInput))
    (if (not (Variables|Default|GetIsCharaSelected))
      (Math|Integer|IncrementInt (Variables|Default|GetActualSelection)
        (:%20%20
          (if (>= (Variables|Default|GetActualSelection) 4)
            (Variables|Default|SetActualSelection 0))
          (CallFunction|Change)
          (Default|RightTurn (Variables|Default|GetCharacterSelectionMesh) (Variables|Default|GetActualSelection))
          (Variables|Default|SetSkinSelection (Variables|Default|GetActualSelection))))
      (else
        (Math|Integer|IncrementInt (Variables|Default|GetSkinSelection)
          (:%20%20
            (if (>= (Variables|Default|GetSkinSelection) 5)
              (Variables|Default|SetSkinSelection 0))
            (Default|SkinSelection (Variables|Default|GetMenuCharacter) (Variables|Default|GetIDcontroller) (Variables|Default|GetSkinSelection))
            (Variables|Default|SetCanTurn false)
            (Default|SetMaterial (Variables|Default|GetCharacterSelectionMesh) (Variables|Default|GetSkinSelection))
            (Utilities|FlowControl|Delay 0.2)
            (Variables|Default|SetCanTurn true)))))))

(event Custom|MenuLeft
  (if (and (Variables|Default|GetCanTurn) (Variables|Default|GetCanInput))
    (if (not (Variables|Default|GetIsCharaSelected))
      (Math|Integer|DecrementInt (Variables|Default|GetActualSelection)
        (:%20%20
          (if (<= (Variables|Default|GetActualSelection) -1)
            (Variables|Default|SetActualSelection 3))
          (CallFunction|Change)
          (Default|LeftTurn (Variables|Default|GetCharacterSelectionMesh) (Variables|Default|GetActualSelection))
          (Variables|Default|SetSkinSelection (Variables|Default|GetActualSelection))))
      (else
        (Math|Integer|DecrementInt (Variables|Default|GetSkinSelection)
          (:%20%20
            (if (<= (Variables|Default|GetSkinSelection) -1)
              (Variables|Default|SetSkinSelection 4))
            (Default|SkinSelection (Variables|Default|GetMenuCharacter) (Variables|Default|GetIDcontroller) (Variables|Default|GetSkinSelection))
            (Default|SetMaterial (Variables|Default|GetCharacterSelectionMesh) (Variables|Default|GetSkinSelection))
            (Variables|Default|SetCanTurn false)
            (Utilities|FlowControl|Delay 0.2)
            (Variables|Default|SetCanTurn true)))))))

(event Custom|OpenGate
  (Utilities|FlowControl|Gate false) ; enters at Open
)

(event Custom|CloseGate
  (Utilities|FlowControl|Gate false) ; enters at Close
)

(event Custom|SkinSelected
  (Variables|Default|SetIsSkinSelected true)
  (Default|PlaySelectionAnim (Variables|Default|GetCharacterSelectionMesh)))

(event Custom|FallAnim
  (Default|FallAnim (Variables|Default|GetCharacterSelectionMesh)))

(event Input|EnhancedActionEvents|EnhancedInputActionIA_MenuLeft
  (params (ActionValue :type Boolean) (ElapsedSeconds :type Float%20%28double-precision%29) (TriggeredSeconds :type Float%20%28double-precision%29) (InputAction :type Input%20Action%20Object%20Reference :default "/Game/Blueprints/MenuManager/Input/IA_MenuLeft.IA_MenuLeft"))
  (:Started
    (if (and (Variables|Default|GetCanTurn) (Variables|Default|GetCanInput))
      (if (not (Variables|Default|GetIsCharaSelected))
        (Math|Integer|DecrementInt (Variables|Default|GetActualSelection)
          (:%20%20
            (if (<= (Variables|Default|GetActualSelection) -1)
              (Variables|Default|SetActualSelection 3))
            (CallFunction|Change)
            (Default|LeftTurn (Variables|Default|GetCharacterSelectionMesh) (Variables|Default|GetActualSelection))
            (Variables|Default|SetSkinSelection (Variables|Default|GetActualSelection))))
        (else
          (Math|Integer|DecrementInt (Variables|Default|GetSkinSelection)
            (:%20%20
              (if (<= (Variables|Default|GetSkinSelection) -1)
                (Variables|Default|SetSkinSelection 4))
              (Default|SkinSelection (Variables|Default|GetMenuCharacter) (Variables|Default|GetIDcontroller) (Variables|Default|GetSkinSelection))
              (Default|SetMaterial (Variables|Default|GetCharacterSelectionMesh) (Variables|Default|GetSkinSelection))
              (Variables|Default|SetCanTurn false)
              (Utilities|FlowControl|Delay 0.2)
              (Variables|Default|SetCanTurn true))))))))

(event Input|EnhancedActionEvents|EnhancedInputActionIA_MenuRight
  (params (ActionValue :type Boolean) (ElapsedSeconds :type Float%20%28double-precision%29) (TriggeredSeconds :type Float%20%28double-precision%29) (InputAction :type Input%20Action%20Object%20Reference :default "/Game/Blueprints/MenuManager/Input/IA_MenuRight.IA_MenuRight"))
  (:Started
    (if (and (Variables|Default|GetCanTurn) (Variables|Default|GetCanInput))
      (if (not (Variables|Default|GetIsCharaSelected))
        (Math|Integer|IncrementInt (Variables|Default|GetActualSelection)
          (:%20%20
            (if (>= (Variables|Default|GetActualSelection) 4)
              (Variables|Default|SetActualSelection 0))
            (CallFunction|Change)
            (Default|RightTurn (Variables|Default|GetCharacterSelectionMesh) (Variables|Default|GetActualSelection))
            (Variables|Default|SetSkinSelection (Variables|Default|GetActualSelection))))
        (else
          (Math|Integer|IncrementInt (Variables|Default|GetSkinSelection)
            (:%20%20
              (if (>= (Variables|Default|GetSkinSelection) 5)
                (Variables|Default|SetSkinSelection 0))
              (Default|SkinSelection (Variables|Default|GetMenuCharacter) (Variables|Default|GetIDcontroller) (Variables|Default|GetSkinSelection))
              (Variables|Default|SetCanTurn false)
              (Default|SetMaterial (Variables|Default|GetCharacterSelectionMesh) (Variables|Default|GetSkinSelection))
              (Utilities|FlowControl|Delay 0.2)
              (Variables|Default|SetCanTurn true))))))))

(event Input|EnhancedActionEvents|EnhancedInputActionIA_Select
  (params (ActionValue :type Boolean) (ElapsedSeconds :type Float%20%28double-precision%29) (TriggeredSeconds :type Float%20%28double-precision%29) (InputAction :type Input%20Action%20Object%20Reference :default "/Game/Blueprints/MenuManager/Input/IA_Select.IA_Select"))
  (:Started
    (if (Variables|Default|GetCanInput)
      (if (not (Variables|Default|GetIsCharaSelected))
        (CallFunction|SelectedCharacter)
        (Default|SelectChara (Variables|Default|GetMenuCharacter) (Variables|Default|GetIDcontroller) (Variables|Default|GetActualSelection))
        (else
          (Default|ConfirmSkin (Variables|Default|GetMenuCharacter) (Variables|Default|GetIDcontroller) (Variables|Default|GetSkinSelection)))))))

(event Input|EnhancedActionEvents|EnhancedInputActionIA_Back
  (params (ActionValue :type Boolean) (ElapsedSeconds :type Float%20%28double-precision%29) (TriggeredSeconds :type Float%20%28double-precision%29) (InputAction :type Input%20Action%20Object%20Reference :default "/Game/Blueprints/MenuManager/Input/IA_Back.IA_Back"))
  (:Started
    (if (Variables|Default|GetCanInput)
      (if (not (Variables|Default|GetIsSkinSelected))
        (Default|UnselectChara (Variables|Default|GetMenuCharacter) (Variables|Default|GetIDcontroller))
        (CallFunction|OpenGate)
        (Default|SkinSelection (Variables|Default|GetMenuCharacter) (Variables|Default|GetIDcontroller) (Variables|Default|GetActualSelection))
        (Default|SetMaterial (Variables|Default|GetCharacterSelectionMesh) (Variables|Default|GetActualSelection))
        (else
          (Variables|Default|SetIsSkinSelected false)
          (Default|CancelSkin (Variables|Default|GetMenuCharacter) (Variables|Default|GetIDcontroller)))))))

(event Input|EnhancedActionEvents|EnhancedInputActionIA_MenuStick
  (params (ActionValue :type Float%20%28double-precision%29) (ElapsedSeconds :type Float%20%28double-precision%29) (TriggeredSeconds :type Float%20%28double-precision%29) (InputAction :type Input%20Action%20Object%20Reference :default "/Game/Blueprints/MenuManager/Input/IA_MenuStick.IA_MenuStick"))
  (Utilities|FlowControl|Gate false
    (:Exit
      (if (Math|Float|NearlyEqual(Float) ActionValue 1.0 0.2)
        (CallFunction|MenuRight)
        (elif (Math|Float|NearlyEqual(Float) ActionValue -1.0 0.2)
          (CallFunction|MenuLeft))))))

(event EventBeginPlay
  (bind _asbp_game_instance (Utilities|Casting|CastToBP_GameInstance (Game|GetGameInstance)))
  (Variables|Default|SetAs%20BP%20Game%20Instance _asbp_game_instance))

(event Collision|EventActorBeginOverlap
  (params (OtherActor :type Actor%20Object%20Reference)))

(event EventTick
  (params (DeltaSeconds :type Float%20%28single-precision%29)))

(event Input|KeyboardEvents|DebugKeyT
  (params (Key :type Key%20Structure :default "None") (ActionValue :type Input%20Action%20Value%20Structure))
  (:Pressed
    (Game|OpenLevel(byName) "Small_Test")))

(event Input|KeyboardEvents|DebugKeyV
  (params (Key :type Key%20Structure :default "None") (ActionValue :type Input%20Action%20Value%20Structure)))

(fn ConstructionScript)