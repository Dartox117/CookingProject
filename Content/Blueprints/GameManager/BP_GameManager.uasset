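; Game manager for a two-player cooking game: runs input combos, scoring, HUD, pause and the win screen.
; Combos feed player input to HUD widgets, score cooked ingredients with a multiplier, then fire their alterations through timers named after the enum.
; Alteration events read DT_Alteration data to speed conveyors, add components to players or stun opponents.
; It also broadcasts conveyor speed each Tick and provides weighted random alteration rolls.
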(event Custom|PauseGame
  (if (not (Game|IsGamePaused))
    (Game|SetGamePaused true)
    (bind _returnvalue (UserInterface|CreateWidget "/Game/Blueprints/Widget/WG_Pause.WG_Pause_C" (Game|GetPlayerController 0)))
    (bind _output_get (Variables|ObjectRef|SetRef_WG_Pause _returnvalue))
    (UserInterface|Viewport|AddtoViewport _output_get 0)
    (Variables|/Script/Engine.PlayerController|SetbShowMouseCursor (Game|GetPlayerController 0) true)
    (Input|SetInputModeGameandUI (Game|GetPlayerController 0) (Variables|ObjectRef|GetRef_WG_Pause) "DoNotLock" true false)
    (else
      (Game|SetGamePaused false)
      (Widget|RemovefromParent (Variables|ObjectRef|GetRef_WG_Pause))
      (Input|SetInputModeGameOnly (Game|GetPlayerController 0) false)
      (Variables|/Script/Engine.PlayerController|SetbShowMouseCursor (Game|GetPlayerController 0) false))))

(event Custom|ActiveBonus
  (params (NewParam :type Array%20of%20ST%20Foods%20Structures) (playerValue :type Integer))
  ;[0.15 0.15 0.15 0.5] Active le bonus si l'aliment possède un bonus et si il est cuit
  (Variables|Default|SetPlayerBonus playerValue)
  (for _array_element NewParam
    (if (.Cooked (Utilities|Struct|BreakST_Foods _array_element))
      (Utilities|Time|SetTimerbyFunctionName 0 (Utilities|String|EnumtoString (.Alteration (Utilities|Struct|BreakST_Foods _array_element))) 0.1))))

(event Custom|Event_Set_Convoyeur
  (params (Ref_Tapis :type BP%20Tapis%20Qui%20Roule%20Object%20Reference))
  ;[0.0298 0.15 0.09166 0.5] Conveyor Belt
  ;;[0.15 0.15 0.15 0.5] Get all the ingrediant spawner
  (Utilities|Array|Add (Variables|Storage|GetStorage_Ref_Convoyer) Ref_Tapis))

(event Custom|Event_Binding_Dispacher
  ;[0.0298 0.15 0.09166 0.5] Conveyor Belt
  ;;[0.15 0.15 0.15 0.5] Get all the ingrediant spawner
  (EventDispatchers|BindEventtoEDListenConveyor (delegate Custom|Event_Set_Convoyeur)))

(event Custom|Event_Instance%20Setting
  ;[0.1495 0.15 0.04701 0.5] GameInstance Setting
  (bind _asbp_game_instance (Utilities|Casting|CastToBP_GameInstance (Game|GetGameInstance)))
  (Variables|/Game/Blueprints/GameInstance/BP_GameInstance.BP_GameInstance_C|SetRef_GameManager _asbp_game_instance self))

(event Custom|EndGameManaging
  (params (Player :type Integer))
  ;[0.15 0.15 0.15 0.5] EndGame Temporaire
  (bind _returnvalue (UserInterface|CreateWidget "/Game/Blueprints/Widget/WG_Win.WG_Win_C"))
  (bind _output_get (Variables|Default|SetWinScreen _returnvalue))
  (UserInterface|Viewport|AddtoViewport _output_get 0)
  (Default|AffichageWin (Variables|Default|GetWinScreen) Player (Variables|Score|GetPlayer_1_Score) (Variables|Score|GetPlayer_2_Score)))

(event EventBeginPlay
  ;[0.003705 0.485 0] Begin Play
  (CallFunction|EventBindingDispacher)
  (CallFunction|EventInstanceSetting)
  (CallFunction|ToolsGettingAlterationData)
  ;[0.15 0.15 0.15 0.5] Creer le hud
  (bind _returnvalue (UserInterface|CreateWidget "/Game/Blueprints/Widget/WG_HUD.WG_HUD_C" 0 self))
  (bind _output_get (Variables|ObjectRef|SetHUD_Ref _returnvalue))
  (UserInterface|Viewport|AddtoViewport _output_get 0)
  (Input|SetInputModeGameOnly (Game|GetPlayerController 0) false))

(event Custom|GoingCrazy
  ;[1 0.2524 0.9479 0.5] GoingCrazy
  (Development|PrintString "GoingCRAAAAAzy")
  (bind _asbp_player (Utilities|Casting|CastToBP_Player (Game|Player|GetPlayerPawn (Variables|Default|GetPlayerBonus))))
  (bind _returnvalue (AddComponent|AddBPCTestPlayer _asbp_player))
  (Utilities|FlowControl|Delay (.duration (.Value (Utilities|Map|Find (Variables|Storage|GetStorage_Alteration) "NewEnumerator8"))))
  (Default|DestroySelf _returnvalue))

(event Custom|Bank%20Tiket
  ;[0 0.15 0.01477 0.5] BankTiket
  (Development|PrintString "BAAAAAm")
  (switch int (Variables|Default|GetPlayerBonus)
    (:0
      (bind _returnvalue (Game|SpawnActorfromClass "/Game/Blueprints/Gameplay/BP_MoneySafe.BP_MoneySafe_C" (Math|Transform|MakeTransform "0, 0, 0" "0, 0, 0" "1.000000,1.000000,1.000000") "Undefined" "MultiplyWithRoot" 0 0))
      (bind _asbp_player (Utilities|Casting|CastToBP_Player (Game|Player|GetPlayerPawn 1)))
      (Default|Stun _returnvalue _asbp_player))
    (:1
      (bind _returnvalue_2 (Game|SpawnActorfromClass "/Game/Blueprints/Gameplay/BP_MoneySafe.BP_MoneySafe_C" (Math|Transform|MakeTransform "0, 0, 0" "0, 0, 0" "1.000000,1.000000,1.000000") "Undefined" "MultiplyWithRoot" 0 0))
      (bind _asbp_player_2 (Utilities|Casting|CastToBP_Player (Game|Player|GetPlayerPawn 0)))
      (Default|Stun _returnvalue_2 _asbp_player_2))))

(event Custom|GymAds
  ;[0.3517 0.08057 0.7031 0.5] GymAds
  (Development|PrintString "ET LE BIBI")
  (switch int (Variables|Default|GetPlayerBonus)
    (:0
      (bind _asbp_player (Utilities|Casting|CastToBP_Player (Game|Player|GetPlayerPawn 1)))
      (bind _returnvalue (AddComponent|AddBPCGymAds _asbp_player))
      (Utilities|FlowControl|Delay (.Duration (Utilities|Struct|BreakST_Alteration (.Value (Utilities|Map|Find (Variables|Storage|GetStorage_Alteration) "NewEnumerator6")))))
      (Default|EndEffect _returnvalue))
    (:1
      (bind _asbp_player_2 (Utilities|Casting|CastToBP_Player (Game|Player|GetPlayerPawn 0)))
      (bind _returnvalue_2 (AddComponent|AddBPCGymAds _asbp_player_2))
      (Utilities|FlowControl|Delay (.Duration (Utilities|Struct|BreakST_Alteration (.Value (Utilities|Map|Find (Variables|Storage|GetStorage_Alteration) "NewEnumerator6")))))
      (Default|EndEffect _returnvalue_2))))

(event Custom|Default
  (Development|PrintString "Ya pas de pouvoir chef"))

(event Custom|Clown%20shoes
  ;[0.15 0.06996 0.01121 0.5] ClownShoes
  (switch int (Variables|Default|GetPlayerBonus)
    (:0
      (bind _asbp_player (Utilities|Casting|CastToBP_Player (Game|Player|GetPlayerPawn 1)))
      (bind _returnvalue (AddComponent|AddBPCSlowPlayer _asbp_player))
      (Utilities|FlowControl|Delay (.Duration (Utilities|Struct|BreakST_Alteration (.Value (Utilities|Map|Find (Variables|Storage|GetStorage_Alteration) "NewEnumerator5")))))
      (Default|DestroySelf _returnvalue))
    (:1
      (bind _asbp_player_2 (Utilities|Casting|CastToBP_Player (Game|Player|GetPlayerPawn 0)))
      (bind _returnvalue_2 (AddComponent|AddBPCSlowPlayer _asbp_player_2))
      (Utilities|FlowControl|Delay (.Duration (Utilities|Struct|BreakST_Alteration (.Value (Utilities|Map|Find (Variables|Storage|GetStorage_Alteration) "NewEnumerator5")))))
      (Default|DestroySelf _returnvalue_2))))

(event Custom|Broken%20Clock
  (bind _storage_alteration (Variables|Storage|GetStorage_Alteration))
  (bind _value (Utilities|Map|Find _storage_alteration "NewEnumerator0"))
  ;[0.1388 0.2482 0.4844 0.5] Broken Clock
  (Rendering|Material|SetScalarParameterValue "/Game/Blueprints/MPC/ConvoyerSpeed.ConvoyerSpeed" "Speed" -3.0 :!class /Script/Engine.KismetMaterialLibrary)
  (Development|PrintString "StartSpeed")
  (Variables|Setting|SetConveyor_Speed (+ (Variables|Setting|GetConveyor_Speed) (.value _value)))
  (Utilities|FlowControl|Delay (.duration _value))
  (Variables|Setting|SetConveyor_Speed (- (Variables|Setting|GetConveyor_Speed) (.value _value)))
  (Development|PrintString "EndSpeed")
  (Rendering|Material|SetScalarParameterValue "/Game/Blueprints/MPC/ConvoyerSpeed.ConvoyerSpeed" "Speed" -1.5 :!class /Script/Engine.KismetMaterialLibrary))

(event Custom|Tools_Getting_AlterationData
  ;[0.15 0.08531 0.000295 0.5] Get alteration Data
  (Utilities|Map|Clear (Variables|Storage|GetStorage_Alteration))
  (bind _returnvalue (Utilities|MacroReadDataTable "/Game/Blueprints/Structures_Data/DT_Alteration.DT_Alteration"))
  (Variables|Temp|SetTemp_Alteration_Row _returnvalue)
  (Utilities|Map|Add (Variables|Storage|GetStorage_Alteration) (.name (Variables|Temp|GetTemp_Alteration_Row)) (Variables|Temp|GetTemp_Alteration_Row)))

(event EventTick
  (params (DeltaSeconds :type Float%20%28single-precision%29))
  ;[0.15 0.002256 0 0.5] Conveyor Clock
  (Default|CallEDCallConveyor (Variables|Setting|GetConveyor_Speed)))

(event Custom|AddScore
  (params (player :type Integer) (points :type Integer))
  ;[0.15 0.15 0.15 0.5] AddScore
  ;;[0.04956 0.15 0.06706 0.5] mise à jour du score en fonction du player et des points des aliments
  (switch int player
    (:0
      (bind _output_get (Variables|Score|SetPlayer_1_Score (+ (Variables|Score|GetPlayer_1_Score) (* (Variables|Score|GetMultiplicateur_P1) points))))
      (Default|Player1Score (Variables|ObjectRef|GetHUD_Ref) _output_get)
      (Default|AddPointsP1 (Variables|ObjectRef|GetHUD_Ref) (* (Variables|Score|GetMultiplicateur_P1) (Variables|Score|Getpoints_Combo_P1)))
      (Variables|Score|SetMultiplicateur_P1 0)
      (Variables|Score|Setpoints_Combo_P1 0))
    (:1
      (bind _output_get_2 (Variables|Score|SetPlayer_2_Score (+ (Variables|Score|GetPlayer_2_Score) (* points (Variables|Score|GetMultiplicateur_P2)))))
      (Default|Player2Score (Variables|ObjectRef|GetHUD_Ref) _output_get_2)
      (Default|AddPointsP2 (Variables|ObjectRef|GetHUD_Ref) (* (Variables|Score|GetMultiplicateur_P2) (Variables|Score|Getpoints_Combo_P2)))
      (Variables|Score|SetMultiplicateur_P2 0)
      (Variables|Score|Setpoints_Combo_P2 0))))

(event Custom|StartCombo
  (params (Player :type Integer) (Food_Struct :type Array%20of%20ST%20Foods%20Structures) (PlanDeTravailRef :type BP%20Plan%20De%20Travail%20Object%20Reference))
  (bind _hud_ref (Variables|ObjectRef|GetHUD_Ref))
  (bind _hud_ref_2 (Variables|ObjectRef|GetHUD_Ref))
  (bind _wg_input_1 (Variables|/Game/Blueprints/Widget/WG_HUD.WG_HUD_C|GetWG_Input_1 _hud_ref))
  (bind _wg_input (Variables|/Game/Blueprints/Widget/WG_HUD.WG_HUD_C|GetWG_Input _hud_ref_2))
  ;[0.15 0.15 0.15 0.5] Show Input
  ;;[0.07192 0.1477 0.15 0.5] Affiche la page d'input du joueur correspondant
  (switch int Player
    (:0
      (Variables|ObjectRef|SetPlan%20De%20Travail_Player_1_Ref PlanDeTravailRef)
      (Variables|Default|SetSt_Food_Player_1 Food_Struct)
      (Widget|SetRenderOpacity _wg_input 1.0)
      (Default|ChangeInput _wg_input (Variables|Default|GetSt_Food_Player_1))
      (Variables|/Game/Blueprints/Widget/WG_Input.WG_Input_C|SetPogressBar _wg_input 0.0))
    (:1
      (Variables|ObjectRef|SetPlan%20De%20Travail_Player_2_Ref PlanDeTravailRef)
      (Variables|Default|SetSt_Food_Player_2 Food_Struct)
      (Widget|SetRenderOpacity _wg_input_1 1.0)
      (Default|ChangeInput _wg_input_1 (Variables|Default|GetST_Food_Player_2))
      (Variables|/Game/Blueprints/Widget/WG_Input.WG_Input_C|SetPogressBar _wg_input_1 0.0))))

(event Custom|FinishedCombo
  (params (Player :type Integer) (ST_Food :type Array%20of%20ST%20Foods%20Structures))
  (bind _hud_ref (Variables|ObjectRef|GetHUD_Ref))
  (bind _hud_ref_2 (Variables|ObjectRef|GetHUD_Ref))
  (bind _hud_ref_3 (Variables|ObjectRef|GetHUD_Ref))
  (bind _hud_ref_4 (Variables|ObjectRef|GetHUD_Ref))
  (bind _wg_input (Variables|/Game/Blueprints/Widget/WG_HUD.WG_HUD_C|GetWG_Input _hud_ref_2))
  (bind _wg_input_1 (Variables|/Game/Blueprints/Widget/WG_HUD.WG_HUD_C|GetWG_Input_1 _hud_ref))
  (bind _wg_input_2 (Variables|/Game/Blueprints/Widget/WG_HUD.WG_HUD_C|GetWG_Input _hud_ref_3))
  (bind _wg_input_1_2 (Variables|/Game/Blueprints/Widget/WG_HUD.WG_HUD_C|GetWG_Input_1 _hud_ref_4))
  ;[0.15 0.15 0.15 0.5] EndCombo
  ;;[0.02291 0.05721 0.15 0.5] Quand le combo est fini, on parcours l'array du joueur correspondant pour comptabilisé les points et si l'aliment a été cuit
  (bind _output_get (Variables|Default|SetPlayer%20Value Player))
  (switch int _output_get
    (:0
      (for _array_element (Variables|Default|GetST_Food_Player_1)
        (if (.Cooked (Utilities|Struct|BreakST_Foods _array_element))
          (Variables|Score|Setpoints_Combo_P1 (+ (Variables|Score|Getpoints_Combo_P1) (.Points (Utilities|Struct|BreakST_Foods _array_element))))
          (Math|Integer|IncrementInt (Variables|Score|GetMultiplicateur_P1))))
      (CallFunction|AddScore _output_get (Variables|Score|Getpoints_Combo_P1))
      (Variables|/Game/Blueprints/Widget/WG_Input.WG_Input_C|SetActualInput _wg_input 0)
      (Variables|/Game/Blueprints/Widget/WG_Input.WG_Input_C|SetPogressBar _wg_input 1e+02)
      (Utilities|FlowControl|Delay 1.0)
      (Widget|SetRenderOpacity _wg_input_2 0.0)
      (Default|ResetProgressBar _wg_input_2)
      (CallFunction|ActiveBonus (Variables|Default|GetST_Food_Player_1) (Variables|Default|GetPlayer%20Value)))
    (:1
      (for _array_element_2 (Variables|Default|GetST_Food_Player_2)
        (if (.Cooked (Utilities|Struct|BreakST_Foods _array_element_2))
          (Variables|Score|Setpoints_Combo_P2 (+ (Variables|Score|Getpoints_Combo_P2) (.Points (Utilities|Struct|BreakST_Foods _array_element_2))))
          (Math|Integer|IncrementInt (Variables|Score|GetMultiplicateur_P2))))
      (CallFunction|AddScore _output_get (Variables|Score|Getpoints_Combo_P2))
      (Variables|/Game/Blueprints/Widget/WG_Input.WG_Input_C|SetActualInput _wg_input_1 0)
      (Variables|/Game/Blueprints/Widget/WG_Input.WG_Input_C|SetPogressBar _wg_input_1 1e+02)
      (Utilities|FlowControl|Delay 1.0)
      (Widget|SetRenderOpacity _wg_input_1_2 0.0)
      (Default|ResetProgressBar _wg_input_1_2)
      (CallFunction|ActiveBonus (Variables|Default|GetST_Food_Player_2) (Variables|Default|GetPlayer%20Value)))))

(event Custom|GetInput
  (params (Player :type Integer) (InputValu :type Float%20%28double-precision%29))
  (bind _st_food_player_1 (Variables|Default|GetST_Food_Player_1))
  (bind _st_food_player_2 (Variables|Default|GetST_Food_Player_2))
  (bind _hud_ref (Variables|ObjectRef|GetHUD_Ref))
  (bind _hud_ref_2 (Variables|ObjectRef|GetHUD_Ref))
  (bind _plan_de_travail_player_1_ref (Variables|ObjectRef|GetPlan%20De%20Travail_Player_1_Ref))
  (bind _plan_de_travail_player_2_ref (Variables|ObjectRef|GetPlan%20De%20Travail_Player_2_Ref))
  (bind _wg_input (Variables|/Game/Blueprints/Widget/WG_HUD.WG_HUD_C|GetWG_Input _hud_ref_2))
  (bind _wg_input_1 (Variables|/Game/Blueprints/Widget/WG_HUD.WG_HUD_C|GetWG_Input_1 _hud_ref))
  (bind _actualinput (Variables|/Game/Blueprints/Widget/WG_Input.WG_Input_C|GetActualInput _wg_input_1))
  (bind _actualinput_2 (Variables|/Game/Blueprints/Widget/WG_Input.WG_Input_C|GetActualInput _wg_input))
  (bind _returnvalue (- _actualinput 1))
  (bind _returnvalue_2 (- _actualinput_2 1))
  (bind _output (Utilities|Array|Get(acopy) _st_food_player_2 _returnvalue))
  (bind _output_2 (Utilities|Array|Get(acopy) _st_food_player_1 _returnvalue_2))
  ;[0.15 0.15 0.15 0.5] GetInput
  ;;[0.15 0.000403 0.1252 0.5] Recupere la valeur d'input et l'envoie au widget d'input, verifie egalement si le combo est fini, si c'est le cas, passage à l'input suivant et comtabilisation
  (switch int Player
    (:0
      (Default|GetInput _wg_input InputValu _plan_de_travail_player_1_ref)
      (if (Variables|/Game/Blueprints/Widget/WG_Input.WG_Input_C|GetIsFinished _wg_input)
        (Utilities|Array|SetArrayElem _st_food_player_1 _returnvalue_2 (Utilities|Struct|MakeST_Foods (.index _output_2) (.foodname _output_2) (.input _output_2) (.points _output_2) (.staticmesh _output_2) true (.bonus _output_2) (.alteration _output_2))))
      (Default|SwitchCombo _plan_de_travail_player_1_ref))
    (:1
      (Default|GetInput _wg_input_1 InputValu _plan_de_travail_player_2_ref)
      (if (Variables|/Game/Blueprints/Widget/WG_Input.WG_Input_C|GetIsFinished _wg_input_1)
        (Utilities|Array|SetArrayElem _st_food_player_2 _returnvalue (Utilities|Struct|MakeST_Foods (.index _output) (.foodname _output) (.input _output) (.points _output) (.staticmesh _output) true (.bonus _output) (.alteration _output))))
      (Default|SwitchCombo _plan_de_travail_player_2_ref))))

(event Custom|WrongInput
  (params (Player :type Integer))
  ;[0.07351 0.15 0.1446 0.5] Erreur de Combo
  (switch int Player
    (:0
      (Default|ErrorCombo (Variables|/Game/Blueprints/Widget/WG_HUD.WG_HUD_C|GetWG_Input (Variables|ObjectRef|GetHUD_Ref))))
    (:1
      (Default|ErrorCombo (Variables|/Game/Blueprints/Widget/WG_HUD.WG_HUD_C|GetWG_Input_1 (Variables|ObjectRef|GetHUD_Ref))))))

(event Custom|EndGame
  ;[1 0.02223 0 0.5] Endgame
  (if (> (Variables|Score|GetPlayer_1_Score) (Variables|Score|GetPlayer_2_Score))
    (CallFunction|EndGameManaging)
    (elif (< (Variables|Score|GetPlayer_1_Score) (Variables|Score|GetPlayer_2_Score))
      (CallFunction|EndGameManaging 1)
      (else
        (CallFunction|EndGameManaging 2)))))

(fn ConstructionScript)

(fn FunctionCalculateSum
  (bind _values (Utilities|Map|Values (Variables|Default|GetBonusMap)))
  (for _array_element _values
    (LocalVariables|SetTotal (+ (LocalVariables|GetTotal) _array_element)))
  (return (LocalVariables|GetTotal)))

(fn FunctionChooseEvent
  (LocalVariables|SetRandomFloat (Math|Random|RandomFloatinRange 0.0 (Variables|Default|GetValueSum)))
  (bind _keys (Utilities|Map|Keys (Variables|Default|GetBonusMap)))
  (for _array_element _keys
    (if (< (LocalVariables|GetRandomFloat) (.Value (Utilities|Map|Find (Variables|Default|GetBonusMap) _array_element)))
      (return _array_element)
      (else
        (LocalVariables|SetRandomFloat (- (LocalVariables|GetRandomFloat) (.Value (Utilities|Map|Find (Variables|Default|GetBonusMap) _array_element))))))))

(fn FunctionSelectAlteration
  (params (Roll :type Float%20%28double-precision%29))
  (LocalVariables|SetLocal_Roll Roll)
  (bind (_keypin _valuepin) (Utilities|Map|ForEachLoop(Map) (Variables|Storage|GetStorage_Alteration))
    (:then
      (LocalVariables|SetLocal_AlterationCandidate _keypin)
      (LocalVariables|SetLocal_Sum (+ (LocalVariables|GetLocal_Sum) (.probability _valuepin)))
      (if (>= (LocalVariables|GetLocal_Sum) (LocalVariables|GetLocal_Roll))
        (return (LocalVariables|GetLocal_AlterationCandidate))))))

(fn FunctionSumOfProbabilityAlteration
  (bind _valuepin (Utilities|Map|ForEachLoop(Map) (Variables|Storage|GetStorage_Alteration))
    (:then
      (LocalVariables|SetLocal_Sum_Alteration_Probability (+ (.probability _valuepin) (LocalVariables|GetLocal_Sum_Alteration_Probability))))
    (:CompletedPin
      (return (LocalVariables|GetLocal_Sum_Alteration_Probability)))))

(fn FunctionRollAlteration
  (bind _sum_alteration_probability (CallFunction|FunctionSumOfProbabilityAlteration))
  (Development|PrintString (Utilities|String|ToString(Float) (Math|Random|RandomFloatinRange 0.0 _sum_alteration_probability)) true true "(R=1.000000,G=0.933157,B=0.000000,A=1.000000)" 2.0 "RNG")
  (bind _selected_alteration (CallFunction|FunctionSelectAlteration (Math|Random|RandomFloatinRange 0.0 _sum_alteration_probability)))
  (Development|PrintString (Utilities|String|EnumtoString _selected_alteration) true true "(R=1.000000,G=0.971795,B=0.000000,A=1.000000)" 2.0 "NAME")
  (return _selected_alteration))