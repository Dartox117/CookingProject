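; Wind hazard actor that shows timed gusts and pushes the player along its Direction component.
; On play it fetches the game manager via the game instance and calls its wind setup event after a short delay.
; The spawn event runs the wind effect for a given duration after a random delay, toggling IsActive.
; Capsule overlap with the player's root loops a timer that launches them horizontally by WindPower, regardless of IsActive.
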(event OnComponentBeginOverlap(Capsule)
  (params (OverlappedComponent :type Primitive%20Component%20Object%20Reference) (OtherActor :type Actor%20Object%20Reference) (OtherComp :type Primitive%20Component%20Object%20Reference) (OtherBodyIndex :type Integer) (bFromSweep :type Boolean) (SweepResult :type Hit%20Result%20Structure%20%28by%20ref%29))
  ;[0.2324 1 0.5898] Wind Effect
  (bind _asbp_player (Utilities|Casting|CastToBP_Player OtherActor))
  (if (== OtherComp (Variables|/Script/Engine.Actor|GetRootComponent _asbp_player))
    (bind _returnvalue (Utilities|Time|SetTimerbyEvent (delegate Custom|CustomEvent) 0.1 true))
    (Variables|Default|SetTimer%20handle _returnvalue)))

(event OnComponentEndOverlap(Capsule)
  (params (OverlappedComponent :type Primitive%20Component%20Object%20Reference) (OtherActor :type Actor%20Object%20Reference) (OtherComp :type Primitive%20Component%20Object%20Reference) (OtherBodyIndex :type Integer))
  (bind _asbp_player (Utilities|Casting|CastToBP_Player OtherActor))
  (if (== OtherComp (Variables|/Script/Engine.Actor|GetRootComponent _asbp_player))
    (Utilities|Time|ClearandInvalidateTimerbyHandle (Variables|Default|GetTimer%20handle))))

(event Custom|Event_Spawn_Wind
  (params (ActivationTime :type Float%20%28double-precision%29))
  ;[1 0.9332 0] Spawn
  (Utilities|FlowControl|Delay (Math|Random|RandomFloatinRange 0.5 1.0))
  (Variables|Default|SetIsActive true)
  (Components|Activation|Activate (Variables|Default|GetNG_Wind) false)
  (Utilities|FlowControl|Delay ActivationTime)
  (Components|Activation|SetActive (Variables|Default|GetNG_Wind) false false)
  (Variables|Default|SetIsActive false))

(event Custom|CustomEvent
  (bind _direction (Variables|Default|GetDirection))
  (bind _returnvalue (Math|Vector|GetForwardVector _direction))
  ;[0.2324 1 0.5898] Wind Effect
  (Character|LaunchCharacter (stale OnComponentBeginOverlap(Capsule) _asbp_player) (* (Math|Vector|MakeVector (.x _returnvalue) (.y _returnvalue) 0.0) (Variables|Default|GetWindPower)) true false))

(event EventBeginPlay
  ;[0.003705 0.485 0] Begin play
  ;;[0 0 0] Reference Setting
  (Utilities|McGetGameManager)
  (Utilities|FlowControl|Delay 0.2)
  (Default|EventSetWind (Variables|Default|GetRef%20Game%20Manager)))

(fn ConstructionScript
  (Variables|Default|SetStart_Location (Transformation|GetWorldLocation (Variables|Default|GetStart)))
  (Variables|Default|SetEnd_Location (Transformation|GetWorldLocation (Variables|Default|GetEnd))))