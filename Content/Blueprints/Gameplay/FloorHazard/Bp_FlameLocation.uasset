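; Floor hazard flame point that, when triggered, burns the player into fast, slippery movement.
; Event_Spawn_Flame waits a short random delay, activates the flame effect, scales the sphere collider through a timeline, and switches off after ActivationTime.
; While active, capsule overlap sets the player's FireLock, movement override and foot flames, then resets them after a fixed delay.
; Game manager registration and debug spawn code are present but never run.
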(event OnComponentBeginOverlap(Collider)
  (params (OverlappedComponent :type Primitive%20Component%20Object%20Reference) (OtherActor :type Actor%20Object%20Reference) (OtherComp :type Primitive%20Component%20Object%20Reference) (OtherBodyIndex :type Integer) (bFromSweep :type Boolean) (SweepResult :type Hit%20Result%20Structure%20%28by%20ref%29))
  ;[1 0.4522 0] Flame Effect
  (if (Variables|Default|GetIsActive)
    (bind _asbp_player (Utilities|Casting|CastToBP_Player OtherActor))
    (if (== OtherComp (Variables|/Script/Engine.Character|GetCapsuleComponent _asbp_player))
      (Variables|/Game/Blueprints/Player/BP_Player.BP_Player_C|SetFireLock _asbp_player true)
      (Default|SetMouvmentSetting _asbp_player 0.05 0.0 0.05 8e+02 3e+03)
      (Components|Activation|Activate (Variables|/Game/Blueprints/Player/BP_Player.BP_Player_C|GetFlammeFoot _asbp_player) false)
      (Utilities|FlowControl|Delay 5.0)
      (Components|Activation|SetActive (Variables|/Game/Blueprints/Player/BP_Player.BP_Player_C|GetFlammeFoot _asbp_player) false false)
      (Variables|Default|SetIsActive false)
      (Variables|/Game/Blueprints/Player/BP_Player.BP_Player_C|SetFireLock _asbp_player false)
      (Default|EventResetMouvement _asbp_player))))

(event Custom|Event_Spawn_Flame
  (params (ActivationTime :type Float%20%28double-precision%29))
  ;[0.15 0.15 0.15 0.5] Spawn
  (Utilities|FlowControl|Delay (Math|Random|RandomFloatinRange 0.5 1.0))
  (Variables|Default|SetIsActive true)
  (Components|Activation|Activate (Variables|Default|GetFlamme) false)
  (bind _newtrack_0 (Timeline|Timeline PlayFromStart)
    (:Update
      (Components|Sphere|SetSphereRadius (Variables|Default|GetCollider) (* _newtrack_0 1.2e+02) true)
      (Utilities|FlowControl|Delay ActivationTime)
      (Components|Activation|SetActive (Variables|Default|GetFlamme) false false)
      (Variables|Default|SetIsActive false))))

(event EventBeginPlay
  ;[0.003705 0.485 0] Begin play
)

(fn ConstructionScript)

(fn SetMouvmentSetting
  (params (GroundFriction :type Float%20%28double-precision%29) (BreakingDecelerationWalking :type Float%20%28double-precision%29) (BreakingFactor :type Float%20%28double-precision%29) (MaxWalkSpeed :type Float%20%28double-precision%29) (MaxAcceleration :type Float%20%28double-precision%29)))