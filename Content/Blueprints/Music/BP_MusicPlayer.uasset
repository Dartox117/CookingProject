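; BP_MusicPlayer is a music actor that starts the soundtrack for the level it is placed in.
; On BeginPlay it maps the WhithLevel enum (Menu, Tv, Pirate, Fary Tale) to the integer Level parameter on the SCMusic audio component, then plays it from the start.
; Track selection is left to the sound asset, driven by that parameter.
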(event EventBeginPlay
  (switch Utilities|FlowControl|Switch|SwitchonE_LevelType (Variables|Default|GetWhithLevel)
    (:NewEnumerator0
      (Effects|Components|ParticleSystem|SetIntParameter (Variables|Default|GetSC_Music) "Level" 0))
    (:NewEnumerator1
      (Effects|Components|ParticleSystem|SetIntParameter (Variables|Default|GetSC_Music) "Level" 3))
    (:NewEnumerator2
      (Effects|Components|ParticleSystem|SetIntParameter (Variables|Default|GetSC_Music) "Level" 2))
    (:NewEnumerator3
      (Effects|Components|ParticleSystem|SetIntParameter (Variables|Default|GetSC_Music) "Level" 1)))
  (Audio|Components|Audio|Play (Variables|Default|GetSC_Music) 0.0))

(fn ConstructionScript)