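; Level design spline actor that lines its spline with repeated copies of a selected static mesh.
; The construction script adds one X-forward, collision-enabled spline mesh component per MeshSize step of spline length.
; Two helper functions supply local positions and tangents at each segment boundary, clamping tangent length to MeshSize.
; Their results feed SetStartAndEnd swapped, so each segment starts at the farther distance along the spline.
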(fn ConstructionScript
  (for _index (range 0 (Math|Float|Truncate (/ (Spline|GetSplineLength (Variables|Default|GetSpline)) (Variables|Default|GetMeshSize))))
    (Variables|Default|SetloopIndex _index)
    (bind _returnvalue (AddComponent|AddSplineMeshComponent false))
    (LocalVariables|SetSplineMeshComp _returnvalue)
    (Components|StaticMesh|SetStaticMesh (LocalVariables|GetSplineMeshComp) (Variables|Default|GetSelectedMesh))
    (SplineMesh|SetForwardAxis (LocalVariables|GetSplineMeshComp) "X" true)
    (bind (_position _tangent) (CallFunction|FunctionGetStartPosition/Tangent (Variables|Default|GetloopIndex)))
    (bind (_position_2 _tangent_2) (CallFunction|FunctionGetEndPosition/Tangent (Variables|Default|GetloopIndex)))
    (SplineMesh|SetStartandEnd (LocalVariables|GetSplineMeshComp) _position_2 _tangent_2 _position _tangent true :!class /Script/Engine.SplineMeshComponent)
    (Collision|SetCollisionEnabled (LocalVariables|GetSplineMeshComp) "QueryAndPhysics")))

(fn FunctionGetStartPosition/Tangent
  (params (Index :type Integer))
  (bind _spline (Variables|Default|GetSpline))
  (bind _meshsize (Variables|Default|GetMeshSize))
  (bind _returnvalue (* Index _meshsize))
  (return (Spline|GetLocationatDistanceAlongSpline _spline _returnvalue "Local") (Math|Vector|ClampVectorSize (Spline|GetTangentatDistanceAlongSpline _spline _returnvalue "Local") 0.0 (Variables|Default|GetMeshSize))))

(fn FunctionGetEndPosition/Tangent
  (params (Index :type Integer))
  (bind _returnvalue (+ Index 1))
  (bind _spline (Variables|Default|GetSpline))
  (bind _meshsize (Variables|Default|GetMeshSize))
  (bind _returnvalue_2 (* _returnvalue _meshsize))
  (return (Spline|GetLocationatDistanceAlongSpline _spline _returnvalue_2 "Local") (Math|Vector|ClampVectorSize (Spline|GetTangentatDistanceAlongSpline _spline _returnvalue_2 "Local") 0.0 (Variables|Default|GetMeshSize))))