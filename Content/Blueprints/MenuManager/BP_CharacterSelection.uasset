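; BP_CharacterSelection is a per-player rotating carousel of four characters for menu character and skin selection.
; It registers with its BP_MenuPawn, turns 90 degrees per step via a timeline that blocks input until finished, and drops in from above.
; SetMaterial maps the skin index to a color and character-specific material instance, applies it to the mesh, then saves both in BP_GameInstance for player one or two.
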(event Custom|SetMaterial
  (params (SkinSelection :type Integer))
  (Variables|Default|SetSkinSelection SkinSelection)
  (CallFunction|ColorSelection)
  (switch int (Variables|Default|GetActualMesh)
    (:0
      (CallFunction|CameleonSkin))
    (:1
      (CallFunction|LemurienSkin))
    (:2
      (CallFunction|PoulpeSkin))
    (:3
      (CallFunction|RenardSkin))))

(event Custom|RightTurn
  (params (Index :type Integer))
  (Variables|Default|SetActualMesh Index)
  (Variables|Default|SetRotation 9e+01)
  (Variables|/Game/Blueprints/MenuManager/BP_MenuPawn.BP_MenuPawn_C|SetCanTurn (Variables|Default|GetAs%20BP%20Menu%20Pawn) false)
  (bind _newtrack_0 (Timeline|Turn PlayFromStart)
    (:Update
      (Transformation|SetRelativeRotation (Variables|Default|GetDefaultSceneRoot) (Math|Rotator|MakeRotator (.roll (Variables|Default|GetBaseRotatation)) (.pitch (Variables|Default|GetBaseRotatation)) (Math|Float|Lerp (.yaw (Variables|Default|GetBaseRotatation)) (+ (.yaw (Variables|Default|GetBaseRotatation)) (Variables|Default|GetRotation)) _newtrack_0)) false false))
    (:Finished
      (Variables|Default|SetBaseRotatation (Variables|/Script/Engine.SceneComponent|GetRelativeRotation (Variables|Default|GetDefaultSceneRoot)))
      (Variables|/Game/Blueprints/MenuManager/BP_MenuPawn.BP_MenuPawn_C|SetCanTurn (Variables|Default|GetAs%20BP%20Menu%20Pawn) true))))

(event Custom|LeftTurn
  (params (Index :type Integer))
  (Variables|Default|SetActualMesh Index)
  (Variables|Default|SetRotation -9e+01)
  (Variables|/Game/Blueprints/MenuManager/BP_MenuPawn.BP_MenuPawn_C|SetCanTurn (Variables|Default|GetAs%20BP%20Menu%20Pawn) false)
  (bind _newtrack_0 (Timeline|Turn PlayFromStart)
    (:Update
      (Transformation|SetRelativeRotation (Variables|Default|GetDefaultSceneRoot) (Math|Rotator|MakeRotator (.roll (Variables|Default|GetBaseRotatation)) (.pitch (Variables|Default|GetBaseRotatation)) (Math|Float|Lerp (.yaw (Variables|Default|GetBaseRotatation)) (+ (.yaw (Variables|Default|GetBaseRotatation)) (Variables|Default|GetRotation)) _newtrack_0)) false false))
    (:Finished
      (Variables|Default|SetBaseRotatation (Variables|/Script/Engine.SceneComponent|GetRelativeRotation (Variables|Default|GetDefaultSceneRoot)))
      (Variables|/Game/Blueprints/MenuManager/BP_MenuPawn.BP_MenuPawn_C|SetCanTurn (Variables|Default|GetAs%20BP%20Menu%20Pawn) true))))

(event Custom|PlaySelectionAnim
  (Variables|Default|SetIsSelected true))

(event Custom|FallAnim
  (bind _returnvalue (Transformation|GetActorLocation))
  (Variables|Default|SetIsFalling true)
  (bind _newtrack_0 (Timeline|Fall PlayFromStart)
    (:Update
      (Transformation|SetActorLocation (Math|Vector|MakeVector (.x _returnvalue) (.y _returnvalue) (Math|Float|Lerp (+ (Variables|Default|GetbaseZ) 1e+03) (Variables|Default|GetbaseZ) _newtrack_0)) false false))
    (:Finished
      (Variables|Default|SetIsFalling false))))

(event Custom|ColorSelection
  (switch int (Variables|Default|GetSkinSelection)
    (:0
      (Variables|Default|SetChosedColor "(R=0.059489,G=0.677083,B=0.000998,A=1.000000)"))
    (:1
      (Variables|Default|SetChosedColor "(R=0.526042,G=0.002401,B=0.434045,A=1.000000)"))
    (:2
      (Variables|Default|SetChosedColor "(R=0.000000,G=0.216244,B=0.593750,A=1.000000)"))
    (:3
      (Variables|Default|SetChosedColor "(R=0.546875,G=0.522440,B=0.000000,A=1.000000)"))
    (:4
      (Variables|Default|SetChosedColor "(R=0.104167,G=0.104167,B=0.104167,A=1.000000)"))))

(event EventBeginPlay
  (bind _returnvalue (Transformation|GetActorLocation))
  (Variables|Default|SetBaseRotatation (Variables|/Script/Engine.SceneComponent|GetRelativeRotation (Variables|Default|GetDefaultSceneRoot)))
  (Utilities|FlowControl|Delay 0.3)
  (bind _asbp_menu_pawn (Utilities|Casting|CastToBP_MenuPawn (Game|Player|GetPlayerPawn (Variables|Default|GetPawnToBe))))
  (bind _output_get (Variables|Default|SetAs%20BP%20Menu%20Pawn _asbp_menu_pawn))
  (Variables|/Game/Blueprints/MenuManager/BP_MenuPawn.BP_MenuPawn_C|SetCharacterSelectionMesh _output_get self)
  (Components|Timeline|SetPlayRate (Variables|Default|GetTurn) 4.0)
  (Variables|Default|SetCharacterMesh (Utilities|Array|MakeArray (Variables|Default|GetCharacter1) (Variables|Default|GetCharacter) (Variables|Default|GetCharacter3) (Variables|Default|GetCharacter2)))
  (Variables|Default|SetbaseZ (.z _returnvalue))
  (Transformation|SetActorLocation (Math|Vector|MakeVector (.x _returnvalue) (.y _returnvalue) (+ (.z _returnvalue) 1e+03)) false false))

(event Custom|CameleonSkin
  (switch int (Variables|Default|GetSkinSelection)
    (:0
      (Variables|Default|SetChosedMat "/Game/Art/Materials/Character/Newton/MI_CelNewton.MI_CelNewton"))
    (:1
      (Variables|Default|SetChosedMat "/Game/Art/Materials/Character/Newton/MI_CelNewton_S2.MI_CelNewton_S2"))
    (:2
      (Variables|Default|SetChosedMat "/Game/Art/Materials/Character/Newton/MI_CelNewton_S3.MI_CelNewton_S3"))
    (:3
      (Variables|Default|SetChosedMat "/Game/Art/Materials/Character/Newton/MI_CelNewton_S4.MI_CelNewton_S4"))
    (:4
      (Variables|Default|SetChosedMat "/Game/Art/Materials/Character/Newton/MI_CelNewton_S1.MI_CelNewton_S1")))
  (Rendering|Material|SetMaterial (Variables|Default|GetCharacter1) 0 (Variables|Default|GetChosedMat))
  (CallFunction|ApplyMaterial))

(event Custom|ApplyMaterial
  (switch int (Variables|Default|GetPawnToBe)
    (:0
      (bind _asbp_game_instance (Utilities|Casting|CastToBP_GameInstance (Game|GetGameInstance)))
      (Variables|/Game/Blueprints/GameInstance/BP_GameInstance.BP_GameInstance_C|SetMaterialPlayer_1 _asbp_game_instance (Variables|Default|GetChosedMat))
      (Variables|/Game/Blueprints/GameInstance/BP_GameInstance.BP_GameInstance_C|SetColorPlayer_1 _asbp_game_instance (Variables|Default|GetChosedColor)))
    (:1
      (bind _asbp_game_instance_2 (Utilities|Casting|CastToBP_GameInstance (Game|GetGameInstance)))
      (Variables|/Game/Blueprints/GameInstance/BP_GameInstance.BP_GameInstance_C|SetMaterialPlayer_2 _asbp_game_instance_2 (Variables|Default|GetChosedMat))
      (Variables|/Game/Blueprints/GameInstance/BP_GameInstance.BP_GameInstance_C|SetColorPlayer_2 _asbp_game_instance_2 (Variables|Default|GetChosedColor)))))

(event Custom|LemurienSkin
  (switch int (Variables|Default|GetSkinSelection)
    (:0
      (Variables|Default|SetChosedMat "/Game/Art/Materials/Character/Jao/MI_CelJao_S4.MI_CelJao_S4"))
    (:1
      (Variables|Default|SetChosedMat "/Game/Art/Materials/Character/Jao/MI_CelJao.MI_CelJao"))
    (:2
      (Variables|Default|SetChosedMat "/Game/Art/Materials/Character/Jao/MI_CelJao_S1.MI_CelJao_S1"))
    (:3
      (Variables|Default|SetChosedMat "/Game/Art/Materials/Character/Jao/MI_CelJao_S2.MI_CelJao_S2"))
    (:4
      (Variables|Default|SetChosedMat "/Game/Art/Materials/Character/Jao/MI_CelJao_S3.MI_CelJao_S3")))
  (Rendering|Material|SetMaterial (Variables|Default|GetCharacter) 0 (Variables|Default|GetChosedMat))
  (CallFunction|ApplyMaterial))

(event Custom|PoulpeSkin
  (switch int (Variables|Default|GetSkinSelection)
    (:0
      ;[0.15 0.15 0.15 0.5] à remplir puis à link
      (Variables|Default|SetChosedMat "/Game/Art/Materials/Character/Cpt_Herlock/MI_CelHerlock_S1.MI_CelHerlock_S1"))
    (:1
      (Variables|Default|SetChosedMat "/Game/Art/Materials/Character/Cpt_Herlock/MI_CelHerlock_S2.MI_CelHerlock_S2"))
    (:2
      (Variables|Default|SetChosedMat "/Game/Art/Materials/Character/Cpt_Herlock/MI_CelHerlock.MI_CelHerlock"))
    (:3
      (Variables|Default|SetChosedMat "/Game/Art/Materials/Character/Cpt_Herlock/MI_CelHerlock_S3.MI_CelHerlock_S3"))
    (:4
      (Variables|Default|SetChosedMat "/Game/Art/Materials/Character/Cpt_Herlock/MI_CelHerlock_S4.MI_CelHerlock_S4")))
  (Rendering|Material|SetMaterial (Variables|Default|GetCharacter3) 0 (Variables|Default|GetChosedMat))
  (CallFunction|ApplyMaterial))

(event Custom|RenardSkin
  (switch int (Variables|Default|GetSkinSelection)
    (:0
      ;[0.15 0.15 0.15 0.5] à remplir puis à link
      (Variables|Default|SetChosedMat "/Game/Art/Materials/Character/Lena/MI_CelLena_S4.MI_CelLena_S4"))
    (:1
      (Variables|Default|SetChosedMat "/Game/Art/Materials/Character/Lena/MI_CelLena_S1.MI_CelLena_S1"))
    (:2
      (Variables|Default|SetChosedMat "/Game/Art/Materials/Character/Lena/MI_CelLena_S2.MI_CelLena_S2"))
    (:3
      (Variables|Default|SetChosedMat "/Game/Art/Materials/Character/Lena/MI_CelLena.MI_CelLena"))
    (:4
      (Variables|Default|SetChosedMat "/Game/Art/Materials/Character/Lena/MI_CelLena_S3.MI_CelLena_S3")))
  (Rendering|Material|SetMaterial (Variables|Default|GetCharacter2) 0 (Variables|Default|GetChosedMat))
  (CallFunction|ApplyMaterial))

(fn ConstructionScript)