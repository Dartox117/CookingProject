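; BP_MoneySafe is a falling-safe hazard that targets a player and stuns them on impact.
; Stun makes it track the player's XY at a set height on Tick until a random timer triggers the drop.
; A timeline lerps it down onto the still-tracked player, disabling dash early in the fall unless protected.
; On landing it freezes an unprotected player with stun VFX, unfreezes after delays, and destroys itself.
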(event Custom|Stun
  (params (PlayerRef :type BP%20Player%20Object%20Reference))
  (Variables|Default|SetPlayer%20Ref PlayerRef)
  (Variables|Default|SetCanTick true)
  (Utilities|Time|SetTimerbyEvent (delegate Custom|GoOnPlayer) (Math|Random|RandomFloatinRange 2.0 4.0)))

(event Custom|GoOnPlayer
  (bind _player_ref (Variables|Default|GetPlayer%20Ref))
  (bind _returnvalue (Transformation|GetActorLocation _player_ref))
  (Components|Activation|Activate (Variables|Default|GetNiagara) false)
  (Variables|Default|SetCanTick false)
  (bind _newtrack_0 (Timeline|Drop PlayFromStart)
    (:Update
      (Transformation|SetActorLocation (Math|Vector|MakeVector (.x _returnvalue) (.y _returnvalue) (Math|Float|Lerp 6e+02 (.z (Transformation|GetActorLocation (Variables|Default|GetPlayer%20Ref))) _newtrack_0)) false false)
      (if (and (>= _newtrack_0 0.11) (not (Variables|/Game/Blueprints/Player/BP_Player.BP_Player_C|GetIsProtected (Variables|Default|GetPlayer%20Ref))))
        (Variables|/Game/Blueprints/Player/BP_Player.BP_Player_C|SetCanDash (Variables|Default|GetPlayer%20Ref) false)))
    (:Finished
      (if (not (Variables|/Game/Blueprints/Player/BP_Player.BP_Player_C|GetIsProtected (Variables|Default|GetPlayer%20Ref)))
        (Components|Activation|Deactivate (Variables|Default|GetNiagara))
        (Default|FreezePlayer (Variables|Default|GetPlayer%20Ref))
        (Components|Activation|Activate (Variables|/Game/Blueprints/Player/BP_Player.BP_Player_C|GetStun_VFX (Variables|Default|GetPlayer%20Ref)) false)
        (Utilities|FlowControl|Delay 0.5)
        (Rendering|SetVisibility (Variables|Default|GetStaticMesh) false false)
        (Utilities|FlowControl|Delay 2.0)
        (Default|UnFreezePlayer (Variables|Default|GetPlayer%20Ref))
        (Actor|DestroyActor)
        (Components|Activation|Deactivate (Variables|/Game/Blueprints/Player/BP_Player.BP_Player_C|GetStun_VFX (Variables|Default|GetPlayer%20Ref)))
        (else
          (Utilities|FlowControl|Delay 1.0)
          (Actor|DestroyActor))))))

(event EventBeginPlay)

(event Collision|EventActorBeginOverlap
  (params (OtherActor :type Actor%20Object%20Reference)))

(event EventTick
  (params (DeltaSeconds :type Float%20%28single-precision%29))
  (bind _player_ref (Variables|Default|GetPlayer%20Ref))
  (bind _returnvalue (Transformation|GetActorLocation _player_ref))
  (if (Variables|Default|GetCanTick)
    (Transformation|SetActorLocation (Math|Vector|MakeVector (.x _returnvalue) (.y _returnvalue) (Variables|Default|GetZ_Location)) false false)))

(fn ConstructionScript)